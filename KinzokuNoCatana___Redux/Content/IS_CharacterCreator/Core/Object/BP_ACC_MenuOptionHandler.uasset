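; BP_ACC_MenuOptionHandler coordinates menu option groups in the character creator and links each group to a widget switcher.
; Initialization registers the handler on every group, then builds a group-to-switcher map by matching array indices.
; When a group reports an option change, the handler looks up its switcher and calls OnMenuOptionClicked with that switcher and item.
; Reset functions deactivate the options in one group by index or in all groups.
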(fn `InitAttachedWS`
  (params (AttachedWSOption :type "Array of WidgetSwitcher Object Reference"))
  (`BlueprintMapLibrary.Map_Clear` (`self.AttachedWSOption`))
  (for (_array_element _array_index) (`self.MenuOptionGroupList`)
    (`BlueprintMapLibrary.Map_Add` (`self.AttachedWSOption`) _array_element (`|GetArrayItem` AttachedWSOption _array_index))))

(fn `InitMenuOptionHandler`
  (params (NewMenuOptionGroupList :type "Array of /Game/IS_CharacterCreator/Core/Widget/Components/Group/WBP_ACC_MenuGroup Object Reference"))
  (bind _output_get (set `self.MenuOptionGroupList` NewMenuOptionGroupList))
  (for _array_element _output_get
    (set `/Game/IS_CharacterCreator/Core/Widget/Components/Group/WBP_ACC_MenuGroup.MenuOptionHandler` self _array_element)))

(fn `OnMenuOptionChange`
  (params (MenuGroup :type "/Game/IS_CharacterCreator/Core/Widget/Components/Group/WBP_ACC_MenuGroup Object Reference") (Item :type "/Game/IS_CharacterCreator/Core/Data/Struct/UI/FStruct_ACC_UI_Item Structure"))
  (bind (_value _returnvalue) (`BlueprintMapLibrary.Map_Find` (`self.AttachedWSOption`) MenuGroup))
  (if _returnvalue
    (`self.OnMenuOptionClicked` _value Item)))

(fn `ResetAllMenu`
  (for _array_element (`self.MenuOptionGroupList`)
    (`/Game/IS_CharacterCreator/Core/Widget/Components/Group/WBP_ACC_MenuGroup.UnactiveAll` _array_element)))

(fn `ResetMenu`
  (params (MenuIndex :type Integer))
  (`/Game/IS_CharacterCreator/Core/Widget/Components/Group/WBP_ACC_MenuGroup.UnactiveAll` (`|GetArrayItem` (`self.MenuOptionGroupList`) MenuIndex)))