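; Data access object for the character creator's items, reading item data and custom colors from DataTables.
; Lookups build row keys from ID, species, maturity and gender, retrying with a common gender key when the first row is missing.
; GetACCItemDataFromGender adds a further fallback that omits the species argument.
; Batch helpers resolve ID lists into item data or into UI entries with ID, label and icon.
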(fn `GetACCItemData`
  (params (Id :type Integer) (Specie :type Name) (Maturity :type "/Game/IS_CharacterCreator/Core/Data/Enum/E_ACC_Maturity Enum" :default "NewEnumerator0") (UseGender :type Boolean) (Gender :type "/Game/IS_CharacterCreator/Core/Data/Enum/E_ACC_Gender Enum" :default "NewEnumerator0"))
  (returns (ACC_ItemData :type "/Game/IS_CharacterCreator/Core/Data/Struct/Common/FStruct_ACC_ItemData Structure") (Found :type Boolean))
  (bind _returnvalue (`|GetDataTableRow` (`self.DT_ItemDataList`) (`self.BuildSpecieDTKey` Id Specie Maturity Gender UseGender))
    (:`then`
      (return _returnvalue true))
    (:`RowNotFound`
      ;[0 0.1094 1] Else try get cmn armor
      (bind _returnvalue_2 (`|GetDataTableRow` (`self.DT_ItemDataList`) (`self.BuildSpecieDTKey` Id Specie Maturity "NewEnumerator2"))
        (:`then`
          (return _returnvalue_2 true))
        (:`RowNotFound`
          (return (struct) false))))))

(fn `GetACCItemDataFromGender`
  (params (Id :type Integer) (Specie :type Name) (Maturity :type "/Game/IS_CharacterCreator/Core/Data/Enum/E_ACC_Maturity Enum" :default "NewEnumerator0") (Gender :type "/Game/IS_CharacterCreator/Core/Data/Enum/E_ACC_Gender Enum" :default "NewEnumerator0"))
  (returns (ACC_ItemData :type "/Game/IS_CharacterCreator/Core/Data/Struct/Common/FStruct_ACC_ItemData Structure"))
  (bind (_acc_itemdata _found) (`self.GetACCItemData` Id Specie Maturity true Gender))
  (if _found
    (return _acc_itemdata)
    (else
      (bind _acc_itemdata_2 (`self.GetACCItemData` Id "None" Maturity false Gender))
      (return _acc_itemdata_2))))

(fn `GetACCItemFromIds`
  (params (Ids :type "Array of Integer") (Specie :type Name) (Maturity :type "/Game/IS_CharacterCreator/Core/Data/Enum/E_ACC_Maturity Enum" :default "NewEnumerator0") (Gender :type "/Game/IS_CharacterCreator/Core/Data/Enum/E_ACC_Gender Enum" :default "NewEnumerator0") (UseGender :type Boolean :default true))
  (returns (ItemList :type "Array of /Game/IS_CharacterCreator/Core/Data/Struct/Common/FStruct_ACC_ItemData Structure"))
  (locals (Tmp_ItemList :type "Array of /Game/IS_CharacterCreator/Core/Data/Struct/Common/FStruct_ACC_ItemData Structure"))
  (for _array_element Ids
    (bind _acc_itemdata (`self.GetACCItemData` _array_element Specie Maturity UseGender Gender))
    (`KismetArrayLibrary.Array_Add` (`local.Tmp_ItemList`) _acc_itemdata))
  (return (`local.Tmp_ItemList`)))

(fn `GetACCUIItemFromItem`
  (params (Ids :type "Array of Integer") (Specie :type Name) (Maturity :type "/Game/IS_CharacterCreator/Core/Data/Enum/E_ACC_Maturity Enum" :default "NewEnumerator0") (Gender :type "/Game/IS_CharacterCreator/Core/Data/Enum/E_ACC_Gender Enum" :default "NewEnumerator0"))
  (returns (UIItemList :type "Array of /Game/IS_CharacterCreator/Core/Data/Struct/UI/FStruct_ACC_UI_Item Structure"))
  (locals (Tmp_UIItemList :type "Array of /Game/IS_CharacterCreator/Core/Data/Struct/UI/FStruct_ACC_UI_Item Structure"))
  (bind _itemlist (`self.GetACCItemFromIds` Ids Specie Maturity Gender))
  (for _array_element _itemlist
    (bind (_itemid _name _priority _icon) (break `/Game/IS_CharacterCreator/Core/Data/Struct/Common/FStruct_ACC_ItemData` _array_element))
    (`KismetArrayLibrary.Array_Add` (`local.Tmp_UIItemList`) (make `/Game/IS_CharacterCreator/Core/Data/Struct/UI/FStruct_ACC_UI_Item` _itemid _name _icon)))
  (return (`local.Tmp_UIItemList`)))

(fn `GetItemCtmColor`
  (params (Key :type Name))
  (returns (ItemCtm :type "/Game/IS_CharacterCreator/Core/Data/Struct/Customization/FStruct_ACC_ItemCustomization Structure"))
  (bind _returnvalue (`|GetDataTableRow` (`self.DT_ItemColorList`) Key)
    (:`then`
      (return _returnvalue))))