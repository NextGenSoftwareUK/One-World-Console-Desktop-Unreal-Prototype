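; BP_ACC_DAO is the character creator's data access module, serving species, species UI config and custom mesh data from data tables.
; On init it constructs Advanced, Item, Head and Character sub-DAOs, passing each the game module, and exposes getters for them.
; Custom mesh rows are keyed by a type-and-ID slug and report success, falling back to default data when missing.
; Character list, save and remove functions are empty stubs here.
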(fn `GetCharacterList`
  (returns (CharacterList :type "Array of /Game/IS_CharacterCreator/Core/Data/Struct/FStruct_ACC_Character Structure"))
  (return))

(fn `GetCustomMeshData`
  (params (CustomType :type Name) (Id :type Integer))
  (returns (MeshData :type "/Game/IS_CharacterCreator/Core/Data/Struct/Customization/FStruct_ACC_HairData Structure") (Success :type Boolean))
  (bind _returnvalue (`|GetDataTableRow` (`self.DT_CustomMeshData`) (`KismetStringLibrary.Conv_StringToName` (`KismetStringLibrary.Concat_StrStr` (`KismetStringLibrary.Concat_StrStr` (`KismetStringLibrary.Conv_NameToString` CustomType) "_") (`KismetStringLibrary.Conv_IntToString` Id))))
    (:`then`
      (return _returnvalue true))
    (:`RowNotFound`
      (return (make `/Game/IS_CharacterCreator/Core/Data/Struct/Customization/FStruct_ACC_HairData` 0 null null) false))))

(fn `GetDAOAdvanced`
  (returns (DAOAdvanced :type "/Game/IS_CharacterCreator/Core/Object/DAO/BP_ACC_DAO_Advanced Object Reference"))
  (return (`self.DAOAdvanced`)))

(fn `GetDAOCharacter`
  (returns (DAOCharacter :type "/Game/IS_CharacterCreator/Core/Object/DAO/BP_ACC_DAO_Character Object Reference"))
  (return (`self.DAOCharacter`)))

(fn `GetDAOHead`
  (returns (DAOHead :type "/Game/IS_CharacterCreator/Core/Object/DAO/BP_ACC_DAO_Head Object Reference"))
  (return (`self.DAOHead`)))

(fn `GetDAOItem`
  (returns (DAOItem :type "/Game/IS_CharacterCreator/Core/Object/DAO/BP_ACC_DAO_Item Object Reference"))
  (return (`self.DAOItem`)))

(fn `GetGameInstance`
  (returns (GameInstance :type "GameInstance Object Reference"))
  (return (`/Game/IS_CharacterCreator/Core/Object/BP_ACC_Game.GetGameInstance` (`self.GetGameModule`))))

(fn `GetSpecie`
  (params (Identifier :type Name))
  (returns (Specie :type "/Game/IS_CharacterCreator/Core/Data/Struct/FStruct_ACC_SpecieParam Structure"))
  (bind _returnvalue (`|GetDataTableRow` (`self.DT_Species`) Identifier)
    (:`then`
      (return _returnvalue))))

(fn `GetSpecieUIConfigData`
  (params (Identifier :type Name))
  (returns (SpecieUIConfig :type "/Game/IS_CharacterCreator/Core/Data/Struct/UI/Config/FStruct_ACC_SpecieUIConfig Structure"))
  (bind _returnvalue (`|GetDataTableRow` (`self.DT_SpecieUIConfig`) Identifier)
    (:`then`
      (return _returnvalue))
    (:`RowNotFound`
      (return))))

(fn `InitModule`
  (`parent.InitModule`)
  (`|ExecutionSequence`
    (:`then_0`
      ;[1 0.5625 0] DAO Advanced
      (bind _returnvalue (`|GenericCreateObject` self "/Game/IS_CharacterCreator/Core/Object/DAO/BP_ACC_DAO_Advanced.BP_ACC_DAO_Advanced_C" (`self.GetGameModule`)))
      (set `self.DAOAdvanced` _returnvalue)
      ;[0.5021 0.3051 1] DAO Item
      (bind _returnvalue_2 (`|GenericCreateObject` self "/Game/IS_CharacterCreator/Core/Object/DAO/BP_ACC_DAO_Item.BP_ACC_DAO_Item_C" (`self.GetGameModule`)))
      (set `self.DAOItem` _returnvalue_2))
    (:`then_1`
      ;[1 0.5625 0] DAO Head
      (bind _returnvalue_3 (`|GenericCreateObject` self "/Game/IS_CharacterCreator/Core/Object/DAO/BP_ACC_DAO_Head.BP_ACC_DAO_Head_C" (`self.GetGameModule`)))
      (set `self.DAOHead` _returnvalue_3)
      ;[0.5021 0.3051 1] DAO Character
      (bind _returnvalue_4 (`|GenericCreateObject` self "/Game/IS_CharacterCreator/Core/Object/DAO/BP_ACC_DAO_Character.BP_ACC_DAO_Character_C" (`self.GetGameModule`)))
      (set `self.DAOCharacter` _returnvalue_4))))

(fn `RemoveCharacter`
  (params (UID :type String)))

(fn `SaveCharacter`
  (params (UID :type String) (ACC_Character :type "/Game/IS_CharacterCreator/Core/Data/Struct/FStruct_ACC_Character Structure")))