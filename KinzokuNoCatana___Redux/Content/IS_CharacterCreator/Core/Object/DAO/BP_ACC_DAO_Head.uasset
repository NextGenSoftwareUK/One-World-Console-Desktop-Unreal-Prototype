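; BP_ACC_DAO_Head is a character creator data access object that serves head-related content from data tables.
; It looks up head meshes and hair meshes by row name, fetches iris textures by ID, and exposes the eyebrow and custom face tables.
; Advanced hair lookup builds an identifier from species, maturity, gender and hair ID, falling back to a common gender variant when that row is missing.
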(fn `GetCustomFaceDT`
  (returns (DT_CustomFaceData :type "DataTable Object Reference"))
  (return (`self.DT_CustomFaceData`)))

(fn `GetEyeBrowDT`
  (returns (DT_EyeBrowData :type "DataTable Object Reference"))
  (return (`self.DT_EyeBrowData`)))

(fn `GetHairData`
  (params (Identifier :type Name))
  (returns (HairData :type "/Game/IS_CharacterCreator/Core/Data/Struct/Customization/FStruct_ACC_HairData Structure") (Success :type Boolean))
  (bind _returnvalue (`|GetDataTableRow` (`self.DT_HairMeshData`) Identifier)
    (:`then`
      (return _returnvalue true))
    (:`RowNotFound`
      (return (struct) false))))

(fn `GetHairDataAdvanced`
  (params (HairId :type Integer) (Specie :type Name) (Maturity :type "/Game/IS_CharacterCreator/Core/Data/Enum/E_ACC_Maturity Enum" :default "NewEnumerator0") (Gender :type "/Game/IS_CharacterCreator/Core/Data/Enum/E_ACC_Gender Enum" :default "NewEnumerator0"))
  (returns (HairData :type "/Game/IS_CharacterCreator/Core/Data/Struct/Customization/FStruct_ACC_HairData Structure") (Success :type Boolean))
  (bind _utilities (`/Game/IS_CharacterCreator/Core/Object/BP_ACC_Game.GetUtilities` (`self.GetGameModule`)))
  (bind (_hairdata _success) (`self.GetHairData` (`/Game/IS_CharacterCreator/Core/Object/Module/BP_ACC_Utilities.BuildHairIdentifier` _utilities Specie Maturity Gender HairId "None")))
  (if _success
    (return _hairdata true)
    (else
      ;[0.07812 0 1] Else try to find cmn
      (bind (_hairdata_2 _success_2) (`self.GetHairData` (`/Game/IS_CharacterCreator/Core/Object/Module/BP_ACC_Utilities.BuildHairIdentifier` _utilities Specie Maturity "NewEnumerator2" HairId "None")))
      (return _hairdata_2 _success_2))))

(fn `GetHeadData`
  (params (RowName :type Name))
  (returns (HeadData :type "/Game/IS_CharacterCreator/Core/Data/Struct/Customization/FStruct_ACC_HeadData Structure") (Success :type Boolean))
  (bind _returnvalue (`|GetDataTableRow` (`self.DT_HeadMeshData`) RowName)
    (:`then`
      (return _returnvalue true))
    (:`RowNotFound`
      (return (struct) false))))

(fn `GetIrisData`
  (params (Id :type Integer))
  (returns (CustomTextureData :type "/Game/IS_CharacterCreator/Core/Data/Struct/Customization/FStruct_ACC_CustomTexture Structure"))
  (bind _customtexturedata (`self.GetCustomTextureData` Id (`self.DT_IrisData`) "Iris_"))
  (return _customtexturedata))