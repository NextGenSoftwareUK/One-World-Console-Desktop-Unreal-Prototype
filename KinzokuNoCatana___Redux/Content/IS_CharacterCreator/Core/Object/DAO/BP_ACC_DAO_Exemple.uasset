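; Example data access object for the character creator that lists, saves and removes characters in the game's save data.
; Each function casts the game instance to BP_ARPG_GameInstance and works on its save game object.
; Saving stores the character by UID and writes the save, while removal writes only if it succeeds.
; Leftover, unconnected nodes still reference BP_ACC_GameInstance.
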(fn `GetCharacterList`
  (returns (CharacterList :type "Array of /Game/IS_CharacterCreator/Core/Data/Struct/FStruct_ACC_Character Structure"))
  (bind _asbp_arpg_game_instance (cast `/Game/ActionRPGStarterSystem/Character/Blueprints/BP_ARPG_GameInstance` (`self.GetGameInstance`)))
  (bind _values (`BlueprintMapLibrary.Map_Values` (`/Game/IS_CharacterCreator/Core/BP_ACC_SaveGame.CharacterList` (`/Game/ActionRPGStarterSystem/Character/Blueprints/BP_ARPG_GameInstance.SaveGameInstance` _asbp_arpg_game_instance))))
  (return _values))

(fn `RemoveCharacter`
  (params (UID :type String))
  (bind _asbp_arpg_game_instance (cast `/Game/ActionRPGStarterSystem/Character/Blueprints/BP_ARPG_GameInstance` (`self.GetGameInstance`)))
  (bind _returnvalue (`/Game/IS_CharacterCreator/Core/BP_ACC_SaveGame.RemoveCharacter` (`/Game/ActionRPGStarterSystem/Character/Blueprints/BP_ARPG_GameInstance.GetSaveGame` _asbp_arpg_game_instance) UID))
  ;[1 1 1] If was removed with success
  (if _returnvalue
    (`/Game/ActionRPGStarterSystem/Character/Blueprints/BP_ARPG_GameInstance.SaveACCGame` _asbp_arpg_game_instance)))

(fn `SaveCharacter`
  (params (UID :type String) (ACC_Character :type "/Game/IS_CharacterCreator/Core/Data/Struct/FStruct_ACC_Character Structure"))
  (bind _asbp_arpg_game_instance (cast `/Game/ActionRPGStarterSystem/Character/Blueprints/BP_ARPG_GameInstance` (`self.GetGameInstance`)))
  (`/Game/IS_CharacterCreator/Core/BP_ACC_SaveGame.SaveCharacter` (`/Game/ActionRPGStarterSystem/Character/Blueprints/BP_ARPG_GameInstance.GetSaveGame` _asbp_arpg_game_instance) UID ACC_Character)
  (`/Game/ActionRPGStarterSystem/Character/Blueprints/BP_ARPG_GameInstance.SaveACCGame` _asbp_arpg_game_instance))