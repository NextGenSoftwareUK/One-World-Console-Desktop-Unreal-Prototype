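; Character creator data-access object that looks up poses in a poses data table by identifier.
; GetPoseAdvanced builds a specific identifier and a common ("cmn") identifier from Id, species, maturity and gender through the game module's utilities.
; It tries the specific row first, falls back to the common row, and reports whether either exists.
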(fn `GetPose`
  (params (Key :type Name))
  (returns (Pose :type "/Game/IS_CharacterCreator/Core/Data/Struct/Customization/FStruct_ACC_Pose Structure") (Exist :type Boolean))
  (bind _returnvalue (`|GetDataTableRow` (`self.DT_Poses`) Key)
    (:`then`
      (return _returnvalue true))
    (:`RowNotFound`
      (return (struct) false))))

(fn `GetPoseAdvanced`
  (params (Id :type Integer) (Specie :type Name :default "None") (Maturity :type "/Game/IS_CharacterCreator/Core/Data/Enum/E_ACC_Maturity Enum" :default "NewEnumerator0") (Gender :type "/Game/IS_CharacterCreator/Core/Data/Enum/E_ACC_Gender Enum" :default "NewEnumerator0"))
  (returns (Pose :type "/Game/IS_CharacterCreator/Core/Data/Struct/Customization/FStruct_ACC_Pose Structure") (Exist :type Boolean))
  (bind (_identifier _cmnidentifier) (`/Game/IS_CharacterCreator/Core/Object/Module/BP_ACC_Utilities.BuildItemIdentifierAndCmn` (`/Game/IS_CharacterCreator/Core/Object/BP_ACC_Game.GetUtilities` (`self.GetGameModule`)) Id Specie Maturity Gender))
  ;[1 0 0.9844] If don't find ,try with "cmn"
  (bind (_pose _exist) (`self.GetPose` _identifier))
  (if _exist
    ;[0.4766 1 0] Finally return
    (return _pose true)
    (else
      ;[0.2656 1 0] Else try to find cmn pose
      (bind (_pose_2 _exist_2) (`self.GetPose` _cmnidentifier))
      ;[0 0.25 1] if find in "cmn"
      (if _exist_2
        ;[0.4766 1 0] Finally return
        (return _pose_2 true)
        (else
          (return (struct) false))))))