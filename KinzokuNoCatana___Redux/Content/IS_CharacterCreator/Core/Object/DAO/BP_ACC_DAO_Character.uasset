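; Data access object for the character creator that looks up character definitions for presets and NPCs.
; Presets come from DTCharacterPresetList by row name or by an index turned into a "Preset_" row name, and NPCs come from DTNPC by Id.
; These lookups return a Found flag, while the species default lookup reuses the preset lookup with the given identifier and drops that flag.
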(fn `GetCharacterNPCFromId`
  (params (Id :type Name))
  (returns (ACC_Character :type "/Game/IS_CharacterCreator/Core/Data/Struct/FStruct_ACC_Character Structure") (Found :type Boolean))
  (bind _returnvalue (`|GetDataTableRow` (`self.DT_NPC`) Id)
    (:`then`
      (return _returnvalue true))
    (:`RowNotFound`
      (return (struct) false))))

(fn `GetCharacterPreset`
  (params (Identifier :type Name))
  (returns (ACC_Character :type "/Game/IS_CharacterCreator/Core/Data/Struct/FStruct_ACC_Character Structure") (Found :type Boolean))
  (bind _returnvalue (`|GetDataTableRow` (`self.DT_CharacterPresetList`) Identifier)
    (:`then`
      (return _returnvalue true))
    (:`RowNotFound`
      (return (struct) false))))

(fn `GetCharacterPresetFromIndex`
  (params (Id :type Integer))
  (returns (ACC_Character :type "/Game/IS_CharacterCreator/Core/Data/Struct/FStruct_ACC_Character Structure") (Found :type Boolean))
  (bind _returnvalue (`|GetDataTableRow` (`self.DT_CharacterPresetList`) (`KismetStringLibrary.Conv_StringToName` (`KismetStringLibrary.Concat_StrStr` "Preset_" (`KismetStringLibrary.Conv_IntToString` Id))))
    (:`then`
      (return _returnvalue true))
    (:`RowNotFound`
      (return (struct) false))))

(fn `GetDefaultCharacterFromSpecie`
  (params (Identifier :type Name))
  (returns (ACC_Character :type "/Game/IS_CharacterCreator/Core/Data/Struct/FStruct_ACC_Character Structure"))
  (bind _acc_character (`self.GetCharacterPreset` Identifier))
  (return _acc_character))