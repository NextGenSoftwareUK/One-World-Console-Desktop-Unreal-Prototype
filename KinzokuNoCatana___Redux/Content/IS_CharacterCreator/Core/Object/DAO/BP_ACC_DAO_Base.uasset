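; Base data-access object for the character creator, with shared helpers for reading DataTables.
; BuildSpecieDTKey composes row names from an integer ID and either a species, maturity and gender prefix or a common "cmn" prefix.
; Maturity and gender key text comes from the game module's constants.
; GetCustomTextureData looks up a row by prefix plus ID and returns the supplied default when none is found.
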(fn `BuildSpecieDTKey`
  (params (InInt :type Integer) (Specie :type Name) (Maturity :type "/Game/IS_CharacterCreator/Core/Data/Enum/E_ACC_Maturity Enum" :default "NewEnumerator0") (Gender :type "/Game/IS_CharacterCreator/Core/Data/Enum/E_ACC_Gender Enum" :default "NewEnumerator0") (UseSpecie :type Boolean :default true))
  (returns (ReturnValue :type Name))
  (bind _constante (`/Game/IS_CharacterCreator/Core/Object/BP_ACC_Game.GetConstante` (`self.GetGameModule`)))
  (return (`KismetStringLibrary.Conv_StringToName` (`KismetTextLibrary.Conv_TextToString` (`|FormatText` "{prefixe}_{id}" (`KismetTextLibrary.Conv_NameToText` (select `bool` UseSpecie :`false` "cmn" :`true` (`KismetStringLibrary.Conv_StringToName` (`KismetTextLibrary.Conv_TextToString` (`|FormatText` "{specie}_{maturity}_{gender}" Specie (`/Game/IS_CharacterCreator/Core/Object/Module/BP_ACC_Constante.GetMaturityKey` _constante Maturity) (`/Game/IS_CharacterCreator/Core/Object/Module/BP_ACC_Constante.GetGenderKey` _constante Gender)))))) (`KismetTextLibrary.Conv_StringToText` (`KismetStringLibrary.Conv_IntToString` InInt)))))))

(fn `GetCustomTextureData`
  (params (Id :type Integer) (DataTable :type "DataTable Object Reference") (Prefix :type Name) (Default :type "/Game/IS_CharacterCreator/Core/Data/Struct/Customization/FStruct_ACC_CustomTexture Structure"))
  (returns (CustomTextureData :type "/Game/IS_CharacterCreator/Core/Data/Struct/Customization/FStruct_ACC_CustomTexture Structure"))
  (bind _returnvalue (`|GetDataTableRow` DataTable (`KismetStringLibrary.Conv_StringToName` (`KismetStringLibrary.Concat_StrStr` (`KismetStringLibrary.Conv_NameToString` Prefix) (`KismetStringLibrary.Conv_IntToString` Id))))
    (:`then`
      (return _returnvalue))
    (:`RowNotFound`
      (return Default))))