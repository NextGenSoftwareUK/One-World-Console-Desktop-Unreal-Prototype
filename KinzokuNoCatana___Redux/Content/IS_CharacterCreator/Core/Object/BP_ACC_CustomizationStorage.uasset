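; BP_ACC_CustomizationStorage is a data holder for the current character in the character creator.
; Setting a character splits its struct into customization, equipment parameter and equipment ID fields, each group with its own setter.
; GetACCCharacterData rebuilds a struct from those working fields, while GetCurrentCharacter returns the character as last set.
; Unless UseSelectedChar is true, Init loads the character at UseCharIndex from the game module's DAO via the GameInstance interface.
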(fn `GetACCCharacterData`
  (returns (Struct_ACC_Character :type "/Game/IS_CharacterCreator/Core/Data/Struct/FStruct_ACC_Character Structure"))
  (return (make `/Game/IS_CharacterCreator/Core/Data/Struct/FStruct_ACC_Character` "Anonymous" "Anonymous" (`self.CurrentCharCtm`) (`self.CurrentEquipCustomList`) (`self.CurrentCharEquipList`))))

(fn `GetCurrentCharacter`
  (returns (CurrentCharacter :type "/Game/IS_CharacterCreator/Core/Data/Struct/FStruct_ACC_Character Structure"))
  (return (`self.CurrentCharacter`)))

(fn `GetGameInstance`
  (returns (GameInstance :type "GameInstance Object Reference"))
  (return (`self.GameInstance`)))

(fn `Init`
  (if (not (`self.bUseSelectedChar`))
    (bind _gamemodule (message `/Game/IS_CharacterCreator/Core/Interface/BPI_ACC_GameInstance.I_GI_GetACCGameModule` (`self.GetGameInstance`)))
    (bind _characterlist (`/Game/IS_CharacterCreator/Core/Object/DAO/BP_ACC_DAO.GetCharacterList` (`/Game/IS_CharacterCreator/Core/Object/BP_ACC_Game.GetDAO` _gamemodule)))
    (`self.SetCurrentCharacter` (`|GetArrayItem` _characterlist (`self.UseCharIndex`)))))

(fn `SetCurrentCharacter`
  (params (CurrentCharacter :type "/Game/IS_CharacterCreator/Core/Data/Struct/FStruct_ACC_Character Structure"))
  (bind _output_get (set `self.CurrentCharacter` CurrentCharacter))
  (bind (_uid _name _charcustom _equipementparamlist _equipementidlist) (break `/Game/IS_CharacterCreator/Core/Data/Struct/FStruct_ACC_Character` _output_get))
  (`self.SetCurrentCustomization` _charcustom)
  (`self.SetCurrentEquipement` _equipementparamlist _equipementidlist))

(fn `SetCurrentCustomization`
  (params (CurrentCharCtm :type "/Game/IS_CharacterCreator/Core/Data/Struct/Customization/FStruct_ACC_CharacterCustom Structure"))
  (set `self.CurrentCharCtm` CurrentCharCtm))

(fn `SetCurrentEquipement`
  (params (CurrentEquipCustomList :type "Map of Name to /Game/IS_CharacterCreator/Core/Data/Struct/Customization/FStruct_ACC_ItemCustomization Structure") (CurrentCharEquipList :type "Map of Name to Integer"))
  (set `self.CurrentCharEquipList` CurrentCharEquipList)
  (set `self.CurrentEquipCustomList` CurrentEquipCustomList))