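; BP_ACC_UIDP_Head is a UI data provider that supplies head item data for the character creator.
; LoadUIItemDataList builds an item identifier from each ID plus specie, maturity and gender, then queries the head DAO through the game module.
; Successful lookups pass through the game module's mapper into UI data and are returned as a list, while failed ones are skipped.
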(fn `LoadUIItemDataList`
  (params (IdList :type "Array of Integer (by ref)") (Specie :type Name) (Maturity :type "/Game/IS_CharacterCreator/Core/Data/Enum/E_ACC_Maturity Enum" :default "NewEnumerator0") (Gender :type "/Game/IS_CharacterCreator/Core/Data/Enum/E_ACC_Gender Enum" :default "NewEnumerator0") (Type :type Name))
  (returns (UIItemList :type "Array of /Game/IS_CharacterCreator/Core/Data/Struct/UI/FStruct_ACC_UI_Item Structure"))
  (locals (TmpData :type "Array of /Game/IS_CharacterCreator/Core/Data/Struct/UI/FStruct_ACC_UI_Item Structure"))
  (for _array_element IdList
    (bind (_headdata _success) (`/Game/IS_CharacterCreator/Core/Object/DAO/BP_ACC_DAO_Head.GetHeadData` (`/Game/IS_CharacterCreator/Core/Object/DAO/BP_ACC_DAO.GetDAOHead` (`/Game/IS_CharacterCreator/Core/Object/BP_ACC_Game.GetDAO` (`self.GetGameModule`))) (`/Game/IS_CharacterCreator/Core/Object/Module/BP_ACC_Utilities.BuildItemIdentifier` (`/Game/IS_CharacterCreator/Core/Object/BP_ACC_Game.GetUtilities` (`self.GetGameModule`)) _array_element Specie Maturity Gender)))
    (if _success
      (`KismetArrayLibrary.Array_Add` (`local.TmpData`) (`/Game/IS_CharacterCreator/Core/Object/Module/BP_ACC_Mapper.MapHeadToUI` (`/Game/IS_CharacterCreator/Core/Object/BP_ACC_Game.GetMapper` (`self.GetGameModule`)) _headdata))))
  ;[0 1 0.4844] Return all data
  (return (`local.TmpData`)))