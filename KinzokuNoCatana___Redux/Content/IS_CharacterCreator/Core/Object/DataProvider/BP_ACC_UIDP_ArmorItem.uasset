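; BP_ACC_UIDP_ArmorItem is a UI data provider for armor items in the character creator.
; Its LoadUIItemDataList function asks the game module's item DAO for items matching an ID list, specie, maturity and gender.
; It converts each result to UI data through the game module's mapper and returns the list.
; The Type parameter is not used.
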(fn `LoadUIItemDataList`
  (params (IdList :type "Array of Integer (by ref)") (Specie :type Name) (Maturity :type "/Game/IS_CharacterCreator/Core/Data/Enum/E_ACC_Maturity Enum" :default "NewEnumerator0") (Gender :type "/Game/IS_CharacterCreator/Core/Data/Enum/E_ACC_Gender Enum" :default "NewEnumerator0") (Type :type Name))
  (returns (UIItemList :type "Array of /Game/IS_CharacterCreator/Core/Data/Struct/UI/FStruct_ACC_UI_Item Structure"))
  (locals (Tmp_UIItemList :type "Array of /Game/IS_CharacterCreator/Core/Data/Struct/UI/FStruct_ACC_UI_Item Structure"))
  (bind _itemlist (`/Game/IS_CharacterCreator/Core/Object/DAO/BP_ACC_DAO_Item.GetACCItemFromIds` (`/Game/IS_CharacterCreator/Core/Object/DAO/BP_ACC_DAO.GetDAOItem` (`/Game/IS_CharacterCreator/Core/Object/BP_ACC_Game.GetDAO` (`self.GetGameModule`))) IdList Specie Maturity Gender true))
  (for _array_element _itemlist
    (`KismetArrayLibrary.Array_Add` (`local.Tmp_UIItemList`) (`/Game/IS_CharacterCreator/Core/Object/Module/BP_ACC_Mapper.MapItemDataToUI` (`/Game/IS_CharacterCreator/Core/Object/BP_ACC_Game.GetMapper` (`self.GetGameModule`)) _array_element)))
  (return (`local.Tmp_UIItemList`)))