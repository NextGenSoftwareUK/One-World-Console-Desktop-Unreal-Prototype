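; Character creator data provider that builds the list of pose items for the UI.
; LoadUIItemDataList looks up each requested ID through the advanced DAO, filtered by specie, maturity and gender.
; Poses that exist are converted to UI data by the game module's mapper, while missing ones are skipped and the Type input is unused.
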(fn `LoadUIItemDataList`
  (params (IdList :type "Array of Integer (by ref)") (Specie :type Name) (Maturity :type "/Game/IS_CharacterCreator/Core/Data/Enum/E_ACC_Maturity Enum" :default "NewEnumerator0") (Gender :type "/Game/IS_CharacterCreator/Core/Data/Enum/E_ACC_Gender Enum" :default "NewEnumerator0") (Type :type Name))
  (returns (UIItemList :type "Array of /Game/IS_CharacterCreator/Core/Data/Struct/UI/FStruct_ACC_UI_Item Structure"))
  (locals (Tmp_UIItemList :type "Array of /Game/IS_CharacterCreator/Core/Data/Struct/UI/FStruct_ACC_UI_Item Structure"))
  (for _array_element IdList
    ;[1 0 0.9844] If don't find ,try with "cmn"
    (bind (_pose _exist) (`/Game/IS_CharacterCreator/Core/Object/DAO/BP_ACC_DAO_Advanced.GetPoseAdvanced` (`/Game/IS_CharacterCreator/Core/Object/DAO/BP_ACC_DAO.GetDAOAdvanced` (`/Game/IS_CharacterCreator/Core/Object/BP_ACC_Game.GetDAO` (`self.GetGameModule`))) _array_element Specie Maturity Gender))
    (if _exist
      (`KismetArrayLibrary.Array_Add` (`local.Tmp_UIItemList`) (`/Game/IS_CharacterCreator/Core/Object/Module/BP_ACC_Mapper.MapPoseDataToUI` (`/Game/IS_CharacterCreator/Core/Object/BP_ACC_Game.GetMapper` (`self.GetGameModule`)) _pose))))
  ;[0.4766 1 0] Finally return
  (return (`local.Tmp_UIItemList`)))