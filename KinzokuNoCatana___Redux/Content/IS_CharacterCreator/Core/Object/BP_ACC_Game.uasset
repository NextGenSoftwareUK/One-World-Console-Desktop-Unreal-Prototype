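; BP_ACC_Game is the root game module object of the character creator, creating and exposing its subsystems.
; InitModule constructs the constants, gameplay, utilities, mapper, DAO and data provider manager objects, passing itself as GameModule to each.
; Only the gameplay and DAO objects receive their own InitModule call.
; Getters expose each subsystem and the stored GameInstance, with example classes filling the constants and DAO roles.
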(fn `GetConstante`
  (returns (Constante :type "/Game/IS_CharacterCreator/Core/Object/Module/BP_ACC_Constante Object Reference"))
  (return (`self.Constante`)))

(fn `GetDAO`
  (returns (DAO :type "/Game/IS_CharacterCreator/Core/Object/DAO/BP_ACC_DAO Object Reference"))
  (return (`self.DAO`)))

(fn `GetDataProviderManager`
  (returns (DataProviderManager :type "/Game/IS_CharacterCreator/Core/Object/Module/BP_ACC_DataProviderManager Object Reference"))
  (return (`self.DataProviderManager`)))

(fn `GetGameInstance`
  (returns (GameInstance :type "GameInstance Object Reference"))
  (return (`self.GameInstance`)))

(fn `GetGameplay`
  (returns (Gameplay :type "/Game/IS_CharacterCreator/Core/Object/Module/BP_ACC_Gameplay Object Reference"))
  (return (`self.Gameplay`)))

(fn `GetMapper`
  (returns (Mapper :type "/Game/IS_CharacterCreator/Core/Object/Module/BP_ACC_Mapper Object Reference"))
  (return (`self.Mapper`)))

(fn `GetUtilities`
  (returns (Utilities :type "/Game/IS_CharacterCreator/Core/Object/Module/BP_ACC_Utilities Object Reference"))
  (return (`self.Utilities`)))

(fn `InitModule`
  (`|ExecutionSequence`
    (:`then_0`
      ;[0 1 0.8359] Constante init
      (bind _returnvalue (`|GenericCreateObject` self "/Game/IS_CharacterCreator/Core/Object/Impl/BP_ACC_Constante_Example.BP_ACC_Constante_Example_C" self))
      (set `self.Constante` _returnvalue)
      ;[1 0.375 0] Construct acc gameplay
      (bind _returnvalue_2 (`|GenericCreateObject` self "/Game/IS_CharacterCreator/Core/Object/Module/BP_ACC_Gameplay.BP_ACC_Gameplay_C" self))
      (bind _output_get (set `self.Gameplay` _returnvalue_2))
      (`/Game/IS_CharacterCreator/Core/Object/Module/BP_ACC_Module.InitModule` _output_get)
      ;[1 0.5156 0] Utilities
      (bind _returnvalue_3 (`|GenericCreateObject` self "/Game/IS_CharacterCreator/Core/Object/Module/BP_ACC_Utilities.BP_ACC_Utilities_C" self))
      (set `self.Utilities` _returnvalue_3))
    (:`then_1`
      ;[0.875 1 0] Mapper
      (bind _returnvalue_4 (`|GenericCreateObject` self "/Game/IS_CharacterCreator/Core/Object/Module/BP_ACC_Mapper.BP_ACC_Mapper_C" self))
      (set `self.Mapper` _returnvalue_4)
      ;[1 0 0.2344] DAO
      (bind _returnvalue_5 (`|GenericCreateObject` self "/Game/IS_CharacterCreator/Core/Object/DAO/BP_ACC_DAO_Exemple.BP_ACC_DAO_Exemple_C" self))
      (bind _output_get_2 (set `self.DAO` _returnvalue_5))
      (`/Game/IS_CharacterCreator/Core/Object/Module/BP_ACC_Module.InitModule` _output_get_2)
      ;[0 1 0.5078] DataProvider Manager
      (bind _returnvalue_6 (`|GenericCreateObject` self "/Game/IS_CharacterCreator/Core/Object/Module/BP_ACC_DataProviderManager.BP_ACC_DataProviderManager_C" self))
      (set `self.DataProviderManager` _returnvalue_6))))