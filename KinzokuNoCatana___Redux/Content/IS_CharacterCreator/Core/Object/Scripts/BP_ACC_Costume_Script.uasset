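; Costume script for the character creator that hides a set of equipment parts while it is active on a character.
; OnEnter and OnLeave call the parent, cast the caster to BP_ACC_MCC_Equip, then hide or show the parts through SetEquipPartsVisible.
; That helper looks up each HiddentParts key on the equip object and toggles the found item's visibility.
; Leaving sets those parts visible without saving their earlier state.
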(fn `OnEnter`
  (params (Caster :type "Object Object Reference"))
  (`parent.OnEnter` Caster)
  ;[0 1 0.2266] Hide all No-Costume parts
  (bind _asbp_acc_mcc_equip (cast `/Game/IS_CharacterCreator/Core/Component/BP_ACC_MCC_Equip` Caster))
  (`self.SetEquipPartsVisible` false _asbp_acc_mcc_equip))

(fn `OnLeave`
  (params (Caster :type "Object Object Reference"))
  (`parent.OnLeave` Caster)
  ;[0 1 0.2266] Restore all No-Costume visiblity parts
  (bind _asbp_acc_mcc_equip (cast `/Game/IS_CharacterCreator/Core/Component/BP_ACC_MCC_Equip` Caster))
  (`self.SetEquipPartsVisible` true _asbp_acc_mcc_equip))

(fn `SetEquipPartsVisible`
  (params (Visible :type Boolean) (Target :type "/Game/IS_CharacterCreator/Core/Component/BP_ACC_MCC_Equip Object Reference"))
  (for _array_element (`self.HiddentParts`)
    (bind (_success _item) (`/Game/IS_CharacterCreator/Core/Component/BP_ACC_MCC_Equip.GetEquipementFromKey` Target _array_element))
    (if _success
      (`/Game/IS_CharacterCreator/Core/Item/BP_ACC_Item.SetVisibility` _item Visible))))