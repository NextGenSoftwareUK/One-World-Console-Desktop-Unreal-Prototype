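; BP_ACC_Mapper converts character creator data entries (hair, head, item and pose) into the shared FStructACCUIItem struct for UI display.
; Each type has its own mapping function that copies its ID and icon and sets a label.
; Hair and head labels are generated from the ID with format text, while item and pose labels come from the entry's name.
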(fn `MapHairToUI`
  (params (HairData :type "/Game/IS_CharacterCreator/Core/Data/Struct/Customization/FStruct_ACC_HairData Structure"))
  (returns (UIData :type "/Game/IS_CharacterCreator/Core/Data/Struct/UI/FStruct_ACC_UI_Item Structure"))
  (bind (_hairid _icon) (break `/Game/IS_CharacterCreator/Core/Data/Struct/Customization/FStruct_ACC_HairData` HairData))
  (return (make `/Game/IS_CharacterCreator/Core/Data/Struct/UI/FStruct_ACC_UI_Item` _hairid (`|FormatText` "Hair {id}" _hairid) _icon)))

(fn `MapHeadToUI`
  (params (HeadData :type "/Game/IS_CharacterCreator/Core/Data/Struct/Customization/FStruct_ACC_HeadData Structure"))
  (returns (UIData :type "/Game/IS_CharacterCreator/Core/Data/Struct/UI/FStruct_ACC_UI_Item Structure"))
  (bind (_id _icon) (break `/Game/IS_CharacterCreator/Core/Data/Struct/Customization/FStruct_ACC_HeadData` HeadData))
  (return (make `/Game/IS_CharacterCreator/Core/Data/Struct/UI/FStruct_ACC_UI_Item` _id (`|FormatText` "Head {id}" _id) _icon)))

(fn `MapItemDataToUI`
  (params (ItemData :type "/Game/IS_CharacterCreator/Core/Data/Struct/Common/FStruct_ACC_ItemData Structure"))
  (returns (UIData :type "/Game/IS_CharacterCreator/Core/Data/Struct/UI/FStruct_ACC_UI_Item Structure"))
  (bind (_itemid _name _priority _icon) (break `/Game/IS_CharacterCreator/Core/Data/Struct/Common/FStruct_ACC_ItemData` ItemData))
  (return (make `/Game/IS_CharacterCreator/Core/Data/Struct/UI/FStruct_ACC_UI_Item` _itemid _name _icon)))

(fn `MapPoseDataToUI`
  (params (ItemData :type "/Game/IS_CharacterCreator/Core/Data/Struct/Customization/FStruct_ACC_Pose Structure"))
  (returns (UIData :type "/Game/IS_CharacterCreator/Core/Data/Struct/UI/FStruct_ACC_UI_Item Structure"))
  (bind (_id _name _icon) (break `/Game/IS_CharacterCreator/Core/Data/Struct/Customization/FStruct_ACC_Pose` ItemData))
  (return (make `/Game/IS_CharacterCreator/Core/Data/Struct/UI/FStruct_ACC_UI_Item` _id (`KismetTextLibrary.Conv_NameToText` _name) _icon)))