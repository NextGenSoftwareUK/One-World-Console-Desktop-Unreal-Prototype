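; BP_ACC_Gameplay is the gameplay module of the character creator, owning an MCC edition object and running gameplay scripts on a caster.
; InitModule runs the parent setup, then constructs the edition object that GetMCCEdition exposes.
; PerformScript calls OnEnter or OnLeave on a script according to the Active flag.
; GetScriptInstance lazily creates and caches one instance per script class, so later calls reuse the same object.
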(fn `GetMCCEdition`
  (returns (MCCEdition :type "/Game/IS_CharacterCreator/Core/Object/Module/BP_ACC_MCCEdition Object Reference"))
  (return (`self.MCCEdition`)))

(fn `GetScriptInstance`
  (params (ScriptClass :type "/Game/IS_CharacterCreator/Core/Object/Scripts/BP_ACC_Script Class Reference"))
  (returns (ReturnValue :type "/Game/IS_CharacterCreator/Core/Object/Scripts/BP_ACC_Script Object Reference"))
  (for _array_element (`self.Scripts`)
    (if (== (`GameplayStatics.GetObjectClass` _array_element) ScriptClass)
      (return _array_element)))
  (bind _returnvalue (`|GenericCreateObject` ScriptClass))
  (`KismetArrayLibrary.Array_Add` (`self.Scripts`) _returnvalue)
  (return _returnvalue))

(fn `InitModule`
  (`parent.InitModule`)
  (bind _returnvalue (`|GenericCreateObject` self "/Game/IS_CharacterCreator/Core/Object/Module/BP_ACC_MCCEdition.BP_ACC_MCCEdition_C"))
  (set `self.MCCEdition` _returnvalue))

(fn `PerformScript`
  (params (Caster :type "Object Object Reference") (ScriptClass :type "/Game/IS_CharacterCreator/Core/Object/Scripts/BP_ACC_Script Class Reference") (bActive :type Boolean))
  (bind _returnvalue (`self.GetScriptInstance` ScriptClass))
  (if bActive
    (`/Game/IS_CharacterCreator/Core/Object/Scripts/BP_ACC_Script.OnEnter` _returnvalue Caster)
    (else
      (`/Game/IS_CharacterCreator/Core/Object/Scripts/BP_ACC_Script.OnLeave` _returnvalue Caster))))