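; BP_ACC_MCCEdition is a character creator module that tracks which MCC is currently being edited, along with the current edit action mode.
; Setting a new MCC unbinds the param change event from the previous one, stores the new one and binds to it.
; Param changes from the active MCC are relayed through the module's own OnMCCParamChange call.
; A helper getter returns the current MCC cast to BP_ACC_MCC_Equip.
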(fn `GetActionMode`
  (returns (bActionEdit :type Boolean))
  (return (`self.bActionEdit`)))

(fn `GetCurrentMCCEdition`
  (returns (CurrentMCCEdition :type "/Game/IS_CharacterCreator/Core/Component/BP_ACC_MCC_Base Object Reference"))
  (return (`self.CurrentMCCEdition`)))

(fn `GetCurrentMCCEquip`
  (returns (MCCEquip :type "/Game/IS_CharacterCreator/Core/Component/BP_ACC_MCC_Equip Object Reference"))
  (bind _asbp_acc_mcc_equip (cast `/Game/IS_CharacterCreator/Core/Component/BP_ACC_MCC_Equip` (`self.GetCurrentMCCEdition`)))
  (return _asbp_acc_mcc_equip))

(fn `OnMCCChange`
  (add `/Game/IS_CharacterCreator/Core/Component/BP_ACC_MCC_Base.OnParamChange` (`self.GetCurrentMCCEdition`) (`|CreateDelegate` :!event `OnParamChange`)))

(fn `OnParamChange`
  (params (ParamName :type Name))
  (`self.OnMCCParamChange` ParamName))

(fn `SetActionMode`
  (params (bActionEdit :type Boolean))
  (set `self.bActionEdit` bActionEdit))

(fn `SetCurrentMCCEdition`
  (params (MCC :type "/Game/IS_CharacterCreator/Core/Component/BP_ACC_MCC_Base Object Reference"))
  (bind _currentmccedition (`self.CurrentMCCEdition`))
  (`|ExecutionSequence`
    (:`then_0`
      ;[0 0.03906 1] Unbind old if exist
      (`/Engine/EditorBlueprintResources/StandardMacros.IsValid` _currentmccedition
        (:`Is Valid`
          (remove `/Game/IS_CharacterCreator/Core/Component/BP_ACC_MCC_Base.OnParamChange` _currentmccedition (`|CreateDelegate` :!event `OnParamChange`)))))
    (:`then_1`
      (set `self.CurrentMCCEdition` MCC)
      (`self.OnMCCChange`))))