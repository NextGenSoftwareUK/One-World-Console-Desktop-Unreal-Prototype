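; BP_ACC_Constante is a constants module for the character creator that resolves lookup keys.
; Getters read map variables for hair type, parameter, maturity and gender keys, returning the value found for the given key.
; Body, head and hair shortcuts call GetKeyParam with hardcoded names, so callers need not pass those key strings.
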(fn `GetBodyParamKeys`
  (returns (Value :type Name))
  (return (`self.GetKeyParam` "BodyParamsKey")))

(fn `GetGenderKey`
  (params (Gender :type "/Game/IS_CharacterCreator/Core/Data/Enum/E_ACC_Gender Enum" :default "NewEnumerator0"))
  (returns (Value :type Name))
  (return (`BlueprintMapLibrary.Map_Find` (`self.GenderKeyList`) Gender)))

(fn `GetHairKeyFromType`
  (params (Key :type "/Game/IS_CharacterCreator/Core/Data/Enum/E_ACC_HairType Enum" :default "NewEnumerator0"))
  (returns (Value :type Name))
  (return (`BlueprintMapLibrary.Map_Find` (`self.HairKeyList`) Key)))

(fn `GetHairParamKeys`
  (returns (Value :type Name))
  (return (`self.GetKeyParam` "HairParamsKey")))

(fn `GetHeadParamKeys`
  (returns (Value :type Name))
  (return (`self.GetKeyParam` "HeadParamsKey")))

(fn `GetKeyParam`
  (params (Key :type Name))
  (returns (Value :type Name))
  (return (`BlueprintMapLibrary.Map_Find` (`self.KeyParamList`) Key)))

(fn `GetMaturityKey`
  (params (Key :type "/Game/IS_CharacterCreator/Core/Data/Enum/E_ACC_Maturity Enum" :default "NewEnumerator0"))
  (returns (Value :type Name))
  (return (`BlueprintMapLibrary.Map_Find` (`self.MaturityKeyList`) Key)))