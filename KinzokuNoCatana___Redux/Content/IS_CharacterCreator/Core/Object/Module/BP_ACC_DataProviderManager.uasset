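; BP_ACC_DataProviderManager is a character creator module object that hands out UI data providers by class.
; GetUIDataProvider returns the cached provider from DataProviderList, cast to BP_ACC_UIDataProvider, or constructs one with the game module and stores it, keeping one instance per class.
; GetDataProvider is a plain map lookup that also reports existence, and GetConstante forwards the constants from the game module.
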(fn `GetConstante`
  (returns (Constante :type "/Game/IS_CharacterCreator/Core/Object/Module/BP_ACC_Constante Object Reference"))
  (return (`/Game/IS_CharacterCreator/Core/Object/BP_ACC_Game.GetConstante` (`self.GetGameModule`))))

(fn `GetDataProvider`
  (params (Class :type "/Game/IS_CharacterCreator/Core/Object/DataProvider/BP_ACC_DataProvider Class Reference (by ref)"))
  (returns (Value :type "/Game/IS_CharacterCreator/Core/Object/DataProvider/BP_ACC_DataProvider Object Reference") (Exist :type Boolean))
  (bind (_value _returnvalue) (`BlueprintMapLibrary.Map_Find` (`self.DataProviderList`) Class))
  (return _value _returnvalue))

(fn `GetUIDataProvider`
  (params (Class :type "/Game/IS_CharacterCreator/Core/Object/DataProvider/BP_ACC_UIDataProvider Class Reference (by ref)"))
  (returns (DataProvider :type "/Game/IS_CharacterCreator/Core/Object/DataProvider/BP_ACC_UIDataProvider Object Reference"))
  (bind (_value _exist) (`self.GetDataProvider` Class))
  (if _exist
    (bind _asbp_acc_uidata_provider (cast `/Game/IS_CharacterCreator/Core/Object/DataProvider/BP_ACC_UIDataProvider` _value))
    (return _asbp_acc_uidata_provider)
    (else
      ;[0.8516 0 1] Else create one and return (singleton pattern)
      (bind _returnvalue (`|GenericCreateObject` self Class (`self.GetGameModule`)))
      (`BlueprintMapLibrary.Map_Add` (`self.DataProviderList`) Class _returnvalue)
      (return _returnvalue))))