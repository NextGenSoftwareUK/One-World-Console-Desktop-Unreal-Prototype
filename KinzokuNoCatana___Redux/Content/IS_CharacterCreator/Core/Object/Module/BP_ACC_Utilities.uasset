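; Character creator utility module that builds the Name keys identifying items and hair by species, maturity and gender.
; Identifiers are formatted from maturity and gender keys looked up in the game module's constants, plus an ID or other suffix.
; One variant also returns a common-gender identifier, and the hair builder ignores its HairType input.
; A side-key helper trims keys matching one hair type's prefix to two characters.
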(fn `BuildHairIdentifier`
  (params (Specie :type Name) (Maturity :type "/Game/IS_CharacterCreator/Core/Data/Enum/E_ACC_Maturity Enum" :default "NewEnumerator0") (Gender :type "/Game/IS_CharacterCreator/Core/Data/Enum/E_ACC_Gender Enum" :default "NewEnumerator0") (HairId :type Integer) (HairType :type Name))
  (returns (Identifier :type Name))
  (return (`self.BuildItemIdentifier` HairId Specie Maturity Gender)))

(fn `BuildHairSideKey`
  (params (Key :type Name))
  (returns (Value :type Name))
  (bind _returnvalue (`KismetStringLibrary.Conv_NameToString` Key))
  (return (select `bool` (`KismetStringLibrary.StartsWith` _returnvalue (`KismetStringLibrary.Conv_NameToString` (`/Game/IS_CharacterCreator/Core/Object/Module/BP_ACC_Constante.GetHairKeyFromType` (`self.GetConstante`) "NewEnumerator5"))) :`false` Key :`true` (`KismetStringLibrary.Conv_StringToName` (`KismetStringLibrary.GetSubstring` _returnvalue 0 2)))))

(fn `BuildItemIdentifier`
  (params (Id :type Integer) (Specie :type Name) (Maturity :type "/Game/IS_CharacterCreator/Core/Data/Enum/E_ACC_Maturity Enum" :default "NewEnumerator0") (Gender :type "/Game/IS_CharacterCreator/Core/Data/Enum/E_ACC_Gender Enum" :default "NewEnumerator0"))
  (returns (Identifier :type Name))
  (bind _constante (`/Game/IS_CharacterCreator/Core/Object/BP_ACC_Game.GetConstante` (`self.GetGameModule`)))
  (return (`self.TextToName` (`|FormatText` "{specie}_{maturity}_{gender}_{id}" Specie (`/Game/IS_CharacterCreator/Core/Object/Module/BP_ACC_Constante.GetMaturityKey` _constante Maturity) (`/Game/IS_CharacterCreator/Core/Object/Module/BP_ACC_Constante.GetGenderKey` _constante Gender) Id))))

(fn `BuildItemIdentifierAndCmn`
  (params (Id :type Integer) (Specie :type Name) (Maturity :type "/Game/IS_CharacterCreator/Core/Data/Enum/E_ACC_Maturity Enum" :default "NewEnumerator0") (Gender :type "/Game/IS_CharacterCreator/Core/Data/Enum/E_ACC_Gender Enum" :default "NewEnumerator0"))
  (returns (Identifier :type Name) (CmnIdentifier :type Name))
  (return (`self.BuildItemIdentifier` Id Specie Maturity Gender) (`self.BuildItemIdentifier` Id Specie Maturity "NewEnumerator2")))

(fn `BuildItemOtherIdentifier`
  (params (Specie :type Name) (Maturity :type "/Game/IS_CharacterCreator/Core/Data/Enum/E_ACC_Maturity Enum" :default "NewEnumerator0") (Gender :type "/Game/IS_CharacterCreator/Core/Data/Enum/E_ACC_Gender Enum" :default "NewEnumerator0") (Other :type Name))
  (returns (Identifier :type Name))
  (bind _constante (`/Game/IS_CharacterCreator/Core/Object/BP_ACC_Game.GetConstante` (`self.GetGameModule`)))
  (return (`self.TextToName` (`|FormatText` "{specie}_{maturity}_{gender}_{other}" Specie (`/Game/IS_CharacterCreator/Core/Object/Module/BP_ACC_Constante.GetMaturityKey` _constante Maturity) (`/Game/IS_CharacterCreator/Core/Object/Module/BP_ACC_Constante.GetGenderKey` _constante Gender) Other))))

(fn `GetConstante`
  (returns (Constante :type "/Game/IS_CharacterCreator/Core/Object/Module/BP_ACC_Constante Object Reference"))
  (return (`/Game/IS_CharacterCreator/Core/Object/BP_ACC_Game.GetConstante` (`self.GetGameModule`))))

(fn `TextToName`
  (params (Text :type "Text (by ref)"))
  (returns (ReturnValue :type Name))
  (return (`KismetStringLibrary.Conv_StringToName` (`KismetTextLibrary.Conv_TextToString` Text))))