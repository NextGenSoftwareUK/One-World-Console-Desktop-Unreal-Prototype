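; Game instance for the character creator that creates the game module and customization storage on init and loads or creates the save game.
; Saving runs asynchronously behind a wait dialog, held open by an artificial one-second delay, then notifies registered UIs that the character list changed.
; Interface functions expose the module and storage, register UIs and observers, and broadcast named events to valid observers.
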(event `self.ReceiveInit`
  (`|ExecutionSequence`
    (:`then_0`
      ;[0 1 0.01562] Game Module
      (bind _returnvalue (`|GenericCreateObject` self "/Game/IS_CharacterCreator/Core/Object/BP_ACC_Game.BP_ACC_Game_C" self))
      (bind _output_get (set `self.ACCGameModule` _returnvalue))
      (`/Game/IS_CharacterCreator/Core/Object/BP_ACC_Game.InitModule` _output_get))
    (:`then_1`
      ;[1 0.2578 0] On Game Instance Init
      (`self.LoadSaveGame`)
      (bind _returnvalue_2 (`|GenericCreateObject` self "/Game/IS_CharacterCreator/Core/Object/BP_ACC_CustomizationStorage.BP_ACC_CustomizationStorage_C" self))
      (bind _output_get_2 (set `self.CustomizationStorage` _returnvalue_2))
      (`/Game/IS_CharacterCreator/Core/Object/BP_ACC_CustomizationStorage.Init` _output_get_2))))

(event `SaveACCGame`
  ;[0.7344 0 1] Save in save game and simule fake delay
  (`self.DialogAction` "Saving Process..." true)
  (`AsyncActionHandleSaveGame.AsyncSaveGameToSlot` (`self.GetSaveGame`) (`self.SaveGameSlot`) (`self.UserIndex`)
    (:`Completed`
      (`KismetSystemLibrary.Delay` 1.0) ; Fake wait
      (`self.DialogAction` "") ; Close Dialog
      ;[0.3594 1 0] Notify To All of Resgistred UI the character list change
      (for _array_element (`self.MainUIList`)
        (message `/Game/IS_CharacterCreator/Core/Interface/BPI_ACC_GameEvent.I_OnCharacterListChanged` _array_element)))))

(event `/Game/IS_CharacterCreator/Core/Interface/BPI_ACC_GameInstance.I_GI_AddUI`
  (params (UI :type "UserWidget Object Reference"))
  ;[1 0.8906 0] Add UI(UMG) in UI List
  (`KismetArrayLibrary.Array_Add` (`self.MainUIList`) UI))

(event `/Game/IS_CharacterCreator/Core/Interface/BPI_ACC_GameInstance.I_GI_AddEventObservable`
  (params (Object :type "Object Object Reference"))
  (`KismetArrayLibrary.Array_AddUnique` (`self.EventObservable`) Object))

(event `/Game/IS_CharacterCreator/Core/Interface/BPI_ACC_GameInstance.I_GI_SendEvent`
  (params (EventName :type Name))
  (for _array_element (`self.EventObservable`)
    (`/Engine/EditorBlueprintResources/StandardMacros.IsValid` _array_element
      (:`Is Valid`
        (message `/Game/IS_CharacterCreator/Core/Interface/BPI_ACC_GameEvent.I_OnEvent` _array_element EventName)))))

(fn `DialogAction`
  (params (DialogMessage :type Text) (ActiveDialog :type Boolean))
  (if ActiveDialog
    ;[1 1 1] Open Dialog
    (bind _returnvalue (`|CreateWidget` "/Game/IS_CharacterCreator/Core/Widget/Components/Dialog/WBP_ACC_Dialog_Wait.WBP_ACC_Dialog_Wait_C"))
    (`UserWidget.AddToViewport` _returnvalue 0)
    (set `self.CurrentDialog` _returnvalue)
    (`/Game/IS_CharacterCreator/Core/Widget/Components/Dialog/WBP_ACC_Dialog_Wait.OpenDialog` _returnvalue DialogMessage)
    (else
      ;[1 1 1] Close Dialog
      (`Widget.RemoveFromParent` (`self.CurrentDialog`)))))

(fn `GetSaveGame`
  (returns (SaveGameInstance :type "/Game/IS_CharacterCreator/Core/BP_ACC_SaveGame Object Reference"))
  (return (`self.SaveGameInstance`)))

(fn `I_GI_GetACCGameModule`
  (returns (GameModule :type "/Game/IS_CharacterCreator/Core/Object/BP_ACC_Game Object Reference"))
  (return (`self.ACCGameModule`)))

(fn `I_GI_GetACCStorage`
  (returns (ACCStorage :type "/Game/IS_CharacterCreator/Core/Object/BP_ACC_CustomizationStorage Object Reference"))
  (return (`self.CustomizationStorage`)))

(fn `LoadSaveGame`
  ;[1 1 1] Try to load existed save game
  (bind _returnvalue (`GameplayStatics.LoadGameFromSlot` (`self.SaveGameSlot`) (`self.UserIndex`)))
  (bind _asbp_acc_save_game (cast `/Game/IS_CharacterCreator/Core/BP_ACC_SaveGame` _returnvalue)
    (:`then`
      (set `self.SaveGameInstance` _asbp_acc_save_game))
    (:`CastFailed`
      ;[1 1 1] If not exist create one
      (bind _returnvalue_2 (`GameplayStatics.CreateSaveGameObject` "/Game/IS_CharacterCreator/Core/BP_ACC_SaveGame.BP_ACC_SaveGame_C"))
      (set `self.SaveGameInstance` _returnvalue_2))))