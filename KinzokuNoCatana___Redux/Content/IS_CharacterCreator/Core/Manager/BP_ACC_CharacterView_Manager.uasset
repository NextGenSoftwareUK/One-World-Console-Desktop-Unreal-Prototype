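; Manager actor that shows a preview of a character creator character and switches the player's view to it.
; On activation it replaces any existing preview actor with the species' preview Blueprint from the ACC DAO, spawned at its own transform and rotated.
; It blends to a camera found by tag and applies species and character data through the modular component interface.
; Deactivation returns view and input to the player.
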(fn `ActiveCharacterPreview`
  (params (ACC_Character :type "/Game/IS_CharacterCreator/Core/Data/Struct/FStruct_ACC_Character Structure"))
  (set `self.ACC_Character` ACC_Character)
  (`self.SpawnCharacterPreview`)
  (`self.SwitchCamera`)
  (bind _modularcharcomp (message `/Game/IS_CharacterCreator/Core/Interface/BPI_ACC_CharacterCustomization.I_GetModularComp` (`self.GetCharacterPreview`)))
  (`/Game/IS_CharacterCreator/Core/Component/BP_ACC_MCC_Base.ChangeSpecie` _modularcharcomp (`.Specie_35_2B7BBCA6419FE018D0239486B86E5365` (break `/Game/IS_CharacterCreator/Core/Data/Struct/Customization/FStruct_ACC_CharacterCustom` (`.CharCustom_2_185AFF684768515E4FE853A48612311C` (break `/Game/IS_CharacterCreator/Core/Data/Struct/FStruct_ACC_Character` (`self.ACC_Character`))))))
  (`/Game/IS_CharacterCreator/Core/Component/BP_ACC_MCC_Base.InitDefaultSetUp` _modularcharcomp)
  (`/Game/IS_CharacterCreator/Core/Component/BP_ACC_MCC_Base.InitFromACCCharData` _modularcharcomp (`self.ACC_Character`)))

(fn `GetCamera`
  (returns (Output :type "Actor Object Reference"))
  (bind _outactors (`GameplayStatics.GetAllActorsWithTag` "CharPreview_Camera"))
  (return (`|GetArrayItem` _outactors)))

(fn `GetCharacterPreview`
  (returns (Output :type "Actor Object Reference"))
  (return (`self.CharacterPreview`)))

(fn `SpawnCharacterPreview`
  (bind _characterpreview (`self.CharacterPreview`))
  (`|ExecutionSequence`
    (:`then_0`
      ;[0 0.01562 1] Remove if exist already
      (`/Engine/EditorBlueprintResources/StandardMacros.IsValid` _characterpreview
        (:`Is Valid`
          (`self.K2_DestroyActor` _characterpreview))))
    (:`then_1`
      (bind _returnvalue (`|SpawnActorFromClass` (`.PreviewBP_2_EBEBC5F347811729A30630A64A1F1E54` (break `/Game/IS_CharacterCreator/Core/Data/Struct/FStruct_ACC_CustomConfParam` (`.CustomConf_16_9952A7684B7AF3A6E39087B165AB2F7F` (break `/Game/IS_CharacterCreator/Core/Data/Struct/FStruct_ACC_SpecieParam` (`/Game/IS_CharacterCreator/Core/Object/DAO/BP_ACC_DAO.GetSpecie` (`/Game/IS_CharacterCreator/Core/Library/BPFL_ACC_Common.GetACCDAO`) (`.Specie_35_2B7BBCA6419FE018D0239486B86E5365` (break `/Game/IS_CharacterCreator/Core/Data/Struct/Customization/FStruct_ACC_CharacterCustom` (`.CharCustom_2_185AFF684768515E4FE853A48612311C` (break `/Game/IS_CharacterCreator/Core/Data/Struct/FStruct_ACC_Character` (`self.ACC_Character`)))))))))) (`self.GetTransform`) "Undefined" "OverrideRootScale" null null))
      (bind _output_get (set `self.CharacterPreview` _returnvalue))
      (`self.K2_AddActorLocalRotation` _output_get (struct :`Yaw` -90.0) false false))))

(fn `SwitchCamera`
  (`PlayerController.SetViewTargetWithBlend` (`GameplayStatics.GetPlayerController` 0) (`self.GetCamera`) 0.0 "VTBlend_Linear" 0.0 false))

(fn `UnactiveCharacterPreview`
  (`PlayerController.SetViewTargetWithBlend` (`GameplayStatics.GetPlayerController` 0) (`GameplayStatics.GetPlayerCharacter` 0) 0.0 "VTBlend_Linear" 0.0 false)
  (`WidgetBlueprintLibrary.SetInputMode_GameAndUIEx` (`GameplayStatics.GetPlayerController` 0) null))

(fn `UserConstructionScript`)