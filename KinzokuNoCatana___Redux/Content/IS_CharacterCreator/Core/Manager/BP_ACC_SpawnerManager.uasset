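; Spawner manager actor for the character creator that populates the level with NPCs when play begins, on the authority only.
; It gathers every NPC spawn point actor, loads each point's character data by NPC ID through the DAO, and spawns a character of that species there.
; Each spawned character is set to look at the player, gets its modular setup, then receives its appearance as net-mapped data.
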(event `self.ReceiveBeginPlay`
  (`parent.ReceiveBeginPlay`)
  (`/Engine/EditorBlueprintResources/ActorMacros.Switch Has Authority`
    (:`Authority`
      (`self.Server_SpawnRandomNPC`))))

(event `Server_SpawnRandomNPC`
  (`self.InitSpawnPointList`)
  (`self.SpawnFromPointList`))

(fn `InitSpawnPointList`
  (bind _outactors (`GameplayStatics.GetAllActorsOfClass` "/Game/IS_CharacterCreator/Core/Utils/BP_ACC_NPC_SpawnPoint.BP_ACC_NPC_SpawnPoint_C"))
  (set `self.SpawnPointList` _outactors))

(fn `SpawnFromPointList`
  (locals (ACC_Character :type "/Game/IS_CharacterCreator/Core/Data/Struct/FStruct_ACC_Character Structure"))
  (bind _specie (break `/Game/IS_CharacterCreator/Core/Data/Struct/Customization/FStruct_ACC_CharacterCustom` (`.CharCustom_2_185AFF684768515E4FE853A48612311C` (break `/Game/IS_CharacterCreator/Core/Data/Struct/FStruct_ACC_Character` (`local.ACC_Character`)))))
  (for _array_element (`self.SpawnPointList`)
    ;[0 0.5781 1] Get NPC Data
    (bind _acc_character (`/Game/IS_CharacterCreator/Core/Object/DAO/BP_ACC_DAO_Character.GetCharacterNPCFromId` (`/Game/IS_CharacterCreator/Core/Object/DAO/BP_ACC_DAO.GetDAOCharacter` (`/Game/IS_CharacterCreator/Core/Library/BPFL_ACC_Common.GetACCDAO`)) (`/Game/IS_CharacterCreator/Core/Utils/BP_ACC_NPC_SpawnPoint.NpcId` _array_element)))
    (set `local.ACC_Character` _acc_character)
    (bind (_spawnedcharacter _success) (`self.SpawnIsCharacter` _specie (+ (`self.K2_GetActorLocation` _array_element) (0.0 0.0 90.0)) (`self.K2_GetActorRotation` _array_element)))
    (if _success
      (set `/Game/IS_CharacterCreator/Core/Character/BP_ACC_Character.bLookAtPlayer` true _spawnedcharacter)
      (bind _modularcharcomp (message `/Game/IS_CharacterCreator/Core/Interface/BPI_ACC_CharacterCustomization.I_GetModularComp` _spawnedcharacter))
      (`/Game/IS_CharacterCreator/Core/Component/BP_ACC_MCC_Base.ChangeSpecie` _modularcharcomp _specie)
      (`/Game/IS_CharacterCreator/Core/Component/BP_ACC_MCC_Base.InitDefaultSetUp` _modularcharcomp)
      (bind _acc_character_net (`/Game/IS_CharacterCreator/Core/Library/BPFL_ACC_Network.MapACC_Char_ToNet` (`local.ACC_Character`)))
      (message `/Game/IS_CharacterCreator/Core/Interface/BPI_ACC_NetChar.I_Net_InitACC_Char` _spawnedcharacter _acc_character_net))))

(fn `UserConstructionScript`
  (`parent.UserConstructionScript`))