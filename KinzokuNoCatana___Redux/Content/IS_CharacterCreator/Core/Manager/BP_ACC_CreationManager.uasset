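; Manager actor for the character creation screen, handling species, gender, maturity, colors, backgrounds and saving or removing characters.
; On BeginPlay it spawns the gyratory, camera rig and UI, then registers with the game instance.
; Edits route through the character's modular component, presets and persistence through the DAO.
; The camera interpolates to per-species socket views, preferring maturity-specific keys and refreshing on height or gender changes.
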(event `self.ReceiveBeginPlay`
  (`|ExecutionSequence`
    (:`then_0`
      ;[0 0.5547 1] Bind event
      (add `/Game/IS_CharacterCreator/Core/Object/Module/BP_ACC_MCCEdition.OnMCCParamChange` (`/Game/IS_CharacterCreator/Core/Object/Module/BP_ACC_Gameplay.GetMCCEdition` (`/Game/IS_CharacterCreator/Core/Library/BPFL_ACC_Common.GetACCGameplay`)) (`|CreateDelegate` :!event `OnMCCParamChange`)))
    (:`then_1`
      (`self.InitEssentials`)
      ;[0.6172 1 0] Registre It in game Observable Event
      (message `/Game/IS_CharacterCreator/Core/Interface/BPI_ACC_GameInstance.I_GI_AddEventObservable` (`GameplayStatics.GetGameInstance`) self)
      (`self.LogACCManager` "Ready"))))

(event `self.ReceiveTick`
  (params (DeltaSeconds :type "Float (single-precision)"))
  ;[1 0 0.6094] Tick Camera target view
  (`self.K2_SetActorLocation` (`self.ActiveCamera`) (`KismetMathLibrary.VInterpTo` (`self.K2_GetActorLocation` (`self.ActiveCamera`)) (`self.K2_GetActorLocation` (`self.CurrentTargetPoint`)) (`GameplayStatics.GetWorldDeltaSeconds`) (`self.CameraSpeed`)) false false)
  ;[0.8047 1 0] Update rotation
  (`self.K2_SetActorRotation` (`self.ActiveCamera`) (`self.K2_GetActorRotation` (`self.CurrentTargetPoint`)) false))

(event `ChangeCameraAsync`
  (params (Key :type Name) (Duration :type "Float (double-precision)"))
  ;[0.8516 1 0] Delay change camera
  (`KismetSystemLibrary.Delay` Duration)
  (`self.UpdateCameraView` Key))

(event `RefreshCameraAsync`
  (params (Duration :type "Float (double-precision)"))
  ;[0.5234 1 0] Delay Refresh Camera
  (`KismetSystemLibrary.Delay` Duration)
  (`self.RefreshCurrentTargetView`))

(event `self.ReceiveDestroyed`
  ;[0.8984 0 1] On Destroyed
  (`self.CleanAll`)
  (`self.RestoreGameControl`)
  (`parent.ReceiveDestroyed`))

(fn `ApplyParamChange`
  (params (ParamName :type Name))
  (bind _value (`self.GetCreatorParameter` ParamName))
  (switch `name` ParamName
    (:`Background`
      (`self.ChangeBackground` _value))
    (:`DisplayCircle`
      (`/Game/IS_CharacterCreator/Core/Utils/UI/BP_ACC_Gyratory_Main.SetDisplayCircle` (`self.GetGiratoryMain`) (== _value 1)))))

(fn `BuildPresetKey`
  (params (Specie :type Name) (Maturity :type "/Game/IS_CharacterCreator/Core/Data/Enum/E_ACC_Maturity Enum" :default "NewEnumerator0") (Gender :type "/Game/IS_CharacterCreator/Core/Data/Enum/E_ACC_Gender Enum" :default "NewEnumerator0"))
  (returns (ReturnValue :type Name))
  (return (`/Game/IS_CharacterCreator/Core/Library/BPFL_ACC_Common.TextToName` (`|FormatText` "{specie}_{maturity}_{gender}" Specie (`/Game/IS_CharacterCreator/Core/Library/BPFL_ACC_Constant.GetMaturityKey` Maturity) (`/Game/IS_CharacterCreator/Core/Library/BPFL_ACC_Constant.GetGenderKey` Gender)))))

(fn `ChangeBackground`
  (params (BackgroundIndex :type Integer))
  (`PrimitiveComponent.SetMaterial` (`/Game/IS_CharacterCreator/Core/Skybox/BP_ACC_Skybox.StaticMesh` (`self.GetSkybox`)) 0 (select `int` BackgroundIndex :`0` "/Game/IS_CharacterCreator/MaterialLibrary/Sky/MI_ACC_SpaceCC_01.MI_ACC_SpaceCC_01" :`1` "/Game/IS_CharacterCreator/MaterialLibrary/Sky/MI_ACC_SpaceCC_02.MI_ACC_SpaceCC_02" :!type "MaterialInterface Object Reference")))

(fn `ChangeCameraView`
  (params (Key :type Name))
  (`self.UpdateCameraView` Key))

(fn `ChangeCharacterData`
  (params (ACC_Character :type "/Game/IS_CharacterCreator/Core/Data/Struct/FStruct_ACC_Character Structure"))
  ;[0 0.3672 1] Change Specie
  (`self.ChangeSpecie` (`.Specie_35_2B7BBCA6419FE018D0239486B86E5365` (break `/Game/IS_CharacterCreator/Core/Data/Struct/Customization/FStruct_ACC_CharacterCustom` (`.CharCustom_2_185AFF684768515E4FE853A48612311C` (break `/Game/IS_CharacterCreator/Core/Data/Struct/FStruct_ACC_Character` ACC_Character)))))
  ;[1 0.9609 0] Init character parameter
  (`/Game/IS_CharacterCreator/Core/Component/BP_ACC_MCC_Base.InitFromACCCharData` (`self.GetModularComp`) (`local.ACC_Character`))
  ;[1 0 0.8437] Change TargetView
  (`self.ChangeCameraAsync` "Global" 0.05))

(fn `ChangeCurrentCharacter`
  (params (TargetCharacter :type "Actor Object Reference"))
  (bind _output_get (set `self.CustomableCharacter` TargetCharacter))
  (bind _modularcharcomp (message `/Game/IS_CharacterCreator/Core/Interface/BPI_ACC_CharacterCustomization.I_GetModularComp` _output_get))
  ;[1 0.2812 0] Change current mcc used for edition
  (`/Game/IS_CharacterCreator/Core/Object/Module/BP_ACC_MCCEdition.SetCurrentMCCEdition` (`/Game/IS_CharacterCreator/Core/Object/Module/BP_ACC_Gameplay.GetMCCEdition` (`/Game/IS_CharacterCreator/Core/Library/BPFL_ACC_Common.GetACCGameplay`)) _modularcharcomp)
  ;[0 0.5312 1] Set Rotable Actor from controller
  (bind _asbp_acc_controller (cast `/Game/IS_CharacterCreator/Core/Controller/BP_ACC_Controller` (`GameplayStatics.GetPlayerController` 0)))
  (set `/Game/IS_CharacterCreator/Core/Controller/BP_ACC_Controller.ActorToRotate` (`self.CustomableCharacter`) _asbp_acc_controller))

(fn `ChangeGender`
  (params (Gender :type "/Game/IS_CharacterCreator/Core/Data/Enum/E_ACC_Gender Enum" :default "NewEnumerator0"))
  (bind _acc_character (`/Game/IS_CharacterCreator/Core/Object/DAO/BP_ACC_DAO_Character.GetCharacterPreset` (`/Game/IS_CharacterCreator/Core/Object/DAO/BP_ACC_DAO.GetDAOCharacter` (`/Game/IS_CharacterCreator/Core/Library/BPFL_ACC_Common.GetACCDAO`)) (`self.BuildPresetKey` (`self.Specie`) (`/Game/IS_CharacterCreator/Core/Component/BP_ACC_MCC_Base.Maturity` (`self.GetModularComp`)) Gender)))
  ;[0.8984 0 1] Notify to the modular component you want change Gender
  (`/Game/IS_CharacterCreator/Core/Component/BP_ACC_MCC_Base.InitFromACCCharData` (`self.GetModularComp`) _acc_character))

(fn `ChangeItemColor`
  (params (ItemPart :type Name) (ColorIndex :type Integer) (Color :type "LinearColor Structure"))
  (`/Game/IS_CharacterCreator/Core/Component/BP_ACC_MCC_Equip.ChangeEquipItemCustom` (`self.GetModularEquipComp`) ItemPart ColorIndex Color))

(fn `ChangeMaturity`
  (params (Maturity :type "/Game/IS_CharacterCreator/Core/Data/Enum/E_ACC_Maturity Enum" :default "NewEnumerator0"))
  (`/Game/IS_CharacterCreator/Core/Component/BP_ACC_MCC_Base.ChangeMaturity` (`self.GetModularComp`) Maturity)
  ;[0 1 0.8125] Default gender
  (`self.ChangeGender` "NewEnumerator2")
  (`self.OnChangeMaturity` Maturity))

(fn `ChangeSpecie`
  (params (Identifier :type Name) (ForceNew :type Boolean))
  (bind _customablecharacter (`self.GetCharacter`))
  ;[0.7109 0 1] if new specie are difference, delete previous character
  (if (or (!= (`self.Specie`) (`local.Identifier`)) (`local.ForceNew`))
    (set `self.Specie` (`local.Identifier`))
    (`|ExecutionSequence`
      (:`then_0`
        ;[0 0.6484 1] Delete old if valid
        (`/Engine/EditorBlueprintResources/StandardMacros.IsValid` _customablecharacter
          (:`Is Valid`
            (`self.ClearCustomableCharacter`)
            (`self.K2_DestroyActor` _customablecharacter))))
      (:`then_1`
        (bind _character (`self.SpawnCustomableCharacter` (`.PreviewBP_2_EBEBC5F347811729A30630A64A1F1E54` (break `/Game/IS_CharacterCreator/Core/Data/Struct/FStruct_ACC_CustomConfParam` (`.CustomConf_16_9952A7684B7AF3A6E39087B165AB2F7F` (break `/Game/IS_CharacterCreator/Core/Data/Struct/FStruct_ACC_SpecieParam` (`/Game/IS_CharacterCreator/Core/Object/DAO/BP_ACC_DAO.GetSpecie` (`/Game/IS_CharacterCreator/Core/Library/BPFL_ACC_Common.GetACCDAO`) (`local.Identifier`))))))))
        ;[0 1 1] Apply Specie identifier to modular
        (bind _modularcharcomp (message `/Game/IS_CharacterCreator/Core/Interface/BPI_ACC_CharacterCustomization.I_GetModularComp` _character))
        (`/Game/IS_CharacterCreator/Core/Component/BP_ACC_MCC_Base.ChangeSpecie` _modularcharcomp (`local.Identifier`))
        ;[0.07812 0 1] Init Default SetUp
        (`/Game/IS_CharacterCreator/Core/Component/BP_ACC_MCC_Base.InitDefaultSetUp` _modularcharcomp)
        ;[0 0.8359 1] Default Empty Specie param
        (`self.DefaultEmptySpecie`)))))

(fn `CleanAll`
  (for _array_element (`self.GetAttachedActors` false)
    (`self.K2_DestroyActor` _array_element))
  (`self.K2_DestroyActor` (`self.GyratoryMain`))
  (`self.K2_DestroyActor` (`self.CurrentTargetPoint`)))

(fn `ClearCustomableCharacter`
  (bind _modularcharcomp (message `/Game/IS_CharacterCreator/Core/Interface/BPI_ACC_CharacterCustomization.I_GetModularComp` (`self.GetCharacter`)))
  (`/Game/IS_CharacterCreator/Core/Component/BP_ACC_MCC_Base.DestroyAll` _modularcharcomp))

(fn `CreateNewEmptyCharacter`
  (`/Game/IS_CharacterCreator/Core/Object/Module/BP_ACC_MCCEdition.SetActionMode` (`/Game/IS_CharacterCreator/Core/Object/Module/BP_ACC_Gameplay.GetMCCEdition` (`/Game/IS_CharacterCreator/Core/Library/BPFL_ACC_Common.GetACCGameplay`)) false)
  (`self.ChangeSpecie` "epic_hmn" true))

(fn `DefaultEmptySpecie`
  ;[1 0 0.4453] Default Empty Specie Character
  (bind _modularcharcomp (message `/Game/IS_CharacterCreator/Core/Interface/BPI_ACC_CharacterCustomization.I_GetModularComp` (`self.GetCharacter`)))
  (bind _acc_character (`/Game/IS_CharacterCreator/Core/Object/DAO/BP_ACC_DAO_Character.GetDefaultCharacterFromSpecie` (`/Game/IS_CharacterCreator/Core/Object/DAO/BP_ACC_DAO.GetDAOCharacter` (`/Game/IS_CharacterCreator/Core/Library/BPFL_ACC_Common.GetACCDAO`)) (`/Game/IS_CharacterCreator/Core/Component/BP_ACC_MCC_Base.SpecieIdentifier` _modularcharcomp)))
  (`/Game/IS_CharacterCreator/Core/Component/BP_ACC_MCC_Base.InitFromACCCharData` _modularcharcomp _acc_character))

(fn `GetCharacter`
  (returns (CustomableCharacter :type "Actor Object Reference"))
  (return (`self.CustomableCharacter`)))

(fn `GetCreatorParameter`
  (params (ParamName :type Name))
  (returns (Value :type Integer))
  (return (`BlueprintMapLibrary.Map_Find` (`self.GetCreatorParametersList`) ParamName)))

(fn `GetCreatorParametersList`
  (returns (CreatorParameters :type "Map of Name to Integer"))
  (return (`self.CreatorParameters`)))

(fn `GetGiratoryMain`
  (returns (GyratoryMain :type "/Game/IS_CharacterCreator/Core/Utils/UI/BP_ACC_Gyratory_Main Object Reference"))
  (return (`self.GyratoryMain`)))

(fn `GetModularComp`
  (returns (ModularCharacter :type "/Game/IS_CharacterCreator/Core/Component/BP_ACC_MCC_Base Object Reference"))
  (bind _modularcharcomp (message `/Game/IS_CharacterCreator/Core/Interface/BPI_ACC_CharacterCustomization.I_GetModularComp` (`self.GetCharacter`)))
  (return _modularcharcomp))

(fn `GetModularEquipComp`
  (returns (ModularCharacter :type "/Game/IS_CharacterCreator/Core/Component/BP_ACC_MCC_Equip Object Reference"))
  (bind _asbp_acc_mcc_equip (cast `/Game/IS_CharacterCreator/Core/Component/BP_ACC_MCC_Equip` (`self.GetModularComp`)))
  (return _asbp_acc_mcc_equip))

(fn `GetSkybox`
  (returns (Skybox :type "/Game/IS_CharacterCreator/Core/Skybox/BP_ACC_Skybox Object Reference"))
  (bind _outactors (`GameplayStatics.GetAllActorsOfClass` "/Game/IS_CharacterCreator/Core/Skybox/BP_ACC_Skybox.BP_ACC_Skybox_C"))
  (return (`|GetArrayItem` _outactors)))

(fn `GetTargetPointHandler`
  (returns (TargetPointHandler :type "/Game/IS_CharacterCreator/Core/Utils/Camera/BP_ACC_TargetPointHandler Object Reference"))
  (return (`self.TargetPointHandler`)))

(fn `GetTargetView`
  (params (Key :type Name))
  (returns (Location :type "Vector Structure") (Offset :type "Vector Structure") (Exist :type Boolean))
  (bind (_value _returnvalue) (`self.TryGetTargetViewData` Key))
  (if _returnvalue
    (bind _refmesh (message `/Game/IS_CharacterCreator/Core/Interface/BPI_ACC_CharacterCustomization.I_GetRefMesh` (`self.GetCharacter`)))
    (bind (_socketname _offset) (break `/Game/IS_CharacterCreator/Core/Data/Struct/Creator/FStruct_ACC_CreatorTargetView` _value))
    (return (`SceneComponent.GetSocketLocation` _refmesh _socketname) _offset true)))

(fn `GetTargetViewData`
  (params (Key :type "Name (by ref)"))
  (returns (Value :type "/Game/IS_CharacterCreator/Core/Data/Struct/Creator/FStruct_ACC_CreatorTargetView Structure") (ReturnValue :type Boolean))
  (bind (_value _returnvalue) (`BlueprintMapLibrary.Map_Find` (`self.CurrentSpecieCreatorViewList`) Key))
  (return _value _returnvalue))

(fn `InitACCDataAndUI`
  (`self.InitUI`))

(fn `InitCameraTargetPoints`
  ;[1 0 0.8672] Target point camera
  (bind _returnvalue (`|SpawnActorFromClass` "/Game/IS_CharacterCreator/Core/Utils/Camera/BP_ACC_CameraTargetPoint.BP_ACC_CameraTargetPoint_C" (`self.GetTransform`) "Undefined" "OverrideRootScale" null null))
  (bind _output_get (set `self.CurrentTargetPoint` _returnvalue))
  (`self.K2_AttachToActor` _output_get self "None" "SnapToTarget" "KeepWorld" "KeepWorld" true)
  (`self.K2_AddActorLocalRotation` _output_get (struct :`Yaw` 180.0) false false)
  ;[1 0 0.7734] Init Camera
  (bind _returnvalue_2 (`|SpawnActorFromClass` "/Game/IS_CharacterCreator/Core/Utils/Camera/BP_ACC_Camera.BP_ACC_Camera_C" (`self.GetTransform`) "Undefined" "OverrideRootScale" null null))
  (bind _output_get_2 (set `self.ActiveCamera` _returnvalue_2))
  (`self.K2_AttachToActor` _output_get_2 self "None" "SnapToTarget" "KeepWorld" "KeepWorld" true)
  ;[0 1 0.6016] Change view
  (`PlayerController.SetViewTargetWithBlend` (`GameplayStatics.GetPlayerController` 0) (`self.ActiveCamera`) (`self.VTSBlendTime`) "VTBlend_Cubic" 1.0 false))

(fn `InitEssentials`
  (`|ExecutionSequence`
    (:`then_0`
      ;[0 1 1] Gyratory
      (bind _returnvalue (`|SpawnActorFromClass` "/Game/IS_CharacterCreator/Core/Utils/UI/BP_ACC_Gyratory_Main.BP_ACC_Gyratory_Main_C" (`self.GetTransform`) "Undefined" "OverrideRootScale" null null))
      (bind _output_get (set `self.GyratoryMain` _returnvalue))
      (`self.K2_AttachToActor` _output_get self "None" "SnapToTarget" "KeepWorld" "KeepWorld" true)
      ;[0 1 1] Target Point Handler
      (bind _returnvalue_2 (`|SpawnActorFromClass` "/Game/IS_CharacterCreator/Core/Utils/Camera/BP_ACC_TargetPointHandler.BP_ACC_TargetPointHandler_C" (`self.GetTransform`) "Undefined" "OverrideRootScale" null null))
      (bind _output_get_2 (set `self.TargetPointHandler` _returnvalue_2))
      (`self.K2_AttachToActor` _output_get_2 self "None" "SnapToTarget" "KeepWorld" "KeepWorld" true))
    (:`then_1`
      (`self.InitCameraTargetPoints`)
      (`self.InitACCDataAndUI`))))

(fn `InitUI`
  (bind _returnvalue (`|CreateWidget` (`self.WidgetClass`)))
  (bind _output_get (set `self.CurrentUI` _returnvalue))
  (`UserWidget.AddToViewport` _output_get 0)
  ;[0 0.9297 1] Registre the UI in GameInstance
  (message `/Game/IS_CharacterCreator/Core/Interface/BPI_ACC_GameInstance.I_GI_AddUI` (`GameplayStatics.GetGameInstance`) (`self.CurrentUI`)))

(fn `LoadFromExistingCharacter`
  (params (TargetCharacter :type "Actor Object Reference"))
  (bind _modularcharacter (`self.GetModularComp`))
  (bind _modularcharcomp (message `/Game/IS_CharacterCreator/Core/Interface/BPI_ACC_CharacterCustomization.I_GetModularComp` TargetCharacter))
  (set `self.Specie` (`/Game/IS_CharacterCreator/Core/Component/BP_ACC_MCC_Base.GetSpecieInformation` _modularcharcomp))
  (`self.ChangeCurrentCharacter` (`local.TargetCharacter`))
  (`self.OnGenderChange`)
  ;[0 0.7187 1] Simule Specie-Maturity-Gender change event
  (`/Game/IS_CharacterCreator/Core/Component/BP_ACC_MCC_Base.FireParamChange` _modularcharacter "Specie")
  (`/Game/IS_CharacterCreator/Core/Component/BP_ACC_MCC_Base.FireParamChange` _modularcharacter "Maturity")
  (`/Game/IS_CharacterCreator/Core/Component/BP_ACC_MCC_Base.FireParamChange` _modularcharacter "Gender"))

(fn `LoadSpecieCreatorConf`
  (bind _returnvalue (`|GetDataTableRow` (`self.DT_CreatorTargetConf`) (`self.Specie`))
    (:`then`
      (set `self.CurrentSpecieCreatorViewList` (`.TargetViewList_6_5E1F7D23450ECCA53C099CA883508BD0` (break `/Game/IS_CharacterCreator/Core/Data/Struct/Creator/FStruct_ACC_CreatorTargetConf` _returnvalue))))))

(fn `LogACCManager`
  (params (Info :type String))
  (`KismetSystemLibrary.PrintString` (`KismetTextLibrary.Conv_TextToString` (`|FormatText` "ACC_Manager : {text}" Info))))

(fn `OnChangeHeight`
  (`self.RefreshCurrentTargetView`))

(fn `OnChangeMaturity`
  (params (Maturity :type "/Game/IS_CharacterCreator/Core/Data/Enum/E_ACC_Maturity Enum" :default "NewEnumerator0"))
  ;[1 0 0.8203] Force pose change handler
  ; (to update height camera)
  (`self.OnChangePose`))

(fn `OnChangePose`
  (`self.RefreshCurrentTargetView`))

(fn `OnGenderChange`
  ;[0 0.5781 1] Load Specie creator view configuration
  (`self.LoadSpecieCreatorConf`)
  ;[0 1 0.2969] Refresh camera pos
  (`self.RefreshCameraAsync` 0.1))

(fn `OnMCCParamChange`
  (params (ParamName :type Name))
  (switch `name` ParamName
    (:`BodyHeight`
      (`self.OnChangeHeight`))
    (:`Gender`
      (`self.OnGenderChange`))))

(fn `RefreshCurrentTargetView`
  (`self.UpdateCameraView` (`self.CurrentCamerakeyView`)))

(fn `RemoveCharacter`
  ;[0 1 0.4609] Update Save Game
  (bind _accstorage (message `/Game/IS_CharacterCreator/Core/Interface/BPI_ACC_GameInstance.I_GI_GetACCStorage` (`GameplayStatics.GetGameInstance`)))
  (`/Game/IS_CharacterCreator/Core/Object/DAO/BP_ACC_DAO.RemoveCharacter` (`/Game/IS_CharacterCreator/Core/Library/BPFL_ACC_Common.GetACCDAO`) (`/Game/IS_CharacterCreator/Core/Library/BPFL_ACC_Common.GetACCCharUID` (`/Game/IS_CharacterCreator/Core/Object/BP_ACC_CustomizationStorage.GetCurrentCharacter` _accstorage)))
  ;[1 0 0.1875] Select by default first character (index 0)
  (bind _characterlist (`/Game/IS_CharacterCreator/Core/Object/DAO/BP_ACC_DAO.GetCharacterList` (`/Game/IS_CharacterCreator/Core/Library/BPFL_ACC_Common.GetACCDAO`)))
  (bind _accstorage_2 (message `/Game/IS_CharacterCreator/Core/Interface/BPI_ACC_GameInstance.I_GI_GetACCStorage` (`GameplayStatics.GetGameInstance`)))
  (`/Game/IS_CharacterCreator/Core/Object/BP_ACC_CustomizationStorage.SetCurrentCharacter` _accstorage_2 (`|GetArrayItem` _characterlist)))

(fn `RestoreGameControl`
  (bind _returnvalue (`GameplayStatics.GetPlayerController` 0))
  (`/Engine/EditorBlueprintResources/StandardMacros.IsValid` _returnvalue
    (:`Is Valid`
      (`PlayerController.SetViewTargetWithBlend` _returnvalue (`GameplayStatics.GetPlayerCharacter` 0) 1.0 "VTBlend_EaseInOut" 1.0 false)
      ;[0 1 0.9063] Restore input game
      (`WidgetBlueprintLibrary.SetInputMode_GameOnly` (`GameplayStatics.GetPlayerController` 0)))))

(fn `SaveCustomization`
  (params (Name :type Text) (ActionEdit :type Boolean))
  (locals (BuildedACC_Character :type "/Game/IS_CharacterCreator/Core/Data/Struct/FStruct_ACC_Character Structure"))
  (bind _returnvalue (`/Game/IS_CharacterCreator/Core/Library/BPFL_ACC_Common.TextToName` Name))
  (bind (_equipitemcustomparam _equipementidlist) (`self.SelectEquipData`))
  (bind _charctmdata (`/Game/IS_CharacterCreator/Core/Component/BP_ACC_MCC_Base.GetCharCustomizationData` (`self.GetModularComp`)))
  (bind _accstorage (message `/Game/IS_CharacterCreator/Core/Interface/BPI_ACC_GameInstance.I_GI_GetACCStorage` (`GameplayStatics.GetGameInstance`)))
  (bind _output_get (set `local.BuildedACC_Character` (`/Game/IS_CharacterCreator/Core/Library/BPFL_ACC_Common.BuildACCCharacter` (`KismetMathLibrary.SelectString` (`/Game/IS_CharacterCreator/Core/Library/BPFL_ACC_Common.GetACCCharUID` (`/Game/IS_CharacterCreator/Core/Object/BP_ACC_CustomizationStorage.GetCurrentCharacter` _accstorage)) (`/Game/IS_CharacterCreator/Core/Library/BPFL_ACC_Common.BuildACCUID` _returnvalue) (`local.ActionEdit`)) _returnvalue _charctmdata _equipitemcustomparam _equipementidlist)))
  (`/Game/IS_CharacterCreator/Core/Object/BP_ACC_CustomizationStorage.SetCurrentCharacter` _accstorage _output_get)
  (`self.SaveGameCharacter` (`local.BuildedACC_Character`)) ; Used for save game (or REST DB as you want)
)

(fn `SaveGameCharacter`
  (params (ACC_Character :type "/Game/IS_CharacterCreator/Core/Data/Struct/FStruct_ACC_Character Structure"))
  ;[0.4531 1 0] Update Save Game
  (`/Game/IS_CharacterCreator/Core/Object/DAO/BP_ACC_DAO.SaveCharacter` (`/Game/IS_CharacterCreator/Core/Library/BPFL_ACC_Common.GetACCDAO`) (`.UID_10_F67780C140DB8E607F2E17B3F8AA0036` (break `/Game/IS_CharacterCreator/Core/Data/Struct/FStruct_ACC_Character` ACC_Character)) ACC_Character))

(fn `SelectCharacter`
  (params (ACCCharacter :type "/Game/IS_CharacterCreator/Core/Data/Struct/FStruct_ACC_Character Structure"))
  (`self.ChangeCharacterData` ACCCharacter))

(fn `SelectEquipData`
  (returns (EquipItemCustomParam :type "Map of Name to /Game/IS_CharacterCreator/Core/Data/Struct/Customization/FStruct_ACC_ItemCustomization Structure") (EquipementIdList :type "Map of Name to Integer"))
  (bind _modularcharacter (`self.GetModularEquipComp`))
  (bind (_equipementparam _equipitemcustomparam _equipementidlist) (`/Game/IS_CharacterCreator/Core/Component/BP_ACC_MCC_Equip.GetEquipementsData` _modularcharacter))
  (`/Engine/EditorBlueprintResources/StandardMacros.IsValid` _modularcharacter
    (:`Is Valid`
      (return _equipitemcustomparam _equipementidlist))
    (:`Is Not Valid`
      (return))))

(fn `SetCreatorParameter`
  (params (ParamName :type Name) (Value :type "Integer (by ref)"))
  (`BlueprintMapLibrary.Map_Add` (`self.CreatorParameters`) ParamName Value)
  (`self.ApplyParamChange` ParamName))

(fn `SpawnCustomableCharacter`
  (params (Class :type "Actor Class Reference"))
  (returns (Character :type "Actor Object Reference"))
  ;[0.4062 1 0] Spawn Customable Character
  (bind _returnvalue (`|SpawnActorFromClass` Class (`KismetMathLibrary.MakeTransform` (0.0 0.0 -90.0)) "Undefined" "OverrideRootScale" null null))
  (`self.ChangeCurrentCharacter` _returnvalue)
  (return (`self.GetCharacter`)))

(fn `StartGame`
  (params (AsServer :type Boolean))
  (if AsServer
    (`GameplayStatics.OpenLevel` "TopDownExampleMap" true "?Listen")
    (else
      (`KismetSystemLibrary.ExecuteConsoleCommand` "open 127.0.0.1" null))))

(fn `TryGetTargetViewData`
  (params (Key :type Name))
  (returns (Value :type "/Game/IS_CharacterCreator/Core/Data/Struct/Creator/FStruct_ACC_CreatorTargetView Structure") (ReturnValue :type Boolean))
  (`/Engine/EditorBlueprintResources/StandardMacros.IsValid` (`self.GetCharacter`)
    (:`Is Valid`
      ;[1 0.8672 0] As first, attempt to get target view data from Maturity (Ex: adult_Global)
      (bind (_value _returnvalue) (`self.GetTargetViewData` (`KismetStringLibrary.Conv_StringToName` (`KismetTextLibrary.Conv_TextToString` (`|FormatText` "{maturity}_{key}" (`/Game/IS_CharacterCreator/Core/Library/BPFL_ACC_Constant.GetMaturityKey` (`/Game/IS_CharacterCreator/Core/Component/BP_ACC_MCC_Base.Maturity` (`self.GetModularComp`))) Key)))))
      (if _returnvalue
        (return _value true)
        (else
          ;[0.9453 0 1] Else get by given key only
          (bind (_value_2 _returnvalue_2) (`self.GetTargetViewData` (`local.Key`)))
          (return _value_2 _returnvalue_2))))
    (:`Is Not Valid`
      ;[1 0 0.9141] If character are null
      (return (struct) false))))

(fn `UpdateCameraView`
  (params (Key :type Name))
  (bind _currenttargetpoint (`self.CurrentTargetPoint`))
  (bind _output_get (set `self.CurrentCamerakeyView` Key))
  (bind (_location _offset _exist) (`self.GetTargetView` _output_get))
  (if _exist
    (bind _output_get_2 (set `self.CurrentTargetLocation` _location))
    (`self.K2_SetActorLocation` _currenttargetpoint _output_get_2 false false)
    (`self.K2_AddActorLocalOffset` _currenttargetpoint _offset false false)))

(fn `UserConstructionScript`)