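; Manager actor for the anime character creator that feeds the scene's global light to materials.
; UpdateLightVector copies the GlobalLight's forward direction, intensity and color, plus a shadow intensity setting, into the MPC_ACC_LightVector parameter collection.
; It runs on construction, BeginPlay and every Tick, and UpdateLightPreview also calls it.
; A TurnDebug flag slowly rotates the light each frame.
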(event `self.ReceiveBeginPlay`
  (`self.UpdateLightVector`))

(event `self.ReceiveTick`
  (params (DeltaSeconds :type "Float (single-precision)"))
  (`self.UpdateLightVector`)
  (if (`self.TurnDebug`)
    (`SceneComponent.K2_AddWorldRotation` (`Light.LightComponent` (`self.GlobalLight`)) (struct :`Yaw` 0.5) false false)))

(fn `UpdateLightPreview`
  (`self.UpdateLightVector`))

(fn `UpdateLightVector`
  (bind _lightcomponent (`Light.LightComponent` (`self.GlobalLight`)))
  (`KismetMaterialLibrary.SetVectorParameterValue` "/Game/IS_CharacterCreator/MaterialLibrary/MPC/MPC_ACC_LightVector.MPC_ACC_LightVector" "GlobalLightVector" (`KismetMathLibrary.Conv_VectorToLinearColor` (`SceneComponent.GetForwardVector` _lightcomponent)))
  (`KismetMaterialLibrary.SetScalarParameterValue` "/Game/IS_CharacterCreator/MaterialLibrary/MPC/MPC_ACC_LightVector.MPC_ACC_LightVector" "LightIntensity" (`LightComponentBase.Intensity` _lightcomponent))
  (`KismetMaterialLibrary.SetVectorParameterValue` "/Game/IS_CharacterCreator/MaterialLibrary/MPC/MPC_ACC_LightVector.MPC_ACC_LightVector" "GlobalLightColor" (`LightComponentBase.GetLightColor` (`Light.LightComponent` (`self.GlobalLight`))))
  (`KismetMaterialLibrary.SetScalarParameterValue` "/Game/IS_CharacterCreator/MaterialLibrary/MPC/MPC_ACC_LightVector.MPC_ACC_LightVector" "GlobalShadowIntensity" (`self.ShadowIntensity`)))

(fn `UserConstructionScript`
  (`self.UpdateLightVector`))