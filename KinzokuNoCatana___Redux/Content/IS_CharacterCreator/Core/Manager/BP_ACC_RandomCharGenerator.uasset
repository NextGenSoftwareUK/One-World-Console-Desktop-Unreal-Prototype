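; BP_ACC_RandomCharGenerator is a character creator manager that spawns a character Blueprint for a given species at a supplied location and rotation.
; SpawnIsCharacter gets the class from GetSpecieBP, which looks up the species row in the DTSpecieGameConfig data table.
; The spawned actor is cast to BP_ACC_Character, stored as CurrentSpawnedChar and returned with a success flag.
; Despite the name, it contains no randomization logic, and its event graph is empty.
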(event `self.ReceiveBeginPlay`)

(fn `GetSpecieBP`
  (params (Specie :type Name))
  (returns (CharacterBPClass :type "Actor Class Reference") (Found :type Boolean))
  (bind _returnvalue (`|GetDataTableRow` (`self.DT_SpecieGameConfig`) Specie)
    (:`then`
      (return (`.CharacterBPClass_3_3ADDDBF342863D79E6224F8BEADB44D9` (break `/Game/IS_CharacterCreator/Core/Data/Struct/Example/FStruct_ACC_SpecieGameConfig` _returnvalue)) true))
    (:`RowNotFound`
      (return "/Script/Engine.Actor" false))))

(fn `SpawnIsCharacter`
  (params (Specie :type Name) (SpawnLocation :type "Vector Structure") (SpawnRotation :type "Rotator Structure"))
  (returns (SpawnedCharacter :type "/Game/IS_CharacterCreator/Core/Character/BP_ACC_Character Object Reference") (Success :type Boolean))
  (locals (CurrentSpawnedChar :type "/Game/IS_CharacterCreator/Core/Character/BP_ACC_Character Object Reference"))
  (bind (_characterbpclass _found) (`self.GetSpecieBP` Specie))
  (if _found
    (bind _returnvalue (`|SpawnActorFromClass` _characterbpclass (`KismetMathLibrary.MakeTransform` SpawnLocation SpawnRotation) "Undefined" "OverrideRootScale" null null))
    (bind _asbp_acc_character (cast `/Game/IS_CharacterCreator/Core/Character/BP_ACC_Character` _returnvalue)
      (:`then`
        (bind _output_get (set `local.CurrentSpawnedChar` _asbp_acc_character))
        (`/Engine/EditorBlueprintResources/StandardMacros.IsValid` _output_get
          (:`Is Valid`
            (return (`local.CurrentSpawnedChar`) true))
          (:`Is Not Valid`
            ;[0 1 0.6719] Not Valid
            (return null false))))
      (:`CastFailed`
        ;[1 0 0.09375] Not Valid Cast
        (return null false)))
    (else
      ;[1 0.9141 0] NotFound
      (return null false))))

(fn `UserConstructionScript`)