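; BP_ACC_Customization is a customization accessory actor for the character creator, apparently a base, since Refresh and OnGenderChange are empty stubs.
; It stores a possessor through SetPossessor and exposes its modular character component through a getter.
; On BeginPlay it binds to that component's parameter change event, with a handler that routes Gender changes to OnGenderChange.
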(event `self.ReceiveBeginPlay`
  ;[0 0.1797 1] Event listener
  (add `/Game/IS_CharacterCreator/Core/Component/BP_ACC_MCC_Base.OnParamChange` (`self.GetModularCharComp`) (`|CreateDelegate` :!event `OnMCCParamChange`)))

(fn `GetModularCharComp`
  (returns (ModulaarCharCtm :type "/Game/IS_CharacterCreator/Core/Component/BP_ACC_MCC_Base Object Reference"))
  (return (`self.ModularCharCtm`)))

(fn `OnGenderChange`)

(fn `OnMCCParamChange`
  (params (ParamName :type Name))
  (switch `name` ParamName
    (:`Gender`
      (`self.OnGenderChange`))))

(fn `Refresh`)

(fn `SetPossessor`
  (params (Possessor :type "Actor Object Reference"))
  (set `self.ActorPossessor` Possessor))

(fn `UserConstructionScript`)