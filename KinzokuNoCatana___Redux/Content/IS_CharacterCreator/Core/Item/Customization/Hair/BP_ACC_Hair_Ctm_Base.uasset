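; Base Blueprint for character-creator hair customization, swapping skeletal meshes per hair type on paired source and outline meshes.
; ChangeHairStyle registers the hair data, restores the mesh's default materials and optionally refreshes the outline.
; Back tail hair reattaches to a selectable socket on the back hair.
; The construction script only clears the mesh map and array; helpers toggle visibility and physics, while the one-frame physics reset is currently disabled.
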(event `self.ReceiveBeginPlay`)

(event `CorrectHairPhysic`
  ;[0 0.4375 1] Event to correct hair physic : he reset all hair physic in "one frame"
  ; - "CorrectHairTask" avoid to call x time in same time the task for reset hair physic (because this event called in change hair style listeneer)
  ; - Example if in one frame we call 5 time this event, it's just useless
  ; - Note: Delay 0 = 1 frame
  ; UE5 INFO : ATM i disabled this because seem appear whe don't need to do this for now. but maybe with feedback...
)

(fn `ChangeHairStyle`
  (params (HairData :type "/Game/IS_CharacterCreator/Core/Data/Struct/Customization/FStruct_ACC_HairData Structure") (HairType :type Name))
  (bind (_hairid _icon _mesh) (break `/Game/IS_CharacterCreator/Core/Data/Struct/Customization/FStruct_ACC_HairData` HairData))
  (bind _hairtype (`local.HairType`))
  (bind (_sourcemesh _outlinemesh) (`/Game/IS_CharacterCreator/Core/Library/BPFL_ACC_Extractor.GetAnimMesh` (`.AnimeHairMesh` (`self.GetHairMeshFromType` HairType))))
  (`|ExecutionSequence`
    (:`then_0`
      (`self.SetHairData` HairType HairData)
      (`SkinnedMeshComponent.SetSkinnedAssetAndUpdate` _sourcemesh _mesh true)
      (`self.UpdateOutline` _sourcemesh _outlinemesh)
      (`/Engine/EditorBlueprintResources/StandardMacros.IsValid` _mesh ; If Hair Mesh not NONE
        (:`Is Valid`
          ;[0.8516 1 0] After Update mesh, reset default materials
          (for (_array_element _array_index) (`SkeletalMesh.Materials` (`.Mesh_5_72D16CA7400AABC99251AC93CA33C180` (break `/Game/IS_CharacterCreator/Core/Data/Struct/Customization/FStruct_ACC_HairData` (`self.GetHairData` _hairtype))))
            (`PrimitiveComponent.SetMaterial` (`self.GetHairMeshFromType` _hairtype) _array_index (`.MaterialInterface` (break `SkeletalMaterial` _array_element)))))))
    (:`then_1`
      ;[0 0.8828 1] Check it's valid hair
      (if (> (`.HairID_2_CBBC059749693DFA625E81BC94347BD2` (break `/Game/IS_CharacterCreator/Core/Data/Struct/Customization/FStruct_ACC_HairData` HairData)) 0)
        ;[1 0.2344 0] Handle Change Hair
        (`self.HandleChangeStyleType` (`local.HairType`))))))

(fn `GetHairData`
  (params (HairType :type "Name (by ref)"))
  (returns (HairData :type "/Game/IS_CharacterCreator/Core/Data/Struct/Customization/FStruct_ACC_HairData Structure"))
  (return (`BlueprintMapLibrary.Map_Find` (`self.RegistredHairData`) HairType)))

(fn `GetHairMeshFromType`
  (params (Type :type Name))
  (returns (HairMesh :type "SkeletalMeshComponent Object Reference") (AnimeHairMesh :type "/Game/IS_CharacterCreator/Core/Data/Struct/FStruct_ACC_AnimeMesh Structure"))
  (bind _value (`BlueprintMapLibrary.Map_Find` (`self.AnimeMeshMap`) Type))
  (return (`/Game/IS_CharacterCreator/Core/Library/BPFL_ACC_Extractor.GetAnimMesh` _value) _value))

(fn `GetOrignalHairScale`
  (params (SourceMesh :type "SkeletalMeshComponent Object Reference"))
  (returns (Scale :type "Vector Structure"))
  (return (`KismetMathLibrary.SelectVector` (-1.0 1.0 1.0) (1.0 1.0 1.0) (== SourceMesh null))))

(fn `HandleChangeStyleType`
  (params (HairType :type Name))
  (bind _hairmesh (`self.GetHairMeshFromType` "hb"))
  (bind _currenttailsocket (`self.CurrentTailSocket`))
  (bind (_sourcemesh _outlinemesh) (`/Game/IS_CharacterCreator/Core/Library/BPFL_ACC_Extractor.GetAnimMesh` (`.AnimeHairMesh` (`self.GetHairMeshFromType` "htb"))))
  (`|ExecutionSequence`
    (:`then_0`
      (switch `name` HairType
        (:`htb`
          ;[0.9219 1 0] When Change tail back hair -> Update Tail Hair Position
          (`/Engine/EditorBlueprintResources/StandardMacros.IsValid` _hairmesh
            (:`Is Valid`
              (`SceneComponent.K2_AttachToComponent` _sourcemesh _hairmesh _currenttailsocket "SnapToTarget" "SnapToTarget" "SnapToTarget" true)
              (`SceneComponent.K2_AttachToComponent` _outlinemesh _hairmesh _currenttailsocket "SnapToTarget" "SnapToTarget" "SnapToTarget" true))))))
    (:`then_1`
      (`self.CorrectHairPhysic`) ; Call this event to reset hair physic
    )))

(fn `InitEssentials`
  ;[0.8281 1 0] Clear
  (`BlueprintMapLibrary.Map_Clear` (`self.AnimeMeshMap`))
  (`KismetArrayLibrary.Array_Clear` (`self.HairMeshArray`)))

(fn `InitVariables`
  (params (Possessor :type "Actor Object Reference"))
  (`self.SetPossessor` Possessor))

(fn `LogHair`
  (params (Message :type String))
  (`KismetSystemLibrary.PrintString` (`KismetStringLibrary.Concat_StrStr` "LOG - Hair Customzation : " Message) true true (struct :`R` 1.0 :`G` 0.379636 :`B` 0.209088 :`A` 1.0)))

(fn `OnMaturityChange`
  (params (Maturity :type "/Game/IS_CharacterCreator/Core/Data/Enum/E_ACC_Maturity Enum" :default "NewEnumerator0")))

(fn `Refresh`
  (`parent.Refresh`))

(fn `SetActiveAllHairPhysic`
  (params (bActive :type Boolean))
  (for _array_element (`self.HairMeshArray`)
    (`self.SetActiveHairPhysic` bActive _array_element) ; Reset and disable physic for one frame
  ))

(fn `SetActiveHairPhysic`
  (params (bActive :type Boolean) (HairMesh :type "PrimitiveComponent Object Reference"))
  (if bActive
    (`PrimitiveComponent.SetSimulatePhysics` HairMesh true)
    (`PrimitiveComponent.SetCollisionEnabled` HairMesh "QueryAndPhysics")
    (else
      (`PrimitiveComponent.SetSimulatePhysics` HairMesh false)
      (`PrimitiveComponent.SetCollisionEnabled` HairMesh "NoCollision"))))

(fn `SetHairData`
  (params (HairType :type "Name (by ref)") (HairData :type "/Game/IS_CharacterCreator/Core/Data/Struct/Customization/FStruct_ACC_HairData Structure (by ref)"))
  (`BlueprintMapLibrary.Map_Add` (`self.RegistredHairData`) HairType HairData))

(fn `SetHairVisibility`
  (params (Visible :type Boolean))
  (for _array_element (`self.HairMeshArray`)
    (`SceneComponent.SetHiddenInGame` _array_element (not Visible) true)))

(fn `UpdateOutline`
  (params (SourceMesh :type "SkeletalMeshComponent Object Reference") (OutlineMesh :type "SkeletalMeshComponent Object Reference"))
  (if (`self.bUseOutline`)
    ;[1 0 0.04688] Update Anime Mesh Outline
    (`/Game/IS_CharacterCreator/Core/Library/BPFL_ACC_Extractor.ACCOutlineMesh` (`SkeletalMeshComponent.GetSkeletalMeshAsset` SourceMesh) SourceMesh OutlineMesh (`self.OutlineMaterial`))))

(fn `UpdateTailSocket`
  (params (SocketId :type Integer))
  (bind (_value _returnvalue) (`BlueprintMapLibrary.Map_Find` (`self.TailSocketList`) SocketId))
  (if _returnvalue
    (set `self.CurrentTailSocket` _value)
    (`self.HandleChangeStyleType` "htb")))

(fn `UserConstructionScript`
  (`self.InitEssentials`))