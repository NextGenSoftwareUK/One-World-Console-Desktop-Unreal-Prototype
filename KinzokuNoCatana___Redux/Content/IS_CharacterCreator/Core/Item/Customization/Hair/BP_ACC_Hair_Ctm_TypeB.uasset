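; BP_ACC_Hair_Ctm_TypeB is a Type B hair customization Blueprint for the anime character creator, built around a single front hair piece.
; Its InitEssentials override calls the parent, then maps one hair-type key to the front hair mesh paired with its outline mesh.
; It also registers the front hair mesh as the only entry in HairMeshArray, leaving all other behavior to the parent class.
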(fn `InitEssentials`
  (`parent.InitEssentials`)
  ;[0.7578 0 1] Anime Mesh map
  (set `self.AnimeMeshMap` (`|MakeMap` (`/Game/IS_CharacterCreator/Core/Library/BPFL_ACC_Constant.GetHairKeyFromType` "NewEnumerator0") (make `/Game/IS_CharacterCreator/Core/Data/Struct/FStruct_ACC_AnimeMesh` (`self.Front_Hair_Mesh`) (`self.Front_Hair_Mesh_Outline`))))
  ;;[0.4766 1 0] Mesh Array
  (set `self.HairMeshArray` (`|MakeArray` (`self.Front_Hair_Mesh`))))

(fn `UserConstructionScript`
  (`parent.UserConstructionScript`))