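; Character creator item actor that displays an item's skeletal mesh, with an optional anime-style outline mesh, on behalf of a Possessor.
; Item data drives InitFromData, which sets the mesh, refreshes the outline and resets default materials.
; Physics items simulate and run their own AnimInstance, which receives the Possessor's body mesh through interface messages.
; DestroyItem reverts morph float parameters to zero and clears master pose links before destroying the actor.
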(event `self.ReceiveBeginPlay`)

(fn `ActiveAnimInstance`
  (params (ItemData :type "/Game/IS_CharacterCreator/Core/Data/Struct/Common/FStruct_ACC_ItemData Structure"))
  (bind (_itemid _name _priority _icon _mesh _outlinemesh _attachtarget _parttype _customattach _rule _usephysic _animinstance) (break `/Game/IS_CharacterCreator/Core/Data/Struct/Common/FStruct_ACC_ItemData` ItemData))
  (if (`KismetSystemLibrary.IsValidClass` _animinstance)
    (`SkeletalMeshComponent.SetAnimInstanceClass` (`self.Mesh`) _animinstance)
    (bind _mesh_2 (message `/Game/IS_CharacterCreator/Core/Interface/BPI_ACC_CharacterCustomization.I_GetBodyMesh` (`self.Possessor`)))
    (message `/Game/IS_CharacterCreator/Core/Interface/BPI_ACC_ModularCloth.I_SetMeshReference` (`SkeletalMeshComponent.GetAnimInstance` (`self.Mesh`)) _mesh_2)))

(fn `ChangeItemData`
  (params (NewItemData :type "/Game/IS_CharacterCreator/Core/Data/Struct/Common/FStruct_ACC_ItemData Structure"))
  (set `self.ItemData` NewItemData)
  (`self.InitFromData`))

(fn `DestroyItem`
  (bind (_sourcemesh _outlinemesh) (`/Game/IS_CharacterCreator/Core/Library/BPFL_ACC_Extractor.GetAnimMesh` (`self.GetAnimeMesh`)))
  (`|ExecutionSequence`
    (:`then_0`
      ;[1 0 0.3984] Revert all float param
      (for _array_element (`/Game/IS_CharacterCreator/Core/Library/BPFL_ACC_Common.GetItemFloatParamList` (`self.ItemData`))
        (`self.RevertFloatParam` _array_element)))
    (:`then_1`
      ;[0.5703 0 1] Remove Old Master pose component
      (`SkinnedMeshComponent.SetLeaderPoseComponent` _sourcemesh null false)
      (`SkinnedMeshComponent.SetLeaderPoseComponent` _outlinemesh null false)
      (`self.K2_DestroyActor`))))

(fn `GetAnimeMesh`
  (returns (AnimeMesh :type "/Game/IS_CharacterCreator/Core/Data/Struct/FStruct_ACC_AnimeMesh Structure"))
  (return (make `/Game/IS_CharacterCreator/Core/Data/Struct/FStruct_ACC_AnimeMesh` (`self.Mesh`) (`self.OutlineMesh`))))

(fn `InitFromData`
  (bind _mesh (`self.Mesh`))
  (bind (_itemid _name _priority _icon _mesh_2 _outlinemesh _attachtarget _parttype _customattach _rule _usephysic) (break `/Game/IS_CharacterCreator/Core/Data/Struct/Common/FStruct_ACC_ItemData` (`self.ItemData`)))
  (`SkinnedMeshComponent.SetSkinnedAssetAndUpdate` (`self.Mesh`) _mesh_2 true)
  (`/Engine/EditorBlueprintResources/StandardMacros.IsValid` _mesh_2
    (:`Is Valid`
      ;[0 0.03906 1] Update Anime Mesh Outline
      (`self.UpdateOutline`)
      (`self.ResetMaterials` _mesh_2)
      ;[0 0.9766 1] AnimInstance if want to use Physic
      (if _usephysic
        (`PrimitiveComponent.SetSimulatePhysics` (`self.Mesh`) true) ; Active Simulate
        (`self.ActiveAnimInstance` (`self.ItemData`))
        (else
          (`SkeletalMeshComponent.SetAnimInstanceClass` _mesh null)
          (`PrimitiveComponent.SetSimulatePhysics` _mesh false))))))

(fn `InitItem`
  (params (Possessor :type "Actor Object Reference") (ItemData :type "/Game/IS_CharacterCreator/Core/Data/Struct/Common/FStruct_ACC_ItemData Structure"))
  (set `self.Possessor` Possessor)
  (set `self.ItemData` ItemData)
  (`self.InitFromData`))

(fn `ResetMaterials`
  (params (SKMesh :type "SkeletalMesh Object Reference"))
  ;[1 1 1] Reset default materials
  (`/Engine/EditorBlueprintResources/StandardMacros.IsValid` SKMesh
    (:`Is Valid`
      (for (_array_element _array_index) (`SkeletalMesh.Materials` SKMesh)
        (`PrimitiveComponent.SetMaterial` (`self.Mesh`) _array_index (`.MaterialInterface` (break `SkeletalMaterial` _array_element)))))))

(fn `RevertFloatParam`
  (params (FloatParam :type "/Game/IS_CharacterCreator/Core/Data/Struct/Param/FStruct_ACC_FloatParam Structure"))
  (bind (_identifier _type) (break `/Game/IS_CharacterCreator/Core/Data/Struct/Param/FStruct_ACC_FloatParam` FloatParam))
  (switch `name` _type
    (:`Morph`
      (`self.OnRevertFloat` _identifier))))

(fn `SetVisibility`
  (params (Visible :type Boolean))
  (`SceneComponent.SetHiddenInGame` (`self.DefaultSceneRoot`) (not Visible) true))

(fn `UpdateData`
  (params (ItemData :type "/Game/IS_CharacterCreator/Core/Data/Struct/Common/FStruct_ACC_ItemData Structure"))
  (set `self.ItemData` ItemData)
  (`self.InitFromData`))

(fn `UpdateOutline`
  (bind (_sourcemesh _outlinemesh) (`/Game/IS_CharacterCreator/Core/Library/BPFL_ACC_Extractor.GetAnimMesh` (`self.GetAnimeMesh`)))
  (if (`self.bUseOutline`)
    (`/Game/IS_CharacterCreator/Core/Library/BPFL_ACC_Extractor.ACCOutlineMesh` (`SkinnedMeshComponent.SkeletalMesh` (`self.Mesh`)) _sourcemesh _outlinemesh (`self.OutlineMaterial`))))

(fn `UserConstructionScript`
  (`self.InitFromData`))