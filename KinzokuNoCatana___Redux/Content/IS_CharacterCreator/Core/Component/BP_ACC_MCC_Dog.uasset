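; Character creator component for dog characters that overrides how body and head color parameters are applied.
; Both overrides call the parent, then branch on color type, writing Material colors to the body mesh, even for head parameters.
; Body Skin Color changes instead re-apply every entry in LayerColorList, reading each color from the body parameter group.
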(fn `ApplyBodyGPColor`
  (params (ColorParam :type "/Game/IS_CharacterCreator/Core/Data/Struct/Param/FStruct_ACC_ColorParam Structure (by ref)"))
  (bind (_identifier _type _value) (break `/Game/IS_CharacterCreator/Core/Data/Struct/Param/FStruct_ACC_ColorParam` ColorParam))
  (`parent.ApplyBodyGPColor` ColorParam)
  (`|ExecutionSequence`
    (:`then_0`
      ;[1 0 0.6328] Check Color Value Type
      (switch `name` _type
        (:`Material`
          (`self.UpdateObjectColor` (`self.GetBodyMesh`) _identifier _value))
        (:`SkinColor`
          (`self.AppySkinColor`))))
    (:`then_1`
      (return))))

(fn `ApplyHdGPColor`
  (params (ColorParam :type "/Game/IS_CharacterCreator/Core/Data/Struct/Param/FStruct_ACC_ColorParam Structure (by ref)"))
  (bind (_identifier _type _value) (break `/Game/IS_CharacterCreator/Core/Data/Struct/Param/FStruct_ACC_ColorParam` ColorParam))
  (`parent.ApplyHdGPColor` ColorParam)
  (`|ExecutionSequence`
    (:`then_0`
      ;[0.2656 1 0] Check Color Value Type
      (switch `name` _type
        (:`Material`
          (`self.UpdateObjectColor` (`self.GetBodyMesh`) _identifier _value))))
    (:`then_1`
      (return))))

(fn `AppySkinColor`
  (locals (LayerColorList :type "Array of Name"))
  (for _array_element (`local.LayerColorList`)
    (`self.UpdateObjectColor` (`self.GetBodyMesh`) _array_element (`/Game/IS_CharacterCreator/Core/Library/BPFL_ACC_GroupParam.GetColorFromGP` (`self.GetGroupParamFromIdentifier` (`/Game/IS_CharacterCreator/Core/Library/BPFL_ACC_Constant.GetBodyParamsKey`)) _array_element))))