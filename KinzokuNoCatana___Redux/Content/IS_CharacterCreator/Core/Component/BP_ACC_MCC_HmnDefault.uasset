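; Human character-creator component that overrides ApplyHeadStyle to rebuild the character's head when its style is applied.
; It clears the head's anim class, swaps the skeletal mesh, updates the anime outline mesh and assigns the anim instance for the current maturity and gender.
; It then resets default materials, recreates dynamic face, brow and eye materials by slot name, and reapplies head parameters and skin color.
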(fn `ApplyHeadStyle`
  (bind _headmesh (`self.GetHeadMesh`))
  (bind (_headmesh_2 _animemesh) (`self.GetHeadMesh`))
  (bind (_sourcemesh _outlinemesh) (`/Game/IS_CharacterCreator/Core/Library/BPFL_ACC_Extractor.GetAnimMesh` _animemesh))
  (`parent.ApplyHeadStyle`)
  ;[0 1 0.3203] Clean ABP
  (`SkeletalMeshComponent.SetAnimInstanceClass` _headmesh_2 null)
  (`SkinnedMeshComponent.SetSkinnedAssetAndUpdate` _headmesh_2 (`.Mesh_5_D6DA1CAC4B943BAE99806AB035B71EFA` (break `/Game/IS_CharacterCreator/Core/Data/Struct/Customization/FStruct_ACC_HeadData` (`self.HeadData`))) true)
  ;[0 0.1797 1] Update Anime Mesh Outline
  (`self.UpdateOutline` _sourcemesh _outlinemesh)
  (`|ExecutionSequence`
    (:`then_0`
      ;[1 0 0.2578] Change Head anim instance
      (`SkeletalMeshComponent.SetAnimInstanceClass` (`self.GetHeadMesh`) (`.HeadAnimInst_11_ABA8DF1B49FFD220CC3C6890CA151ECB` (break `/Game/IS_CharacterCreator/Core/Data/Struct/FStruct_ACC_GenderConfig` (`self.GetOneGenderData` (`self.Maturity`) (`self.Gender`))))))
    (:`then_1`
      ;[0.3828 0 1] Reset Default Material
      (for (_array_element _array_index) (`SkeletalMesh.Materials` (`.Mesh_5_D6DA1CAC4B943BAE99806AB035B71EFA` (break `/Game/IS_CharacterCreator/Core/Data/Struct/Customization/FStruct_ACC_HeadData` (`self.HeadData`))))
        (`PrimitiveComponent.SetMaterial` (`self.GetHeadMesh`) _array_index (`.MaterialInterface` (break `SkeletalMaterial` _array_element)))))
    (:`then_2`
      ;[0.8281 1 0.6562] Remake Instance Material
      ;;[0.8516 1 0] FaceHead Part
      (bind _returnvalue (`/Game/IS_CharacterCreator/Core/Library/BPFL_ACC_Extractor.SetMatDynamicFromName` _headmesh "MI_Char_Human_Adult"))
      (set `self.HeadDynamicMaterial` _returnvalue)
      ;;[1 0 0.9609] Brow Part
      (bind _returnvalue_2 (`/Game/IS_CharacterCreator/Core/Library/BPFL_ACC_Extractor.SetMatDynamicFromName` _headmesh "MI_Human_Brow"))
      (set `self.EyeBrowMaterial` _returnvalue_2)
      ;;[0 0.2266 1] Eye Part
      (`KismetArrayLibrary.Array_Clear` (`self.EyeMaterial`))
      (for _index (range 2)
        (bind _returnvalue_3 (`/Game/IS_CharacterCreator/Core/Library/BPFL_ACC_Extractor.SetMatDynamicFromName` _headmesh (select `int` _index :`0` "MI_Eye_L" :`1` "MI_Eye_R" :!type "Name")))
        (`/Engine/EditorBlueprintResources/StandardMacros.IsValid` _returnvalue_3
          (:`Is Valid`
            (`KismetArrayLibrary.Array_AddUnique` (`self.EyeMaterial`) _returnvalue_3)))))
    (:`then_3`
      ;[0 0.6953 1] Apply head param and skin color
      (`self.ApplyHeadParam`)
      (`self.AppySkinColor`))))