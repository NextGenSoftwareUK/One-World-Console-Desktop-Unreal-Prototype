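; Character creator component that extends its parent customization component with equippable, recolorable clothing, armor and accessories.
; Item IDs resolve through a DAO into spawned BP_ACC_Item actors, socket-attached or skinned to the body via master pose unless physics-driven.
; Equipping also drives body-hide textures, float parameters and three-channel colors, while morphs propagate to skinned pieces.
; IDs and colors save and restore with character data, and item tag changes trigger tag scripts.
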(event `self.ReceiveEndPlay`
  (params (EndPlayReason :type "EEndPlayReason Enum" :default "Destroyed"))
  ;[0 0.1328 1] On end
  (`self.DestroyAll`))

(fn `ApplyBodyMorphToSkinned`
  (params (MorphName :type Name) (MorphValue :type "Float (double-precision)"))
  (bind _keys (`BlueprintMapLibrary.Map_Keys` (`self.SkinnedMeshes`)))
  (for _array_element _keys
    (bind (_value _returnvalue) (`BlueprintMapLibrary.Map_Find` (`self.SkinnedMeshes`) _array_element))
    (if _returnvalue
      (`/Engine/EditorBlueprintResources/StandardMacros.IsValid` _value
        (:`Is Valid`
          (`SkeletalMeshComponent.SetMorphTarget` _value (`local.MorphName`) (`local.MorphValue`) true))))))

(fn `ApplyEquipItemCustom`
  (params (EquipKey :type Name))
  (locals (ItemCustomParam :type "/Game/IS_CharacterCreator/Core/Data/Struct/Customization/FStruct_ACC_ItemCustomization Structure"))
  (bind (_success _item) (`self.GetEquipementFromKey` EquipKey))
  (if _success
    (set `local.ItemCustomParam` (`/Game/IS_CharacterCreator/Core/Library/BPFL_ACC_Common.GetEquipCustomParam` (`self.ItemCustomParamList`) (`local.EquipKey`)))
    (for _index (range 3)
      (`self.UpdateObjectColor` (`/Game/IS_CharacterCreator/Core/Item/BP_ACC_Item.Mesh` _item) (`/Game/IS_CharacterCreator/Core/Library/BPFL_ACC_Common.BuildColorPaletteName` _index) (`/Game/IS_CharacterCreator/Core/Library/BPFL_ACC_Common.SelectItemColorCustom` (`local.ItemCustomParam`) _index)))))

(fn `ApplyFloatParam`
  (params (FloatParam :type "/Game/IS_CharacterCreator/Core/Data/Struct/Param/FStruct_ACC_FloatParam Structure") (Reset :type Boolean) (MeshTarget :type "MeshComponent Object Reference"))
  (bind (_identifier _type _value) (break `/Game/IS_CharacterCreator/Core/Data/Struct/Param/FStruct_ACC_FloatParam` FloatParam))
  (`parent.ApplyFloatParam` FloatParam Reset MeshTarget)
  (switch `name` _type
    (:`Morph`
      (`self.ApplyBodyMorphToSkinned` _identifier _value))))

(fn `ChangeEquipId`
  (params (Type :type Name) (Id :type Integer))
  (`|ExecutionSequence`
    (:`then_0`
      (if (> Id 0)
        ;[0.4766 1 0] Continue only if different item
        (if (!= (`local.Id`) (`BlueprintMapLibrary.Map_Find` (`self.EquipementIdList`) (`local.Type`)))
          ;[0 1 1] Get item from DAO
          (bind _acc_itemdata (`self.GetItemData` (`local.Id`)))
          ;[0.7812 1 0] Apply equip
          (`self.EquipItem` _acc_itemdata) ; Equip item
          ;[0 1 0.5781] Store id
          (`BlueprintMapLibrary.Map_Add` (`self.EquipementIdList`) (`local.Type`) (`local.Id`))
          ;[0.6406 1 0] Store data
          (`BlueprintMapLibrary.Map_Add` (`self.ItemDataList`) (`local.Type`) _acc_itemdata)
          ;[1 0.9844 0] Apply Color
          (`self.ApplyEquipItemCustom` (`local.Type`)))
        (else
          ;[0.3828 1 0] If id < 1 : Unequip the item
          (`self.UnequipItem` (`local.Type`)))))
    (:`then_1`
      (`self.ComputeTags`))))

(fn `ChangeEquipItemCustom`
  (params (ItemPart :type Name) (ColorIndex :type Integer) (Color :type "LinearColor Structure"))
  (`self.ChangeItemColor` ItemPart ColorIndex Color))

(fn `ChangeItemColor`
  (params (ItemPart :type Name) (ColorIndex :type Integer) (Color :type "LinearColor Structure"))
  (locals (ItemKey :type Name :default "None") (NewItemParam :type "/Game/IS_CharacterCreator/Core/Data/Struct/Customization/FStruct_ACC_ItemCustomization Structure"))
  (bind _color (`local.Color`))
  (bind _output_get (set `local.ItemKey` ItemPart))
  (`|ExecutionSequence`
    (:`then_0`
      (switch `int` ColorIndex
        (:`0`
          (bind _itemcustomparam (`/Game/IS_CharacterCreator/Core/Library/BPFL_ACC_Common.GetEquipCustomParam` (`self.ItemCustomParamList`) _output_get))
          (bind _structout (setmembers `/Game/IS_CharacterCreator/Core/Data/Struct/Customization/FStruct_ACC_ItemCustomization` :`StructRef` _itemcustomparam :`ColorA` _color))
          (set `local.NewItemParam` _structout))
        (:`1`
          (bind _structout_2 (setmembers `/Game/IS_CharacterCreator/Core/Data/Struct/Customization/FStruct_ACC_ItemCustomization` :`StructRef` _itemcustomparam :`ColorB` _color))
          (set `local.NewItemParam` _structout_2))
        (:`2`
          (bind _structout_3 (setmembers `/Game/IS_CharacterCreator/Core/Data/Struct/Customization/FStruct_ACC_ItemCustomization` :`StructRef` _itemcustomparam :`ColorC` _color))
          (set `local.NewItemParam` _structout_3))))
    (:`then_1`
      ;[1 0.8438 0] Edit Struct
      (`BlueprintMapLibrary.Map_Add` (`self.ItemCustomParamList`) (`local.ItemKey`) (`local.NewItemParam`))
      ;[0 0.7891 1] Apply
      (`self.ApplyEquipItemCustom` (`local.ItemKey`)))))

(fn `ComputeTags`
  (locals (PreviousTags :type "Array of Name"))
  (`KismetArrayLibrary.Array_Append` (`local.PreviousTags`) (`self.Tags`))
  (`|ExecutionSequence`
    (:`then_0`
      (`KismetArrayLibrary.Array_Clear` (`self.Tags`))
      (bind _values (`BlueprintMapLibrary.Map_Values` (`self.ItemDataList`)))
      (for _array_element _values
        (for _array_element_2 (`.Tags_68_359435584ED536D1710E16AA9AA8EAC0` (break `/Game/IS_CharacterCreator/Core/Data/Struct/Common/FStruct_ACC_ItemData` _array_element))
          (`KismetArrayLibrary.Array_AddUnique` (`self.Tags`) _array_element_2)
          ;[1 0.3281 0] Detect New Tags
          (if (not (`KismetArrayLibrary.Array_Contains` (`local.PreviousTags`) _array_element_2))
            (`self.PerformTagScript` _array_element_2 true)))))
    (:`then_1`
      (for _array_element_3 (`local.PreviousTags`)
        ;[0.5469 1 0] Detect Leave Tags Script
        (if (not (`KismetArrayLibrary.Array_Contains` (`self.Tags`) _array_element_3))
          (`self.PerformTagScript` _array_element_3))))))

(fn `DestroyAll`
  (`self.UnequipAllItem`)
  (`parent.DestroyAll`))

(fn `DestroyEquipItem`
  (params (Part :type Name))
  (returns (Success :type Boolean))
  (locals (ItemToDestroy :type "/Game/IS_CharacterCreator/Core/Item/BP_ACC_Item Object Reference"))
  (bind (_success _item) (`self.GetEquipementFromKey` Part))
  (set `local.ItemToDestroy` _item)
  ;[0 1 0.08594] Remove stored struct
  (`BlueprintMapLibrary.Map_Remove` (`self.ItemDataList`) (`local.Part`))
  ;[0.9688 1 0] Remove stored id
  (`BlueprintMapLibrary.Map_Remove` (`self.EquipementIdList`) (`local.Part`))
  ;[1 0.1875 0] Remove from registred item array
  (bind _returnvalue (`BlueprintMapLibrary.Map_Remove` (`self.EquipedItemInst`) (`local.Part`)))
  ;[0 1 0.9766] Remove skinned meshes
  (`BlueprintMapLibrary.Map_Remove` (`self.SkinnedMeshes`) (`local.Part`))
  ;[1 0 0.4922] Reset Body Hide and Destroy item
  (if _returnvalue
    (`/Game/IS_CharacterCreator/Core/Item/BP_ACC_Item.DestroyItem` (`local.ItemToDestroy`))
    (return true)
    (else
      (return false))))

(fn `EquipItem`
  (params (ItemData :type "/Game/IS_CharacterCreator/Core/Data/Struct/Common/FStruct_ACC_ItemData Structure"))
  (locals (CurrentItemInst :type "/Game/IS_CharacterCreator/Core/Item/BP_ACC_Item Object Reference"))
  (bind (_itemid _name _priority _icon _mesh _outlinemesh _attachtarget _parttype _customattach _rule _usephysic _animinstance _attachtype _defaultctm) (break `/Game/IS_CharacterCreator/Core/Data/Struct/Common/FStruct_ACC_ItemData` ItemData))
  (bind _currentiteminst (`local.CurrentItemInst`))
  (bind _itemdata (`local.ItemData`))
  (bind (_itemid_2 _name_2 _priority_2 _icon_2 _mesh_2 _outlinemesh_2 _attachtarget_2 _parttype_2 _customattach_2 _rule_2 _usephysic_2 _animinstance_2 _attachtype_2) (break `/Game/IS_CharacterCreator/Core/Data/Struct/Common/FStruct_ACC_ItemData` (`local.ItemData`)))
  (bind _part (`/Game/IS_CharacterCreator/Core/Library/BPFL_ACC_Common.GetItemPartKey` (`local.ItemData`)))
  (bind _part_2 (`/Game/IS_CharacterCreator/Core/Library/BPFL_ACC_Common.GetItemPartKey` (`local.ItemData`)))
  (`/Engine/EditorBlueprintResources/StandardMacros.IsValid` _mesh
    (:`Is Valid`
      (`|ExecutionSequence`
        (:`then_0`
          ;[0.9453 1 0] If already have equiped item from the key, unequip it to replace by the newer
          (bind _success (`self.GetEquipementFromKey` _part_2))
          (if _success
            (`self.UnequipItem` _part_2)))
        (:`then_1`
          ;[0.6875 1 0] Update or Add item data
          (`BlueprintMapLibrary.Map_Add` (`self.ItemDataList`) (`/Game/IS_CharacterCreator/Core/Library/BPFL_ACC_Common.GetItemPartKey` _itemdata) _itemdata)
          (`self.HandlePartEquip` _parttype) ; Handle Equip type before any application
          ;[0 0.08594 1] Instance BP_Item and attach to character
          (bind _returnvalue (`|SpawnActorFromClass` "/Game/IS_CharacterCreator/Core/Item/BP_ACC_Item.BP_ACC_Item_C" (`KismetMathLibrary.MakeTransform` (0.0 0.0 0.0)) "Undefined" "OverrideRootScale" null (`local.ItemData`) (`self.GetPossesor`) null))
          (bind _output_get (set `local.CurrentItemInst` _returnvalue))
          ;;[1 0.4716 0.4018] Bind revert float
          (add `/Game/IS_CharacterCreator/Core/Item/BP_ACC_Item.OnRevertFloat` _output_get (`|CreateDelegate` :!event `OnItemRevertFloat`))
          (`BlueprintMapLibrary.Map_Add` (`self.EquipedItemInst`) (`/Game/IS_CharacterCreator/Core/Library/BPFL_ACC_Common.BuildEquipItemKey` (`local.ItemData`)) (`local.CurrentItemInst`))
          ;[0 1 0.1562] Select Attach method from type
          ; Exemple : For armor it'll be skinned mesh
          ; But for an simply accessory is just an attach actor
          (switch `/Game/IS_CharacterCreator/Core/Data/Enum/E_ACC_ItemAttachType` _attachtype_2
            (:`NewEnumerator0`
              (`self.EquipSkinnedArmor` _currentiteminst (`local.ItemData`)))
            (:`NewEnumerator1`
              (`Actor.K2_AttachToComponent` _currentiteminst (`self.GetAttachMeshTarget` _attachtarget_2) _customattach_2 "SnapToTarget" "SnapToTarget" "KeepRelative" true))))
        (:`then_2`
          ;[1 0 0.5625] Default Item Color
          (if (not (`BlueprintMapLibrary.Map_Contains` (`self.ItemCustomParamList`) (`/Game/IS_CharacterCreator/Core/Library/BPFL_ACC_Common.GetItemPartKey` (`local.ItemData`))))
            (bind _itemctm (`/Game/IS_CharacterCreator/Core/Object/DAO/BP_ACC_DAO_Item.GetItemCtmColor` (`/Game/IS_CharacterCreator/Core/Object/DAO/BP_ACC_DAO.GetDAOItem` (`/Game/IS_CharacterCreator/Core/Library/BPFL_ACC_Common.GetACCDAO`)) _defaultctm))
            ;;[1 0.8438 0] Edit Struct
            (`BlueprintMapLibrary.Map_Add` (`self.ItemCustomParamList`) _part _itemctm)
            ;;[0 0.7891 1] Apply
            (`self.ApplyEquipItemCustom` _part)))))))

(fn `EquipSkinnedArmor`
  (params (BPItem :type "/Game/IS_CharacterCreator/Core/Item/BP_ACC_Item Object Reference") (ItemData :type "/Game/IS_CharacterCreator/Core/Data/Struct/Common/FStruct_ACC_ItemData Structure"))
  (bind (_itemid _name _priority _icon _mesh _outlinemesh _attachtarget _parttype _customattach _rule _usephysic) (break `/Game/IS_CharacterCreator/Core/Data/Struct/Common/FStruct_ACC_ItemData` ItemData))
  (`Actor.K2_AttachToComponent` BPItem (`self.GetBodyMesh`) "Socket_Root" "SnapToTarget" "SnapToTarget" "SnapToTarget" true)
  ;[0.9137 0.8235 1] SKINNED MESH -> Skin New Item to body
  (`self.SetNewSkinnedMesh` _parttype (`/Game/IS_CharacterCreator/Core/Item/BP_ACC_Item.Mesh` BPItem) _usephysic)
  ;[0 0.5078 1] Set body hide from item
  (`self.UpdateBodyHide` (`local.ItemData`))
  (`self.ApplyItemFloatParam` (`local.ItemData`) (`self.GetBodyMesh`)))

(fn `GetACCCharData`
  (returns (ACC_Character :type "/Game/IS_CharacterCreator/Core/Data/Struct/FStruct_ACC_Character Structure"))
  (bind (_equipementparam _equipitemcustomparam _equipementidlist) (`self.GetEquipementsData`))
  (bind _charctmdata (`self.GetCharCustomizationData`))
  (return (make `/Game/IS_CharacterCreator/Core/Data/Struct/FStruct_ACC_Character` "Anonymous" "Anonymous" _charctmdata _equipitemcustomparam _equipementidlist)))

(fn `GetEquipDataFromPart`
  (params (EquipKey :type Name))
  (returns (Id :type Integer) (Value :type "/Game/IS_CharacterCreator/Core/Data/Struct/Common/FStruct_ACC_ItemData Structure"))
  (bind _value (`BlueprintMapLibrary.Map_Find` (`self.ItemDataList`) EquipKey))
  (return (`/Game/IS_CharacterCreator/Core/Library/BPFL_ACC_Common.GetItemId` _value) _value))

(fn `GetEquipedItemList`
  (returns (EquipedItemInst :type "Map of Name to /Game/IS_CharacterCreator/Core/Item/BP_ACC_Item Object Reference"))
  (return (`self.EquipedItemInst`)))

(fn `GetEquipementFromKey`
  (params (ItemKey :type Name))
  (returns (Success :type Boolean) (Item :type "/Game/IS_CharacterCreator/Core/Item/BP_ACC_Item Object Reference"))
  (bind (_value _returnvalue) (`BlueprintMapLibrary.Map_Find` (`self.GetEquipedItemList`) ItemKey))
  (if _returnvalue
    (return true _value)
    (else
      (return false null))))

(fn `GetEquipementsData`
  (returns (EquipementParam :type "Map of Name to /Game/IS_CharacterCreator/Core/Data/Struct/Common/FStruct_ACC_ItemData Structure") (EquipItemCustomParam :type "Map of Name to /Game/IS_CharacterCreator/Core/Data/Struct/Customization/FStruct_ACC_ItemCustomization Structure") (EquipementIdList :type "Map of Name to Integer"))
  (return (`self.ItemDataList`) (`self.ItemCustomParamList`) (`self.EquipementIdList`)))

(fn `GetItemData`
  (params (Id :type Integer))
  (returns (ACC_ItemData :type "/Game/IS_CharacterCreator/Core/Data/Struct/Common/FStruct_ACC_ItemData Structure"))
  (bind _acc_itemdata (`/Game/IS_CharacterCreator/Core/Object/DAO/BP_ACC_DAO_Item.GetACCItemDataFromGender` (`/Game/IS_CharacterCreator/Core/Object/DAO/BP_ACC_DAO.GetDAOItem` (`/Game/IS_CharacterCreator/Core/Library/BPFL_ACC_Common.GetACCDAO`)) Id (`self.SpecieIdentifier`) (`self.Maturity`) (`self.Gender`)))
  (return _acc_itemdata))

(fn `HandlePartEquip`
  (params (ItemPart :type Name) (ActiveEquip :type Boolean :default true))
  (switch `name` ItemPart
    (:`Top`
      ;[1 0 0.4922] For exemple: Hide female bra when equip Top outfit (opacity = 0)
      ; If unequip show bra outfit (opacity = 1)
      (`MeshComponent.SetScalarParameterValueOnMaterials` (`self.GetBodyMesh`) "BraOpacity" (`KismetMathLibrary.SelectFloat` 0.0 1.0 ActiveEquip)))))

(fn `InitEquipement fromIdList`
  (params (NewIdList :type "Map of Name to Integer"))
  (bind _keys (`BlueprintMapLibrary.Map_Keys` NewIdList))
  ;[0.3594 0 1] Get all Equipements Data from given ids
  (for _array_element _keys
    (bind (_value _returnvalue) (`BlueprintMapLibrary.Map_Find` (`local.NewIdList`) _array_element))
    (if _returnvalue
      ;[0.3594 0 1] Change equip id
      (`self.ChangeEquipId` _array_element _value))))

(fn `InitFromACCCharData`
  (params (ACC_CharacterData :type "/Game/IS_CharacterCreator/Core/Data/Struct/FStruct_ACC_Character Structure"))
  (bind (_uid _name _charcustom _equipementparamlist _equipementidlist) (break `/Game/IS_CharacterCreator/Core/Data/Struct/FStruct_ACC_Character` ACC_CharacterData))
  (`parent.InitFromACCCharData` ACC_CharacterData)
  (set `self.ItemCustomParamList` _equipementparamlist)
  (`self.InitEquipement fromIdList` _equipementidlist))

(fn `OnItemRevertFloat`
  (params (MorphName :type Name) (MorphValue :type "Float (double-precision)"))
  (`self.ApplyBodyMorphToSkinned` MorphName MorphValue))

(fn `RemoveSkinnedMesh`
  (params (Part :type Name))
  (returns (Success :type Boolean))
  (bind _returnvalue (`BlueprintMapLibrary.Map_Remove` (`self.SkinnedMeshes`) Part))
  (return _returnvalue))

(fn `ResetBody`
  (`self.UnequipAllItem`)
  (`parent.ResetBody`))

(fn `SetGlobalMorphTarget`
  (params (MorphTargetName :type Name) (Mesh :type "SkeletalMeshComponent Object Reference") (Value :type "Float (double-precision)") (ApplyOnSkinnedMesh :type Boolean))
  (`parent.SetGlobalMorphTarget` MorphTargetName Mesh Value ApplyOnSkinnedMesh)
  ;[1 0.75 0] If Authorized apply morph in skinned mesh (armors, accessory, etc)
  (if (`local.ApplyOnSkinnedMesh`)
    (`self.ApplyBodyMorphToSkinned` (`local.MorphTargetName`) (`local.Value`))))

(fn `SetItemVisiblity`
  (params (HairVisible :type Boolean) (SkinnedVisible :type Boolean))
  (`parent.SetItemVisiblity` HairVisible SkinnedVisible)
  ;[1 0 0.6094] Items/Clothes visiblity
  (bind _values (`BlueprintMapLibrary.Map_Values` (`self.SkinnedMeshes`)))
  (for _array_element _values
    (`SceneComponent.SetHiddenInGame` _array_element (not (`local.SkinnedVisible`)) false)))

(fn `SetNewSkinnedMesh`
  (params (Part :type Name) (SkinnedMesh :type "SkeletalMeshComponent Object Reference") (UsePhysic :type Boolean))
  (`|ExecutionSequence`
    (:`then_0`
      ;[0.3359 1 0] Use Master Pose Componenet Only fi not use physic
      (if (not UsePhysic)
        (`self.MasterPoseSkinnedMesh` SkinnedMesh true)))
    (:`then_1`
      ;[1 0 0.1641] Add to TMap
      (`BlueprintMapLibrary.Map_Add` (`self.SkinnedMeshes`) Part SkinnedMesh)
      (return))))

(fn `UnequipAllItem`
  ;[1 0.2109 0] Foreach all equiped item, delete each item type
  (bind _values (`BlueprintMapLibrary.Map_Values` (`self.GetEquipementsData`)))
  (for _array_element _values
    ;[0 1 0.1797] Unequip Current item type
    (`self.UnequipItem` (`/Game/IS_CharacterCreator/Core/Library/BPFL_ACC_Common.GetItemType` _array_element)))
  ;[0 0.8359 1] Default return
  (return))

(fn `UnequipItem`
  (params (ItemPart :type Name))
  (returns (Success :type Boolean))
  (bind (_id _value) (`self.GetEquipDataFromPart` (`local.ItemPart`)))
  ;[0.4531 0 1] Handle Unequip
  (`self.HandlePartEquip` ItemPart false) ; Handle Equip type before any application
  ;[0.2188 0 1] If item exist
  (bind _success (`self.GetEquipementFromKey` ItemPart))
  (if _success
    ;[0 1 0.7656] Remove the hide body texture
    (`self.UpdateBodyHide` _value true)
    ;[0.4766 0 1] Reset some float param
    (`self.ApplyItemFloatParam` _value (`self.GetBodyMesh`) true)
    ;[0 1 0.1094] Remove color
    (`BlueprintMapLibrary.Map_Remove` (`self.ItemCustomParamList`) (`local.ItemPart`))
    ;[1 0 0.7969] Destroy Item
    (bind _success_2 (`self.DestroyEquipItem` (`local.ItemPart`)))
    (return _success_2)
    (else
      ;[0.1719 0 1] Return false
      (return false))))

(fn `UpdateBodyHide`
  (params (ItemData :type "/Game/IS_CharacterCreator/Core/Data/Struct/Common/FStruct_ACC_ItemData Structure") (Reset :type Boolean) (ResetAll :type Boolean))
  (locals (CurrentDynamicMat :type "MaterialInstanceDynamic Object Reference"))
  (bind (_itemid _name _priority _icon _mesh _outlinemesh _attachtarget _parttype _customattach _rule _usephysic _animinstance _attachtype _defaultctm _tags _groupparam) (break `/Game/IS_CharacterCreator/Core/Data/Struct/Common/FStruct_ACC_ItemData` (`local.ItemData`)))
  (bind (_value _exist) (`self.GetGPTexValueFromGP` _groupparam "BodyHideTexture"))
  ;[0 1 0.2031] Create Dynamic Material to param "Texture body hide"
  (bind _bodydynamicmaterials (`self.GetDynamicBodyMats`))
  (for _array_element _bodydynamicmaterials
    (set `local.CurrentDynamicMat` _array_element)
    (if ResetAll
      ;[0.7396 0.9294 1] Reset all body hide
      (bind _keys (`BlueprintMapLibrary.Map_Keys` (`self.EquipedItemInst`)))
      (for _array_element_2 _keys
        (`MaterialInstanceDynamic.SetTextureParameterValue` (`local.CurrentDynamicMat`) (`self.SelectBodyHideParamName` _array_element_2) "/Game/IS_CharacterCreator/TextureLibrary/Common/T_ACC_BlankHide.T_ACC_BlankHide"))
      (else
        ;[1 0.8777 0.6519] BodyHide from item data
        (`MaterialInstanceDynamic.SetTextureParameterValue` (`local.CurrentDynamicMat`) (`self.SelectBodyHideParamName` _parttype) (select `bool` (or (`local.Reset`) (not _exist)) :`false` _value :`true` "/Game/IS_CharacterCreator/TextureLibrary/Common/T_ACC_BlankHide.T_ACC_BlankHide" :!type "Texture Object Reference"))))))