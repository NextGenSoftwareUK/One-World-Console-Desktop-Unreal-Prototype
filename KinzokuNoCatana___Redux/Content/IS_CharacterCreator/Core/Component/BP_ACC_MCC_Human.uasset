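; Human modular character customization component that applies body, head, face and hair parameters to the character's meshes.
; Parent apply hooks are extended to route parameters by type into material colors, scalars and textures, with styles looked up through DAO data.
; Separate hair and face customization actors are spawned, with hair re-instanced when the gender's class differs.
; Gender changes reset the body, swap mesh and optional AnimBP, reattach the head and reapply all parameters.
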(fn `ApplyAllHair`
  (params (HairColor :type Boolean))
  ;[1 0.7734 0] HairColorPart
  (if HairColor
    (for _array_element (`/Game/IS_CharacterCreator/Core/Item/Customization/Hair/BP_ACC_Hair_Ctm_Base.HairMeshArray` (`self.BP_Hair_Customization`))
      (`self.ApplyHairColor` _array_element))
    (`self.ApplyHairColor` (`/Game/IS_CharacterCreator/Core/Item/Customization/BP_ACC_Face_Customization.CustomMesh` (`self.BP_Face_Customization`)))
    (`self.ApplyHairColor` (`self.GetHeadMesh`))))

(fn `ApplyBodyGPColor`
  (params (ColorParam :type "/Game/IS_CharacterCreator/Core/Data/Struct/Param/FStruct_ACC_ColorParam Structure (by ref)"))
  (bind (_identifier _type _value) (break `/Game/IS_CharacterCreator/Core/Data/Struct/Param/FStruct_ACC_ColorParam` ColorParam))
  (bind _headmesh (`self.GetHeadMesh`))
  (`parent.ApplyBodyGPColor` ColorParam)
  (`|ExecutionSequence`
    (:`then_0`
      ;[1 0 0.6328] Check Color Value Type
      (switch `name` _type
        (:`Material`
          (`|ExecutionSequence`
            (:`then_0`
              (`/Engine/EditorBlueprintResources/StandardMacros.IsValid` _headmesh
                (:`Is Valid`
                  (`self.UpdateObjectColor` _headmesh _identifier _value))))
            (:`then_1`
              (`self.UpdateObjectColor` (`self.GetBodyMesh`) _identifier _value))))
        (:`SkinColor`
          (`self.AppySkinColor`))))
    (:`then_1`
      (return))))

(fn `ApplyBodyGPFloat`
  (params (FloatParam :type "/Game/IS_CharacterCreator/Core/Data/Struct/Param/FStruct_ACC_FloatParam Structure"))
  (`parent.ApplyBodyGPFloat` FloatParam)
  ;[0 1 0.3672] Check Color Value Type
  (switch `name` (`.Type_4_AD0794D74C6B2A0A5E3306B4A8B21CE1` (break `/Game/IS_CharacterCreator/Core/Data/Struct/Param/FStruct_ACC_FloatParam` FloatParam))
    (:`BodyHeight`
      (`self.ApplyBodyHeight`)
      ;[1 0 0] OPC: BodyHeight
      (`self.FireParamChange` "BodyHeight"))))

(fn `ApplyCustomFace`
  (bind (_value _exist) (`self.GetGPIntValue` "HeadParams" "CustomFaceId"))
  (if _exist
    (bind _customtexturedata (`self.GetCustomTextureData` _value (`/Game/IS_CharacterCreator/Core/Object/DAO/BP_ACC_DAO_Head.GetCustomFaceDT` (`/Game/IS_CharacterCreator/Core/Object/DAO/BP_ACC_DAO.GetDAOHead` (`/Game/IS_CharacterCreator/Core/Library/BPFL_ACC_Common.GetACCDAO`))) "CustomFace_" (make `/Game/IS_CharacterCreator/Core/Data/Struct/Customization/FStruct_ACC_CustomTexture` "/Game/IS_CharacterCreator/TextureLibrary/Common/T_ACC_EmptyAlpha.T_ACC_EmptyAlpha")))
    (`MaterialInstanceDynamic.SetTextureParameterValue` (`self.HeadDynamicMaterial`) "T_Custom" (`.Texture_2_ACC6D25C4C3B8F0B8E0B3EB2A2225306` (break `/Game/IS_CharacterCreator/Core/Data/Struct/Customization/FStruct_ACC_CustomTexture` _customtexturedata)))))

(fn `ApplyEyeBrow`
  (params (Id :type Integer))
  (bind _eyebrowmaterial (`self.EyeBrowMaterial`))
  (bind _customtexturedata (`self.GetCustomTextureData` Id (`/Game/IS_CharacterCreator/Core/Object/DAO/BP_ACC_DAO_Head.GetEyeBrowDT` (`/Game/IS_CharacterCreator/Core/Object/DAO/BP_ACC_DAO.GetDAOHead` (`/Game/IS_CharacterCreator/Core/Library/BPFL_ACC_Common.GetACCDAO`))) "EB_" (make `/Game/IS_CharacterCreator/Core/Data/Struct/Customization/FStruct_ACC_CustomTexture` null)))
  (`/Engine/EditorBlueprintResources/StandardMacros.IsValid` _eyebrowmaterial
    (:`Is Valid`
      (`MaterialInstanceDynamic.SetTextureParameterValue` _eyebrowmaterial "T_Brow" (`.Texture_2_ACC6D25C4C3B8F0B8E0B3EB2A2225306` (break `/Game/IS_CharacterCreator/Core/Data/Struct/Customization/FStruct_ACC_CustomTexture` _customtexturedata)))
      (`self.ApplyHairColor` (`self.GetHeadMesh`)))))

(fn `ApplyGender`
  (bind (_bodymesh _animemesh) (`self.GetBodyMesh`))
  (bind (_skmesh _animinstance) (`self.SelectGenderMeshes`))
  (bind (_sourcemesh _outlinemesh) (`/Game/IS_CharacterCreator/Core/Library/BPFL_ACC_Extractor.GetAnimMesh` _animemesh))
  ;[0.5938 0 1] Reset body :
  ; - Unequip all, reset dynamic materials array
  (`self.ResetBody`)
  (`self.CheckInstanceCtm`)
  (`|ExecutionSequence`
    (:`then_0`
      ;[0 0.9766 1] Clear body anim inst
      (`SkeletalMeshComponent.SetAnimInstanceClass` (`self.GetRefMesh`) null) ; Ref mesh
      (`SkinnedMeshComponent.SetSkinnedAssetAndUpdate` _bodymesh _skmesh true)
      (`self.UpdateOutline` _sourcemesh _outlinemesh)
      (`self.InitBodyCopyRef`)
      ;[0.5703 1 0] Reclean and assign materials from new mesh
      (for (_array_element _array_index) (`SkeletalMesh.Materials` _skmesh)
        (`PrimitiveComponent.SetMaterial` (`self.GetBodyMesh`) _array_index (`.MaterialInterface` (break `SkeletalMaterial` _array_element)))))
    (:`then_1`
      ;[0 1 0.1328] If want use ABP from specie config
      (if (`self.GetBoolParam` "UseABP")
        (`SkeletalMeshComponent.SetAnimInstanceClass` (`self.GetRefMesh`) _animinstance) ; Ref mesh
      ))
    (:`then_2`
      ;[0 1 0.6953] Attack head to socket
      (`SceneComponent.K2_AttachToComponent` (`self.GetHeadMesh`) (`self.GetBodyMesh`) (`.HeadSocket_17_3B7050A64F8091BC6B1CDA98ECF9FD0D` (break `/Game/IS_CharacterCreator/Core/Data/Struct/FStruct_ACC_GenderConfig` (`self.GetCurrentGenderData`))) "SnapToTarget" "SnapToTarget" "KeepWorld" true))
    (:`then_3`
      ;[0.5234 1 0] Change SKMesh and AnimInstance from new Gender
      (`self.InitDynamicBodyMat`)
      (`self.ApplyAllParameters`)
      ;[1 0 0] OPC: Gender
      (`self.FireParamChange` "Gender"))))

(fn `ApplyHairColor`
  (params (Mesh :type "MeshComponent Object Reference"))
  (`self.UpdateObjectColor` Mesh "L3_Color" (`/Game/IS_CharacterCreator/Core/Library/BPFL_ACC_GroupParam.GetColorFromGP` (`self.GetGroupParamFromIdentifier` (`/Game/IS_CharacterCreator/Core/Library/BPFL_ACC_Constant.GetHairParamsKey`)) "L3_Color")))

(fn `ApplyHairGPColor`
  (params (ColorParam :type "/Game/IS_CharacterCreator/Core/Data/Struct/Param/FStruct_ACC_ColorParam Structure (by ref)"))
  (bind (_identifier _type _value) (break `/Game/IS_CharacterCreator/Core/Data/Struct/Param/FStruct_ACC_ColorParam` ColorParam))
  (`parent.ApplyHairGPColor` ColorParam)
  (`|ExecutionSequence`
    (:`then_0`
      ;[1 0.02344 0] Check Color Value Type
      (switch `name` _type
        (:`Material`
          (`self.UpdateObjectColor` (`self.GetHeadMesh`) _identifier _value))
        (:`HairColor`
          (`self.ApplyAllHair` true))))
    (:`then_1`
      (return))))

(fn `ApplyHairGPInt`
  (params (IntParam :type "/Game/IS_CharacterCreator/Core/Data/Struct/Param/FStruct_ACC_IntParam Structure (by ref)"))
  (bind (_identifier _type _value) (break `/Game/IS_CharacterCreator/Core/Data/Struct/Param/FStruct_ACC_IntParam` IntParam))
  (`parent.ApplyHairGPInt` IntParam)
  (`|ExecutionSequence`
    (:`then_0`
      (if (`KismetStringLibrary.StartsWith` (`KismetStringLibrary.Conv_NameToString` _type) "HairStyle")
        (`self.ApplyHairStyle` _value (`/Game/IS_CharacterCreator/Core/Library/BPFL_ACC_Common.ExtractHairStyleSuffix` _type))
        (else
          (switch `name` _type
            (:`HairTailSocket`
              ;[0 1 0.9062] HairTailSocket
              (`self.ApplyTailSocket` (`.Value_9_9FCA4F124E3FE5A4992336B2AFEAD7B4` (break `/Game/IS_CharacterCreator/Core/Data/Struct/Param/FStruct_ACC_IntParam` (`local.IntParam`)))))))))
    (:`then_1`
      (return))))

(fn `ApplyHairStyle`
  (params (HairId :type Integer) (HairType :type Name))
  (bind _bp_hair_customization (`self.BP_Hair_Customization`))
  (bind _hairtype (`local.HairType`))
  ;[0.03125 0 1] Apply hair only if found data
  (bind (_hairdata _success) (`self.GetHairMeshData` HairId HairType))
  (if _success
    ;[0 1 0.625] New Hair Style
    (`/Game/IS_CharacterCreator/Core/Item/Customization/Hair/BP_ACC_Hair_Ctm_Base.ChangeHairStyle` _bp_hair_customization _hairdata _hairtype)
    ;[0.05469 0 1] Apply Color
    (`self.ApplyHairColor` (`/Game/IS_CharacterCreator/Core/Item/Customization/Hair/BP_ACC_Hair_Ctm_Base.GetHairMeshFromType` _bp_hair_customization _hairtype))
    (else
      ;[0.5234 0 1] Remove Hair
      (`/Game/IS_CharacterCreator/Core/Item/Customization/Hair/BP_ACC_Hair_Ctm_Base.ChangeHairStyle` (`self.BP_Hair_Customization`) (make `/Game/IS_CharacterCreator/Core/Data/Struct/Customization/FStruct_ACC_HairData` 0 null null) (`local.HairType`)))))

(fn `ApplyHdGPColor`
  (params (ColorParam :type "/Game/IS_CharacterCreator/Core/Data/Struct/Param/FStruct_ACC_ColorParam Structure (by ref)"))
  (bind (_identifier _type _value) (break `/Game/IS_CharacterCreator/Core/Data/Struct/Param/FStruct_ACC_ColorParam` ColorParam))
  (`parent.ApplyHdGPColor` ColorParam)
  (`|ExecutionSequence`
    (:`then_0`
      ;[0.2656 1 0] Check Color Value Type
      (switch `name` _type
        (:`Material`
          (`self.UpdateObjectColor` (`self.GetHeadMesh`) _identifier _value))))
    (:`then_1`
      (return))))

(fn `ApplyHdGPFloat`
  (params (FloatParam :type "/Game/IS_CharacterCreator/Core/Data/Struct/Param/FStruct_ACC_FloatParam Structure"))
  (bind (_identifier _type _value) (break `/Game/IS_CharacterCreator/Core/Data/Struct/Param/FStruct_ACC_FloatParam` FloatParam))
  (`parent.ApplyHdGPFloat` FloatParam)
  (switch `name` _type
    (:`EyeMaterial`
      ;[0 0.7891 1] Eye Material Float Param
      (for _array_element (`self.EyeMaterial`)
        (`MaterialInstanceDynamic.SetScalarParameterValue` _array_element _identifier _value)))))

(fn `ApplyHdGPInt`
  (params (IntParam :type "/Game/IS_CharacterCreator/Core/Data/Struct/Param/FStruct_ACC_IntParam Structure (by ref)"))
  (bind (_identifier _type _value) (break `/Game/IS_CharacterCreator/Core/Data/Struct/Param/FStruct_ACC_IntParam` IntParam))
  (`parent.ApplyHdGPInt` IntParam)
  (`|ExecutionSequence`
    (:`then_0`
      (switch `name` _type
        (:`IrisStyle`
          (`self.ApplyIris` _value))
        (:`EyeBrowStyle`
          (`self.ApplyEyeBrow` _value))
        (:`HeadStyle`
          (`self.ApplyHeadStyle`))))
    (:`then_1`
      (return))))

(fn `ApplyHeadParam`
  (bind (_identifier _intparamlist _floatparamlist _colorparamlist) (break `/Game/IS_CharacterCreator/Core/Data/Struct/Param/FStruct_ACC_GroupParam` (`self.GetGroupParamFromIdentifier` (`/Game/IS_CharacterCreator/Core/Library/BPFL_ACC_Constant.GetHeadParamsKey`))))
  (`|ExecutionSequence`
    (:`then_0`
      (bind _values (`BlueprintMapLibrary.Map_Values` _intparamlist))
      (for _array_element _values
        ;[1 0 0.7266] Check if not "HeadStyle" to avoid infinite loop
        (if (!= (`.Type_4_AD0794D74C6B2A0A5E3306B4A8B21CE1` (break `/Game/IS_CharacterCreator/Core/Data/Struct/Param/FStruct_ACC_IntParam` _array_element)) "HeadStyle")
          (`self.ApplyHdGPInt` _array_element))))
    (:`then_1`
      (bind _values_2 (`BlueprintMapLibrary.Map_Values` _floatparamlist))
      (for _array_element_2 _values_2
        (`self.ApplyHdGPFloat` _array_element_2)))
    (:`then_2`
      (bind _values_3 (`BlueprintMapLibrary.Map_Values` _colorparamlist))
      (for _array_element_3 _values_3
        (`self.ApplyHdGPColor` _array_element_3)))))

(fn `ApplyHeadStyle`
  (locals (CurrentHeadData :type Boolean))
  ;[0 0.6016 1] If head exist
  (`/Engine/EditorBlueprintResources/StandardMacros.IsValid` (`self.GetHeadMesh`)
    (:`Is Valid`
      ;[1 0.1172 0] Get data if exist
      (bind (_headdata _exist) (`self.GetHeadMeshData` (`self.GetGPIntValue` "HeadParams" "HeadIndex")))
      (if _exist
        ;[0 0.6953 1] Store head data
        (set `self.HeadData` _headdata)))))

(fn `ApplyIris`
  (params (Id :type Integer))
  (bind _customtexturedata (`/Game/IS_CharacterCreator/Core/Object/DAO/BP_ACC_DAO_Head.GetIrisData` (`/Game/IS_CharacterCreator/Core/Object/DAO/BP_ACC_DAO.GetDAOHead` (`/Game/IS_CharacterCreator/Core/Library/BPFL_ACC_Common.GetACCDAO`)) Id))
  (for _array_element (`self.EyeMaterial`)
    (`MaterialInstanceDynamic.SetTextureParameterValue` _array_element "T_Iris" (`.Texture_2_ACC6D25C4C3B8F0B8E0B3EB2A2225306` (break `/Game/IS_CharacterCreator/Core/Data/Struct/Customization/FStruct_ACC_CustomTexture` _customtexturedata))))
  (return))

(fn `ApplyTailSocket`
  (params (SocketId :type Integer))
  (`/Game/IS_CharacterCreator/Core/Item/Customization/Hair/BP_ACC_Hair_Ctm_Base.UpdateTailSocket` (`self.BP_Hair_Customization`) SocketId))

(fn `AppySkinColor`
  (bind _headmesh (`self.GetHeadMesh`))
  (bind _value (`/Game/IS_CharacterCreator/Core/Library/BPFL_ACC_GroupParam.GetColorFromGP` (`self.GetGroupParamFromIdentifier` (`/Game/IS_CharacterCreator/Core/Library/BPFL_ACC_Constant.GetBodyParamsKey`)) "L1_Color"))
  (`self.UpdateObjectColor` (`self.GetBodyMesh`) "L1_Color" _value)
  ;[1 0.2812 0] Head part
  (`/Engine/EditorBlueprintResources/StandardMacros.IsValid` _headmesh
    (:`Is Valid`
      (`self.UpdateObjectColor` _headmesh "L1_Color" _value))))

(fn `CheckInstanceCtm`
  (bind _bp_hair_customization (`self.BP_Hair_Customization`))
  (bind (_skmesh _defaultaniminst _headaniminst _hairctmclass) (break `/Game/IS_CharacterCreator/Core/Data/Struct/FStruct_ACC_GenderConfig` (`self.GetCurrentGenderData`)))
  (`parent.CheckInstanceCtm`)
  (`|ExecutionSequence`
    (:`then_0`
      (if (!= _hairctmclass (`GameplayStatics.GetObjectClass` (`self.BP_Hair_Customization`)))
        (`|ExecutionSequence`
          (:`then_0`
            ;[1 0 0.9844] Destroy before if want to replace
            (`/Engine/EditorBlueprintResources/StandardMacros.IsValid` _bp_hair_customization
              (:`Is Valid`
                (`Actor.K2_DestroyActor` _bp_hair_customization))))
          (:`then_1`
            ;[0 1 0.1328] Instance Hair
            (bind _returnvalue (`|SpawnActorFromClass` _hairctmclass (`KismetMathLibrary.MakeTransform` (0.0 0.0 0.0)) "Undefined" "OverrideRootScale" null self null))
            (bind _output_get (set `self.BP_Hair_Customization` _returnvalue))
            (`/Game/IS_CharacterCreator/Core/Item/Customization/Hair/BP_ACC_Hair_Ctm_Base.InitVariables` _output_get (`self.GetPossesor`))
            (`Actor.K2_AttachToComponent` (`self.BP_Hair_Customization`) (`self.GetHeadMesh`) (`self.GetHairSocket`) "SnapToTarget" "SnapToTarget" "SnapToTarget" true)))))
    (:`then_1`
      ;[0.2422 1 0] If first time
      (`/Engine/EditorBlueprintResources/StandardMacros.IsValid` (`self.BP_Face_Customization`)
        (:`Is Not Valid`
          ;[0 0.4375 1] Face Customization (Bearb for exemple)
          (bind _returnvalue_2 (`|SpawnActorFromClass` "/Game/IS_CharacterCreator/Core/Item/Customization/BP_ACC_Face_Customization.BP_ACC_Face_Customization_C" (`KismetMathLibrary.MakeTransform` (0.0 0.0 0.0)) "Undefined" "OverrideRootScale" null self null))
          (bind _output_get_2 (set `self.BP_Face_Customization` _returnvalue_2))
          (`/Game/IS_CharacterCreator/Core/Item/Customization/BP_ACC_Face_Customization.InitCustomMesh` _output_get_2 (`self.GetPossesor`) self))))
    (:`then_2`
      (return))))

(fn `GetHairMeshData`
  (params (id :type Integer) (Type :type Name))
  (returns (HairData :type "/Game/IS_CharacterCreator/Core/Data/Struct/Customization/FStruct_ACC_HairData Structure") (Success :type Boolean))
  (bind (_specieidentifier _maturity _gender) (`self.GetSpecieInformation`))
  (bind (_hairdata _success) (`/Game/IS_CharacterCreator/Core/Object/DAO/BP_ACC_DAO_Head.GetHairDataAdvanced` (`/Game/IS_CharacterCreator/Core/Object/DAO/BP_ACC_DAO.GetDAOHead` (`/Game/IS_CharacterCreator/Core/Library/BPFL_ACC_Common.GetACCDAO`)) id (`self.GetHairSpeciePrefix`) _maturity _gender))
  (return _hairdata _success))

(fn `GetHairSocket`
  (returns (Socket :type Name))
  (return (`/Game/IS_CharacterCreator/Core/Library/BPFL_ACC_Common.TextToName` (`|FormatText` "{headKind}_HairSocket" (`.HeadKindIdentifier_5_E4EDFABB4D6BC79AB11849B1AD1855E1` (break `/Game/IS_CharacterCreator/Core/Data/Struct/FStruct_ACC_CustomConfParam` (`.CustomConf_16_9952A7684B7AF3A6E39087B165AB2F7F` (break `/Game/IS_CharacterCreator/Core/Data/Struct/FStruct_ACC_SpecieParam` (`self.SpecieConfiguration`)))))))))

(fn `GetHeadMeshData`
  (params (id :type Integer))
  (returns (HeadData :type "/Game/IS_CharacterCreator/Core/Data/Struct/Customization/FStruct_ACC_HeadData Structure") (Exist :type Boolean))
  (bind (_specieidentifier _maturity _gender) (`self.GetSpecieInformation`))
  (bind (_headdata _success) (`/Game/IS_CharacterCreator/Core/Object/DAO/BP_ACC_DAO_Head.GetHeadData` (`/Game/IS_CharacterCreator/Core/Object/DAO/BP_ACC_DAO.GetDAOHead` (`/Game/IS_CharacterCreator/Core/Library/BPFL_ACC_Common.GetACCDAO`)) (`/Game/IS_CharacterCreator/Core/Library/BPFL_ACC_Common.BuildSpecieDTKey` id _specieidentifier _maturity _gender)))
  (return _headdata _success))