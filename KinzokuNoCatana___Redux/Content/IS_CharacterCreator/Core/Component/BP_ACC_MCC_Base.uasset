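; Base character-creator component that customizes its owner's species, maturity, gender and appearance, reaching meshes through interface messages.
; Species configuration supplies per-maturity and gender meshes and anim classes; gender changes rebuild body materials and reapply parameters.
; Int, float and color parameters live in named groups, dispatched to head, hair and body handlers, many empty for overriding.
; Changes notify owner and listeners; InitFromACCCharDataAsync queues data until initialization completes.
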(event `self.ReceiveBeginPlay`
  (`parent.ReceiveBeginPlay`))

(event `self.ReceiveTick`
  (params (DeltaSeconds :type "Float (single-precision)"))
  (`parent.ReceiveTick` DeltaSeconds))

(fn `ApplyAllGroupParam`
  (bind _groupparamlist (`self.GroupParamList`))
  (bind _keys (`BlueprintMapLibrary.Map_Keys` _groupparamlist))
  (for _array_element _keys
    (`|ExecutionSequence`
      (:`then_0`
        (bind (_identifier _intparamlist _floatparamlist _colorparamlist) (break `/Game/IS_CharacterCreator/Core/Data/Struct/Param/FStruct_ACC_GroupParam` (`BlueprintMapLibrary.Map_Find` _groupparamlist _array_element)))
        ;[0.125 1 0] Apply All Int Param
        (bind _values (`BlueprintMapLibrary.Map_Values` _intparamlist))
        (for _array_element_2 _values
          (bind (_identifier_2 _type _value) (break `/Game/IS_CharacterCreator/Core/Data/Struct/Param/FStruct_ACC_IntParam` _array_element_2))
          (`self.ApplyGPInt` _identifier _identifier_2 _type _value)))
      (:`then_1`
        ;[1 0.2344 0] Apply All Float Param
        (bind _values_2 (`BlueprintMapLibrary.Map_Values` _floatparamlist))
        (for _array_element_3 _values_2
          (bind (_identifier_3 _type_2 _value_2) (break `/Game/IS_CharacterCreator/Core/Data/Struct/Param/FStruct_ACC_FloatParam` _array_element_3))
          (`self.ApplyGPFloat` _identifier _identifier_3 _type_2 _value_2)))
      (:`then_2`
        ;[0.6641 0 1] Apply All Color Param
        (bind _values_3 (`BlueprintMapLibrary.Map_Values` _colorparamlist))
        (for _array_element_4 _values_3
          (bind (_identifier_4 _type_3 _value_3) (break `/Game/IS_CharacterCreator/Core/Data/Struct/Param/FStruct_ACC_ColorParam` _array_element_4))
          (`self.ApplyGPColor` _identifier _identifier_4 _type_3 _value_3))))))

(fn `ApplyAllParameters`
  (`self.ApplyAllGroupParam`)
  ;[0.8047 0 1] Notify all data has changed
  (`self.OnChangeAnyData`))

(fn `ApplyBodyGPColor`
  (params (ColorParam :type "/Game/IS_CharacterCreator/Core/Data/Struct/Param/FStruct_ACC_ColorParam Structure (by ref)"))
  (return))

(fn `ApplyBodyGPFloat`
  (params (FloatParam :type "/Game/IS_CharacterCreator/Core/Data/Struct/Param/FStruct_ACC_FloatParam Structure"))
  ;[0 1 0.8828] Apply Common Float Param
  (`self.ApplyCmnFloatParam` (`self.GetBodyMesh`) FloatParam))

(fn `ApplyBodyGPInt`
  (params (IntParam :type "/Game/IS_CharacterCreator/Core/Data/Struct/Param/FStruct_ACC_IntParam Structure (by ref)"))
  ;[0.8984 1 0] To Override
  (return))

(fn `ApplyBodyHeight`)

(fn `ApplyCmnFloatParam`
  (params (Mesh :type "SkeletalMeshComponent Object Reference") (FloatParam :type "/Game/IS_CharacterCreator/Core/Data/Struct/Param/FStruct_ACC_FloatParam Structure"))
  (bind (_identifier _type _value) (break `/Game/IS_CharacterCreator/Core/Data/Struct/Param/FStruct_ACC_FloatParam` FloatParam))
  (bind _mesh (`local.Mesh`))
  (switch `name` _type
    (:`Morph`
      (`self.SetGlobalMorphTarget` _identifier _mesh _value))
    (:`Material`
      (`MeshComponent.SetScalarParameterValueOnMaterials` _mesh _identifier _value))))

(fn `ApplyFloatParam`
  (params (FloatParam :type "/Game/IS_CharacterCreator/Core/Data/Struct/Param/FStruct_ACC_FloatParam Structure") (Reset :type Boolean) (MeshTarget :type "MeshComponent Object Reference"))
  (bind (_identifier _type _value) (break `/Game/IS_CharacterCreator/Core/Data/Struct/Param/FStruct_ACC_FloatParam` (`local.FloatParam`)))
  (switch `name` (`.Type_4_AD0794D74C6B2A0A5E3306B4A8B21CE1` (break `/Game/IS_CharacterCreator/Core/Data/Struct/Param/FStruct_ACC_FloatParam` FloatParam))
    (:`Material`
      (`MeshComponent.SetScalarParameterValueOnMaterials` (`local.MeshTarget`) _identifier (`KismetMathLibrary.SelectFloat` 0.0 _value (`local.Reset`))))))

(fn `ApplyGender`
  (bind (_bodymesh _animemesh) (`self.GetBodyMesh`))
  (bind (_skmesh _animinstance) (`self.SelectGenderMeshes`))
  (bind (_sourcemesh _outlinemesh) (`/Game/IS_CharacterCreator/Core/Library/BPFL_ACC_Extractor.GetAnimMesh` _animemesh))
  ;[0.5938 0 1] Reset body :
  ; - Unequip all, reset dynamic materials array
  (`self.ResetBody`)
  (`self.CheckInstanceCtm`)
  (`|ExecutionSequence`
    (:`then_0`
      ;[0 0.9766 1] Clear body anim inst
      (`SkeletalMeshComponent.SetAnimInstanceClass` (`self.GetRefMesh`) null) ; Ref mesh
      (`SkinnedMeshComponent.SetSkinnedAssetAndUpdate` _bodymesh _skmesh true)
      (`self.UpdateOutline` _sourcemesh _outlinemesh)
      (`self.InitBodyCopyRef`)
      ;[0.5703 1 0] Reclean and assign materials from new mesh
      (for (_array_element _array_index) (`SkeletalMesh.Materials` _skmesh)
        (`PrimitiveComponent.SetMaterial` (`self.GetBodyMesh`) _array_index (`.MaterialInterface` (break `SkeletalMaterial` _array_element)))))
    (:`then_1`
      ;[0 1 0.1328] If want use ABP from specie config
      (if (`self.GetBoolParam` "UseABP")
        (`SkeletalMeshComponent.SetAnimInstanceClass` (`self.GetRefMesh`) _animinstance) ; Ref mesh
      ))
    (:`then_2`
      ;[0.5234 1 0] Change SKMesh and AnimInstance from new Gender
      (`self.InitDynamicBodyMat`)
      (`self.ApplyAllParameters`)
      ;[1 0 0] OPC: Gender
      (`self.FireParamChange` "Gender"))))

(fn `ApplyGPColor`
  (params (GroupParamIdentifier :type Name) (Identifier :type Name) (Type :type Name) (Value :type "LinearColor Structure"))
  (bind (_colorparam _exist) (`/Game/IS_CharacterCreator/Core/Library/BPFL_ACC_GroupParam.GetColorParamFromGP` (`self.GetGroupParamFromIdentifier` GroupParamIdentifier) Identifier))
  (if _exist
    (switch `name` (`local.GroupParamIdentifier`)
      (:`HeadParams`
        (`self.ApplyHdGPColor` _colorparam))
      (:`HairParams`
        (`self.ApplyHairGPColor` _colorparam))
      (:`BodyParams`
        (`self.ApplyBodyGPColor` _colorparam)))))

(fn `ApplyGPFloat`
  (params (GroupParamIdentifier :type Name) (Identifier :type Name) (Type :type Name) (Value :type "Float (double-precision)"))
  (bind (_floatparam _exist) (`self.GetGPFloatFromGP` (`self.GetGroupParamFromIdentifier` GroupParamIdentifier) Identifier))
  (if _exist
    (switch `name` (`local.GroupParamIdentifier`)
      (:`HeadParams`
        (`self.ApplyHdGPFloat` _floatparam))
      (:`HairParams`
        (`self.ApplyHairGPFloat` _floatparam))
      (:`BodyParams`
        (`self.ApplyBodyGPFloat` _floatparam)))))

(fn `ApplyGPInt`
  (params (GroupParamIdentifier :type "Name (by ref)") (Identifier :type Name) (Type :type Name) (Value :type Integer))
  (bind (_value _exist) (`self.GetGPIntFromGP` (`self.GetGroupParamFromIdentifier` GroupParamIdentifier) Identifier))
  (if _exist
    (switch `name` (`local.GroupParamIdentifier`)
      (:`HeadParams`
        (`self.ApplyHdGPInt` _value))
      (:`HairParams`
        (`self.ApplyHairGPInt` _value)))))

(fn `ApplyHairGPColor`
  (params (ColorParam :type "/Game/IS_CharacterCreator/Core/Data/Struct/Param/FStruct_ACC_ColorParam Structure (by ref)"))
  (return))

(fn `ApplyHairGPFloat`
  (params (FloatParam :type "/Game/IS_CharacterCreator/Core/Data/Struct/Param/FStruct_ACC_FloatParam Structure"))
  (return))

(fn `ApplyHairGPInt`
  (params (IntParam :type "/Game/IS_CharacterCreator/Core/Data/Struct/Param/FStruct_ACC_IntParam Structure (by ref)"))
  (return))

(fn `ApplyHdGPColor`
  (params (ColorParam :type "/Game/IS_CharacterCreator/Core/Data/Struct/Param/FStruct_ACC_ColorParam Structure (by ref)"))
  (return))

(fn `ApplyHdGPFloat`
  (params (FloatParam :type "/Game/IS_CharacterCreator/Core/Data/Struct/Param/FStruct_ACC_FloatParam Structure"))
  ;[1 0.8438 0] Apply Common Float Param
  (`self.ApplyCmnFloatParam` (`self.GetHeadMesh`) FloatParam))

(fn `ApplyHdGPInt`
  (params (IntParam :type "/Game/IS_CharacterCreator/Core/Data/Struct/Param/FStruct_ACC_IntParam Structure (by ref)"))
  (return))

(fn `ApplyItemFloatParam`
  (params (ItemData :type "/Game/IS_CharacterCreator/Core/Data/Struct/Common/FStruct_ACC_ItemData Structure") (MeshTarget :type "MeshComponent Object Reference") (Reset :type Boolean))
  (for _array_element (`/Game/IS_CharacterCreator/Core/Library/BPFL_ACC_Common.GetItemFloatParamList` ItemData)
    (bind (_identifier _type _value) (break `/Game/IS_CharacterCreator/Core/Data/Struct/Param/FStruct_ACC_FloatParam` _array_element))
    ;[0.5938 0 1] Put float value in char group param
    (`self.ChangeGroupParamFloat` "Other" _identifier _type (`KismetMathLibrary.SelectFloat` 0.0 _value Reset)))
  ;[0.1484 0 1] Apply Other (Ohter it's like Extra) Float Group Param
  (bind _values (`BlueprintMapLibrary.Map_Values` (`.FloatParamList_11_BB7DF942497FBCFDA5A1F8AC3FE12DC2` (break `/Game/IS_CharacterCreator/Core/Data/Struct/Param/FStruct_ACC_GroupParam` (`self.GetGroupParamFromIdentifier` "Other")))))
  (for _array_element_2 _values
    (`self.ApplyFloatParam` _array_element_2 Reset MeshTarget)))

(fn `BuildItemIdentifier`
  (params (Other :type Name))
  (returns (Identifier :type Name))
  (bind (_specieidentifier _maturity _gender) (`self.GetSpecieInformation`))
  (return (`/Game/IS_CharacterCreator/Core/Library/BPFL_ACC_Common.TextToName` (`|FormatText` "{specie}_{maturity}_{gender}_{other}" _specieidentifier (`/Game/IS_CharacterCreator/Core/Library/BPFL_ACC_Constant.GetMaturityKey` _maturity) (`/Game/IS_CharacterCreator/Core/Library/BPFL_ACC_Constant.GetGenderKey` _gender) Other))))

(fn `ChangeGender`
  (params (NewGender :type "/Game/IS_CharacterCreator/Core/Data/Enum/E_ACC_Gender Enum" :default "NewEnumerator0"))
  (set `self.Gender` NewGender)
  (`self.ApplyGender`))

(fn `ChangeGroupParamColor`
  (params (GroupParamIdentifier :type Name) (Identifier :type Name) (Type :type Name) (Value :type "LinearColor Structure"))
  (bind _groupparam (`self.GetGroupParamFromIdentifier` GroupParamIdentifier))
  (bind (_identifier _intparamlist _floatparamlist _colorparamlist) (break `/Game/IS_CharacterCreator/Core/Data/Struct/Param/FStruct_ACC_GroupParam` _groupparam))
  ;[1 0.6797 0] Change the value and update the entire struct
  (bind _newvalues (`/Game/IS_CharacterCreator/Core/Library/BPFL_ACC_GroupParam.ChangeColorParam` _colorparamlist Identifier Type Value))
  (bind _structout (setmembers `/Game/IS_CharacterCreator/Core/Data/Struct/Param/FStruct_ACC_GroupParam` :`StructRef` _groupparam :`ColorParamList` _newvalues))
  (`BlueprintMapLibrary.Map_Add` (`self.GroupParamList`) _identifier _structout)
  ;[0.8281 0 1] Apply Change
  (`self.ApplyGPColor` (`local.GroupParamIdentifier`) (`local.Identifier`) (`local.Type`) (`local.Value`))
  ;[0.6967 1 0.9194] Notify data changed
  (`self.OnChangeAnyData`))

(fn `ChangeGroupParamFloat`
  (params (GroupParamIdentifier :type Name) (Identifier :type Name) (Type :type Name) (Value :type "Float (double-precision)"))
  (bind _groupparam (`self.GetGroupParamFromIdentifier` GroupParamIdentifier))
  (bind (_identifier _intparamlist _floatparamlist) (break `/Game/IS_CharacterCreator/Core/Data/Struct/Param/FStruct_ACC_GroupParam` _groupparam))
  (`|ExecutionSequence`
    (:`then_0`
      ;[0 1 0.1797] If group not exist, create empty
      (`/Game/IS_CharacterCreator/Core/Library/BPFL_ACC_GroupParam.CreateEmptyGroupParam` (`self.GroupParamList`) (`local.GroupParamIdentifier`)))
    (:`then_1`
      ;[0 0.3203 1] Change the value and update the entire struct
      (bind _newvalues (`/Game/IS_CharacterCreator/Core/Library/BPFL_ACC_GroupParam.ChangeFloatParam` _floatparamlist Identifier Type Value))
      (bind _structout (setmembers `/Game/IS_CharacterCreator/Core/Data/Struct/Param/FStruct_ACC_GroupParam` :`StructRef` _groupparam :`FloatParamList` _newvalues))
      (`BlueprintMapLibrary.Map_Add` (`self.GroupParamList`) _identifier _structout)
      ;[0 0.6719 1] Apply Change
      (`self.ApplyGPFloat` (`local.GroupParamIdentifier`) (`local.Identifier`) (`local.Type`) (`local.Value`))
      ;[0.6967 1 0.9194] Notify data changed
      (`self.OnChangeAnyData`))))

(fn `ChangeGroupParamInt`
  (params (GroupParamIdentifier :type Name) (Identifier :type Name) (Type :type Name) (Value :type Integer))
  (bind _groupparam (`self.GetGroupParamFromIdentifier` GroupParamIdentifier))
  (bind (_identifier _intparamlist) (break `/Game/IS_CharacterCreator/Core/Data/Struct/Param/FStruct_ACC_GroupParam` _groupparam))
  ;[1 0 0.5156] Change the value and update the entire struct
  (bind _newvalues (`/Game/IS_CharacterCreator/Core/Library/BPFL_ACC_GroupParam.ChangeIntParam` _intparamlist Identifier Type Value))
  (bind _structout (setmembers `/Game/IS_CharacterCreator/Core/Data/Struct/Param/FStruct_ACC_GroupParam` :`StructRef` _groupparam :`IntParamList` _newvalues))
  (`BlueprintMapLibrary.Map_Add` (`self.GroupParamList`) _identifier _structout)
  ;[0 1 0.3438] Apply Change
  (`self.ApplyGPInt` (`local.GroupParamIdentifier`) (`local.Identifier`) (`local.Type`) (`local.Value`))
  ;[0.6967 1 0.9194] Notify data changed
  (`self.OnChangeAnyData`))

(fn `ChangeMaturity`
  (params (NewMaturity :type "/Game/IS_CharacterCreator/Core/Data/Enum/E_ACC_Maturity Enum" :default "NewEnumerator0"))
  (set `self.Maturity` NewMaturity)
  ;[1 0.7734 0] Notify to Character Maturity Change
  (message `/Game/IS_CharacterCreator/Core/Interface/BPI_ACC_CharacterCustomization.I_OnMaturityChange` (`self.GetPossesor`) (`self.Maturity`))
  ;[1 0 0] OPC: Maturity
  (`self.FireParamChange` "Maturity"))

(fn `ChangeSpecie`
  (params (SpecieIdentifier :type Name))
  (bind _output_get (set `self.SpecieIdentifier` SpecieIdentifier))
  (set `self.SpecieConfiguration` (`/Game/IS_CharacterCreator/Core/Object/DAO/BP_ACC_DAO.GetSpecie` (`/Game/IS_CharacterCreator/Core/Library/BPFL_ACC_Common.GetACCDAO`) _output_get))
  ;[0.5 0 1] Clear
  (`self.ClearSpecie`)
  ;[1 0 0] OPC: Specie
  (`self.FireParamChange` "Specie"))

(fn `CheckInstanceCtm`
  ;[0 1 0.25] To override
  (return))

(fn `ClearSpecie`
  ;[0.7109 0 1] Clear Body Mats
  (`KismetArrayLibrary.Array_Clear` (`self.BodyDynamicMaterials`))
  ;[1 0.3281 0] Clear eye
  (`KismetArrayLibrary.Array_Clear` (`self.EyeMaterial`)))

(fn `ComputeTags`)

(fn `DestroyAll`
  (bind _bp_hair_customization (`self.BP_Hair_Customization`))
  (bind _bp_face_customization (`self.BP_Face_Customization`))
  (`|ExecutionSequence`
    (:`then_0`
      ;[0 0.8359 1] Destroy Hair
      (`/Engine/EditorBlueprintResources/StandardMacros.IsValid` _bp_hair_customization
        (:`Is Valid`
          (`Actor.K2_DestroyActor` _bp_hair_customization))))
    (:`then_1`
      ;[1 0.09375 0] Destroy Face Customization
      (`/Engine/EditorBlueprintResources/StandardMacros.IsValid` _bp_face_customization
        (:`Is Valid`
          (`Actor.K2_DestroyActor` _bp_face_customization))))))

(fn `FireParamChange`
  (params (ParamName :type Name))
  ;[1 0 0] OPC: Gender
  (`self.OnParamChange` ParamName))

(fn `GetACCCharData`
  (returns (ACC_Character :type "/Game/IS_CharacterCreator/Core/Data/Struct/FStruct_ACC_Character Structure"))
  (bind _charctmdata (`self.GetCharCustomizationData`))
  (return (make `/Game/IS_CharacterCreator/Core/Data/Struct/FStruct_ACC_Character` "Anonymous" "Anonymous" _charctmdata)))

(fn `GetAnimInstance`
  (returns (ReturnValue :type "AnimInstance Object Reference"))
  (return (`SkeletalMeshComponent.GetAnimInstance` (`self.GetRefMesh`))))

(fn `GetAttachMeshTarget`
  (params (AttachTarget :type "/Game/IS_CharacterCreator/Core/Data/Enum/E_ACC_AttachTarget Enum" :default "NewEnumerator0"))
  (returns (Mesh :type "SkeletalMeshComponent Object Reference"))
  (return (select `/Game/IS_CharacterCreator/Core/Data/Enum/E_ACC_AttachTarget` AttachTarget :`NewEnumerator0` (`self.GetBodyMesh`) :`NewEnumerator1` (`self.GetHeadMesh`))))

(fn `GetBodyMesh`
  (returns (BodyMesh :type "SkeletalMeshComponent Object Reference") (AnimeMesh :type "/Game/IS_CharacterCreator/Core/Data/Struct/FStruct_ACC_AnimeMesh Structure"))
  ;[0.3828 1 0] Interface to get body mesh for easier integration
  (bind (_mesh _animemesh) (message `/Game/IS_CharacterCreator/Core/Interface/BPI_ACC_CharacterCustomization.I_GetBodyMesh` (`self.GetPossesor`)))
  (return _mesh _animemesh))

(fn `GetBoolParam`
  (params (Key :type Name))
  (returns (Value :type Boolean))
  (return (`BlueprintMapLibrary.Map_Find` (`self.BoolParams`) Key)))

(fn `GetCharCustomizationData`
  (returns (CharCtmData :type "/Game/IS_CharacterCreator/Core/Data/Struct/Customization/FStruct_ACC_CharacterCustom Structure"))
  (return (make `/Game/IS_CharacterCreator/Core/Data/Struct/Customization/FStruct_ACC_CharacterCustom` (`self.SpecieIdentifier`) (`self.Maturity`) (`self.Gender`) (`self.GroupParamList`))))

(fn `GetCurrentGenderData`
  (returns (GenderData :type "/Game/IS_CharacterCreator/Core/Data/Struct/FStruct_ACC_GenderConfig Structure"))
  (return (`self.GetOneGenderData` (`self.Maturity`) (`self.Gender`))))

(fn `GetCustomTextureData`
  (params (Id :type Integer) (DataTable :type "DataTable Object Reference") (Prefix :type Name) (Default :type "/Game/IS_CharacterCreator/Core/Data/Struct/Customization/FStruct_ACC_CustomTexture Structure"))
  (returns (CustomTextureData :type "/Game/IS_CharacterCreator/Core/Data/Struct/Customization/FStruct_ACC_CustomTexture Structure"))
  (bind _returnvalue (`|GetDataTableRow` DataTable (`KismetStringLibrary.Conv_StringToName` (`KismetStringLibrary.Concat_StrStr` (`KismetStringLibrary.Conv_NameToString` Prefix) (`KismetStringLibrary.Conv_IntToString` Id))))
    (:`then`
      (return _returnvalue))
    (:`RowNotFound`
      (return Default))))

(fn `GetDynamicBodyMats`
  (returns (BodyDynamicMaterials :type "Array of MaterialInstanceDynamic Object Reference"))
  (return (`self.BodyDynamicMaterials`)))

(fn `GetGPFloatFromGP`
  (params (GroupParam :type "/Game/IS_CharacterCreator/Core/Data/Struct/Param/FStruct_ACC_GroupParam Structure (by ref)") (Identifier :type Name))
  (returns (FloatParam :type "/Game/IS_CharacterCreator/Core/Data/Struct/Param/FStruct_ACC_FloatParam Structure") (Exist :type Boolean))
  (bind (_value _returnvalue) (`BlueprintMapLibrary.Map_Find` (`.FloatParamList_11_BB7DF942497FBCFDA5A1F8AC3FE12DC2` (break `/Game/IS_CharacterCreator/Core/Data/Struct/Param/FStruct_ACC_GroupParam` GroupParam)) Identifier))
  (return _value _returnvalue))

(fn `GetGPFloatValueFromGP`
  (params (GroupParam :type "/Game/IS_CharacterCreator/Core/Data/Struct/Param/FStruct_ACC_GroupParam Structure (by ref)") (Identifier :type Name))
  (returns (Value :type "Float (double-precision)") (Exist :type Boolean))
  (bind (_floatparam _exist) (`self.GetGPFloatFromGP` GroupParam Identifier))
  (return (`.Value_5_9FCA4F124E3FE5A4992336B2AFEAD7B4` (break `/Game/IS_CharacterCreator/Core/Data/Struct/Param/FStruct_ACC_FloatParam` _floatparam)) _exist))

(fn `GetGPIntFromGP`
  (params (GroupParam :type "/Game/IS_CharacterCreator/Core/Data/Struct/Param/FStruct_ACC_GroupParam Structure (by ref)") (Identifier :type Name))
  (returns (Value :type "/Game/IS_CharacterCreator/Core/Data/Struct/Param/FStruct_ACC_IntParam Structure") (Exist :type Boolean))
  (bind (_value _returnvalue) (`BlueprintMapLibrary.Map_Find` (`.IntParamList_6_03F5988F47C559338AD1C6A821043712` (break `/Game/IS_CharacterCreator/Core/Data/Struct/Param/FStruct_ACC_GroupParam` GroupParam)) Identifier))
  (return _value _returnvalue))

(fn `GetGPIntValue`
  (params (GroupParamIdentifier :type Name) (Identifier :type Name))
  (returns (Value :type Integer) (Exist :type Boolean))
  (bind (_value _returnvalue) (`BlueprintMapLibrary.Map_Find` (`.IntParamList_6_03F5988F47C559338AD1C6A821043712` (break `/Game/IS_CharacterCreator/Core/Data/Struct/Param/FStruct_ACC_GroupParam` (`self.GetGroupParamFromIdentifier` GroupParamIdentifier))) Identifier))
  (return (`.Value_9_9FCA4F124E3FE5A4992336B2AFEAD7B4` (break `/Game/IS_CharacterCreator/Core/Data/Struct/Param/FStruct_ACC_IntParam` _value)) _returnvalue))

(fn `GetGPIntValueFromGP`
  (params (GroupParam :type "/Game/IS_CharacterCreator/Core/Data/Struct/Param/FStruct_ACC_GroupParam Structure (by ref)") (Identifier :type Name))
  (returns (Value :type Integer) (Exist :type Boolean))
  (bind (_value _returnvalue) (`BlueprintMapLibrary.Map_Find` (`.IntParamList_6_03F5988F47C559338AD1C6A821043712` (break `/Game/IS_CharacterCreator/Core/Data/Struct/Param/FStruct_ACC_GroupParam` GroupParam)) Identifier))
  (return (`.Value_9_9FCA4F124E3FE5A4992336B2AFEAD7B4` (break `/Game/IS_CharacterCreator/Core/Data/Struct/Param/FStruct_ACC_IntParam` _value)) _returnvalue))

(fn `GetGPTexValueFromGP`
  (params (GroupParam :type "/Game/IS_CharacterCreator/Core/Data/Struct/Param/FStruct_ACC_GroupParam Structure (by ref)") (Identifier :type Name))
  (returns (Value :type "Texture2D Object Reference") (Exist :type Boolean))
  (bind (_value _returnvalue) (`BlueprintMapLibrary.Map_Find` (`.TexParamList_17_F7107AE448951437923FD5888D98F51E` (break `/Game/IS_CharacterCreator/Core/Data/Struct/Param/FStruct_ACC_GroupParam` GroupParam)) Identifier))
  (return (`.Value_11_9FCA4F124E3FE5A4992336B2AFEAD7B4` (break `/Game/IS_CharacterCreator/Core/Data/Struct/Param/FStruct_ACC_TexParam` _value)) _returnvalue))

(fn `GetGroupParamFromIdentifier`
  (params (Identifier :type Name))
  (returns (GroupParam :type "/Game/IS_CharacterCreator/Core/Data/Struct/Param/FStruct_ACC_GroupParam Structure") (Exist :type Boolean))
  (bind (_groupparam _exist) (`/Game/IS_CharacterCreator/Core/Library/BPFL_ACC_GroupParam.GetGroupParam` (`self.GroupParamList`) Identifier))
  (return _groupparam _exist))

(fn `GetHairSpeciePrefix`
  (returns (Specie :type Name))
  (return (`.HairKindIdentifier_9_926B80384BC905B146293AB36880665C` (break `/Game/IS_CharacterCreator/Core/Data/Struct/FStruct_ACC_CustomConfParam` (`.CustomConf_16_9952A7684B7AF3A6E39087B165AB2F7F` (break `/Game/IS_CharacterCreator/Core/Data/Struct/FStruct_ACC_SpecieParam` (`self.SpecieConfiguration`)))))))

(fn `GetHeadMesh`
  (returns (HeadMesh :type "SkeletalMeshComponent Object Reference") (AnimeMesh :type "/Game/IS_CharacterCreator/Core/Data/Struct/FStruct_ACC_AnimeMesh Structure"))
  ;[0 1 0.7422] Interface to get head mesh for easier integration
  (bind (_mesh _animemesh) (message `/Game/IS_CharacterCreator/Core/Interface/BPI_ACC_CharacterCustomization.I_GetHeadMesh` (`self.GetPossesor`)))
  (return _mesh _animemesh))

(fn `GetMaturityConf`
  (returns (MaturityMesh :type "Map of /Game/IS_CharacterCreator/Core/Data/Enum/E_ACC_Maturity Enum to /Game/IS_CharacterCreator/Core/Data/Struct/FStruct_ACC_MaturityParam Structure"))
  (return (`.MaturityList_18_E570BB114E32D76AF3D651B958A3CE6B` (break `/Game/IS_CharacterCreator/Core/Data/Struct/FStruct_ACC_SpecieParam` (`self.SpecieConfiguration`)))))

(fn `GetOneGenderData`
  (params (Maturity :type "/Game/IS_CharacterCreator/Core/Data/Enum/E_ACC_Maturity Enum" :default "NewEnumerator0") (Gender :type "/Game/IS_CharacterCreator/Core/Data/Enum/E_ACC_Gender Enum" :default "NewEnumerator0"))
  (returns (GenderData :type "/Game/IS_CharacterCreator/Core/Data/Struct/FStruct_ACC_GenderConfig Structure"))
  (return (`BlueprintMapLibrary.Map_Find` (`.Gender_4_5FF97CF340F24C0366E8588AEDC26D88` (break `/Game/IS_CharacterCreator/Core/Data/Struct/FStruct_ACC_MaturityParam` (`self.GetOneMaturityData` Maturity))) Gender)))

(fn `GetOneMaturityData`
  (params (Maturity :type "/Game/IS_CharacterCreator/Core/Data/Enum/E_ACC_Maturity Enum" :default "NewEnumerator0"))
  (returns (Value :type "/Game/IS_CharacterCreator/Core/Data/Struct/FStruct_ACC_MaturityParam Structure"))
  (return (`BlueprintMapLibrary.Map_Find` (`self.GetMaturityConf`) Maturity)))

(fn `GetPossesor`
  (returns (Possessor :type "Actor Object Reference"))
  (return (`self.GetOwner`)))

(fn `GetRefMesh`
  (returns (RefMesh :type "SkeletalMeshComponent Object Reference"))
  (bind _refmesh (message `/Game/IS_CharacterCreator/Core/Interface/BPI_ACC_CharacterCustomization.I_GetRefMesh` (`self.GetPossesor`)))
  (return _refmesh))

(fn `GetSpecieInformation`
  (returns (SpecieIdentifier :type Name) (Maturity :type "/Game/IS_CharacterCreator/Core/Data/Enum/E_ACC_Maturity Enum") (Gender :type "/Game/IS_CharacterCreator/Core/Data/Enum/E_ACC_Gender Enum"))
  (return (`self.SpecieIdentifier`) (`self.Maturity`) (`self.Gender`)))

(fn `InitBodyCopyRef`
  (bind _bodymesh (`self.GetBodyMesh`))
  (if (`self.UseSeparateBody`)
    (`SkeletalMeshComponent.SetAnimInstanceClass` _bodymesh "/Game/IS_CharacterCreator/Character/OldHuman/Maturity/Adult/ABP_ACC_OldHmn_Adult_Ref.ABP_ACC_OldHmn_Adult_Ref_C")
    (message `/Game/IS_CharacterCreator/Core/Interface/BPI_ACC_ModularCloth.I_SetMeshReference` (`SkeletalMeshComponent.GetAnimInstance` _bodymesh) (`self.GetRefMesh`))))

(fn `InitDefaultSetUp`
  ;[1 0.7969 0] Instance all necessary actor and apply all parameters
  (`self.CheckInstanceCtm`)
  ;[0.4062 1 0] Hook : Set init true and init param if waiting for (espcially for network)
  (`self.SetIsInit` true)
  ;[1 0 0.75] Custom init
  (message `/Game/IS_CharacterCreator/Core/Interface/BPI_ACC_CharacterCustomization.I_CustomInit` (`self.GetPossesor`))
  ;[0 0.01562 1] Callback (on have init all necessary object)
  (`self.OnACCInit`))

(fn `InitDynamicBodyMat`
  (bind _bodymesh (`self.GetBodyMesh`))
  (`KismetArrayLibrary.Array_Clear` (`self.BodyDynamicMaterials`))
  (switch `name` (`self.SpecieIdentifier`) ; RG: ACC_WRN_IMPORTANT
    (:`Default`
      ;[0 0.25 1] By default register all body mats
      (for (_array_element _array_index) (`MeshComponent.GetMaterials` _bodymesh)
        (bind _returnvalue (`PrimitiveComponent.CreateDynamicMaterialInstance` _bodymesh _array_index _array_element "None"))
        (`KismetArrayLibrary.Array_AddUnique` (`self.BodyDynamicMaterials`) _returnvalue)))
    (:`epic_hmn`
      ;[1 0 0.4219] Epic Hmn Body
      (bind _returnvalue_2 (`PrimitiveComponent.CreateDynamicMaterialInstance` (`self.GetBodyMesh`) 0 null "None"))
      (`KismetArrayLibrary.Array_AddUnique` (`self.BodyDynamicMaterials`) _returnvalue_2))
    (:`old_hmn`
      ;[0 0.4141 1] Old Hmn Body
      (for _index (range 2)
        (bind _returnvalue_3 (`PrimitiveComponent.CreateDynamicMaterialInstance` (`self.GetBodyMesh`) _index null "None"))
        (`KismetArrayLibrary.Array_AddUnique` (`self.BodyDynamicMaterials`) _returnvalue_3)))))

(fn `InitFromACCCharData`
  (params (ACC_CharacterData :type "/Game/IS_CharacterCreator/Core/Data/Struct/FStruct_ACC_Character Structure"))
  ;[0 0.5312 1] Init character customization before equipement
  (`self.InitFromParameters` (`.CharCustom_2_185AFF684768515E4FE853A48612311C` (break `/Game/IS_CharacterCreator/Core/Data/Struct/FStruct_ACC_Character` ACC_CharacterData))))

(fn `InitFromACCCharDataAsync`
  (params (ACC_CharacterData :type "/Game/IS_CharacterCreator/Core/Data/Struct/FStruct_ACC_Character Structure"))
  (if (`self.bInit`)
    (`self.InitFromACCCharData` ACC_CharacterData)
    (else
      (`self.SetInitTask` ACC_CharacterData))))

(fn `InitFromParameters`
  (params (CharParameters :type "/Game/IS_CharacterCreator/Core/Data/Struct/Customization/FStruct_ACC_CharacterCustom Structure"))
  ;[1 0.8906 0] Change Specie
  (`self.ChangeSpecie` (`.Specie_35_2B7BBCA6419FE018D0239486B86E5365` (break `/Game/IS_CharacterCreator/Core/Data/Struct/Customization/FStruct_ACC_CharacterCustom` CharParameters)))
  (`self.MapCharParameters` CharParameters)
  (`self.ChangeMaturity` (`self.Maturity`)) ; Maturity is the top level modification
  (`self.ChangeGender` (`self.Gender`))
  ;[0 1 0.4609] Notify any data change for all observable class
  ; In case the character or actor possessor
  (`self.OnChangeAnyData`))

(fn `MapCharParameters`
  (params (CharParameters :type "/Game/IS_CharacterCreator/Core/Data/Struct/Customization/FStruct_ACC_CharacterCustom Structure"))
  (bind (_specie _maturity _gender _groupparamlist) (break `/Game/IS_CharacterCreator/Core/Data/Struct/Customization/FStruct_ACC_CharacterCustom` CharParameters))
  (set `self.SpecieIdentifier` _specie)
  (set `self.GroupParamList` _groupparamlist)
  (set `self.Maturity` _maturity)
  (set `self.Gender` _gender))

(fn `MasterPoseSkinnedMesh`
  (params (SkinnedMesh :type "SkinnedMeshComponent Object Reference") (ActiveMasterPose :type Boolean))
  (if ActiveMasterPose
    (`SkinnedMeshComponent.SetLeaderPoseComponent` SkinnedMesh (`self.GetBodyMesh`) false)
    (else
      (`SkinnedMeshComponent.SetLeaderPoseComponent` SkinnedMesh null false) ; IMPORTANT : SetMasterPose empty else UE4 will crash for violation adress
    )))

(fn `OnChangeAnyData`
  (bind _charctmdata (`self.GetCharCustomizationData`))
  (message `/Game/IS_CharacterCreator/Core/Interface/BPI_ACC_CharacterCustomization.I_OnCharCtmChange` (`self.GetPossesor`) _charctmdata)
  ;[1 0 0] OPC: AnyData
  (`self.FireParamChange` "AnyData"))

(fn `PerformTagScript`
  (params (Key :type Name) (bActive :type Boolean))
  (bind (_returnvalue _valid) (`/Game/IS_CharacterCreator/Core/Data/DataAsset/DA_ACC_Component.GetTagScript` (`self.DataConfig`) Key))
  (if _valid
    (`/Game/IS_CharacterCreator/Core/Object/Module/BP_ACC_Gameplay.PerformScript` (`/Game/IS_CharacterCreator/Core/Library/BPFL_ACC_Common.GetACCGameplay`) self _returnvalue bActive)))

(fn `ResetBody`
  (`KismetArrayLibrary.Array_Clear` (`self.BodyDynamicMaterials`)))

(fn `SelectBodyHideParamName`
  (params (ItemPart :type Name))
  (returns (ParamName :type Name))
  (return (`/Game/IS_CharacterCreator/Core/Library/BPFL_ACC_Common.TextToName` (`|FormatText` "T_{Part}Hide" ItemPart))))

(fn `SelectGenderMeshes`
  (returns (SKMesh :type "SkeletalMesh Object Reference") (AnimInstance :type "AnimInstance Class Reference"))
  (bind (_skmesh _defaultaniminst) (break `/Game/IS_CharacterCreator/Core/Data/Struct/FStruct_ACC_GenderConfig` (`self.GetCurrentGenderData`)))
  (return _skmesh _defaultaniminst))

(fn `SetGlobalMorphTarget`
  (params (MorphTargetName :type Name) (Mesh :type "SkeletalMeshComponent Object Reference") (Value :type "Float (double-precision)") (ApplyOnSkinnedMesh :type Boolean :default true))
  ;[1 0.9844 0] Update in Body
  (`SkeletalMeshComponent.SetMorphTarget` Mesh MorphTargetName Value true))

(fn `SetInitTask`
  (params (ACC_CharacterTask :type "/Game/IS_CharacterCreator/Core/Data/Struct/FStruct_ACC_Character Structure"))
  (set `self.ACC_CharacterTask` ACC_CharacterTask)
  (set `self.bInitParamTask` true))

(fn `SetIsInit`
  (params (bInit :type Boolean))
  (set `self.bInit` bInit)
  (if (`self.bInitParamTask`)
    (`self.InitFromACCCharData` (`self.ACC_CharacterTask`))
    (set `self.bInitParamTask` false)))

(fn `SetItemVisiblity`
  (params (HairVisible :type Boolean) (SkinnedVisible :type Boolean))
  ;[0.7578 0 1] Hair Visiblity
  (`/Game/IS_CharacterCreator/Core/Item/Customization/Hair/BP_ACC_Hair_Ctm_Base.SetHairVisibility` (`self.BP_Hair_Customization`) HairVisible))

(fn `UpdateObjectColor`
  (params (Mesh :type "MeshComponent Object Reference") (ParamName :type Name) (Color :type "LinearColor Structure"))
  (`MeshComponent.SetVectorParameterValueOnMaterials` Mesh ParamName (`KismetMathLibrary.Conv_LinearColorToVector` Color)))

(fn `UpdateOutline`
  (params (SourceMesh :type "SkeletalMeshComponent Object Reference") (OutlineMesh :type "SkeletalMeshComponent Object Reference"))
  (if (`/Game/IS_CharacterCreator/Core/Data/DataAsset/DA_ACC_Component.bUseOutline` (`self.DataConfig`))
    (`/Game/IS_CharacterCreator/Core/Library/BPFL_ACC_Extractor.ACCOutlineMesh` (`SkinnedMeshComponent.SkeletalMesh` SourceMesh) SourceMesh OutlineMesh (`self.OutlineMaterial`))))