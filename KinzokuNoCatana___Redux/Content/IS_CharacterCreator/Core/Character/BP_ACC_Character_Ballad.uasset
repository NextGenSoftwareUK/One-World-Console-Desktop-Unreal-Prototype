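; BP_ACC_Character_Ballad is a character Blueprint in the character creator that adds a networked dash to movement.
; SetActiveDash forwards to a server event, which sets the replicated Dash flag and updates max walk speed.
; The RepNotify reapplies that speed and passes the dash state to the anim instance.
; Dash speed is a multiple of the maturity-based walk speed.
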(event `self.ReceiveBeginPlay`
  (`parent.ReceiveBeginPlay`))

(event `/Game/IS_CharacterCreator/Core/Interface/BPI_ACC_CharacterMovement.SetActiveDash`
  (params (Active :type Boolean))
  ;[0.6875 1 0] On receive client side call server side
  (`self.Server_ActiveDash` Active))

(event `Server_ActiveDash`
  (params (Active :type Boolean))
  ;[0 0.9766 1] Server side : Receive active dash and update movement walk speed
  (set `self.bDash` Active)
  (set `CharacterMovementComponent.MaxWalkSpeed` (`self.GetDashSpeed`) (`self.CharacterMovement`)))

(fn `GetDashSpeed`
  (returns (ReturnValue :type "Float (double-precision)"))
  (bind _value (`self.GetWalkSpeedMaturity`))
  (return (select `bool` (`self.bDash`) :`false` _value :`true` (* _value 1.5))))

(fn `OnRep_bDash`
  (set `CharacterMovementComponent.MaxWalkSpeed` (`self.GetDashSpeed`) (`self.CharacterMovement`))
  (message `/Game/IS_CharacterCreator/Core/Interface/BPI_ACC_CharacterMovement.SetActiveDash` (`self.GetAnimInst`) (`self.bDash`)))

(fn `UserConstructionScript`
  (`parent.UserConstructionScript`))