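; Character for the modular character creator (ACC), exposing its meshes and modular component through interface functions.
; The modular component builds a default setup on BeginPlay; replicated compact data is mapped back on RepNotify to set species and asynchronously load the saved look.
; Jump, movement mode, maturity and customization changes are forwarded to the AnimInstance, and gender changes refresh maturity-based walk speed.
; Tick optionally aims the head at the player or camera, skipped on dedicated servers.
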(event `self.ReceiveBeginPlay`
  (bind _modularcharcomp (`self.I_GetModularComp`))
  (`/Game/IS_CharacterCreator/Core/Component/BP_ACC_MCC_Base.InitDefaultSetUp` _modularcharcomp))

(event `self.ReceiveTick`
  (params (DeltaSeconds :type "Float (single-precision)"))
  (`self.UpdateLookAt`))

(event `/Game/IS_CharacterCreator/Core/Interface/BPI_ACC_CharacterMovement.JumpStart`
  ;[0.8281 0 1] When want to jump
  (`self.Jump`)
  (message `/Game/IS_CharacterCreator/Core/Interface/BPI_ACC_CharacterMovement.JumpStart` (`self.GetAnimInst`)))

(event `self.K2_OnMovementModeChanged`
  (params (PrevMovementMode :type "EMovementMode Enum" :default "MOVE_None") (NewMovementMode :type "EMovementMode Enum" :default "MOVE_None") (PrevCustomMode :type Byte) (NewCustomMode :type Byte))
  ;[0.1484 0 1] Notify to anim instance when movement mode changed
  (message `/Game/IS_CharacterCreator/Core/Interface/BPI_ACC_CharacterMovement.OnMovementModeChanged` (`self.GetAnimInst`) PrevMovementMode NewMovementMode))

(event `self.I_OnMaturityChange`
  (params (Maturity :type "/Game/IS_CharacterCreator/Core/Data/Enum/E_ACC_Maturity Enum" :default "NewEnumerator0"))
  ;[0 1 0.9766] Notify to anim instance Matuirty changed
  (message `/Game/IS_CharacterCreator/Core/Interface/BPI_ACC_CharacterCustomization.I_OnMaturityChange` (`self.GetAnimInst`) Maturity))

(event `self.I_OnCharCtmChange`
  (params (ACC_CharCtm :type "/Game/IS_CharacterCreator/Core/Data/Struct/Customization/FStruct_ACC_CharacterCustom Structure"))
  ;[0 0.2734 1] Notify to any parameters change
  (message `/Game/IS_CharacterCreator/Core/Interface/BPI_ACC_CharParamListener.I_OnCharParamChange` (`self.GetAnimInst`) ACC_CharCtm))

(event `self.BP_ACC_MCC_HmnDefault.OnACCInit`
  ;[1 0.8411 0.5051] WARNING: Used for example, notify to her ballad controller in
  ; demo that ACC Modular Comp has init and can load your created char
  (bind _asbp_acc_ballad_controller (cast `/Game/IS_CharacterCreator/Core/Controller/BP_ACC_Ballad_Controller` (`self.GetController`)))
  (`/Game/IS_CharacterCreator/Core/Controller/BP_ACC_Ballad_Controller.OnACCInit` _asbp_acc_ballad_controller))

(event `/Game/IS_CharacterCreator/Core/Interface/BPI_ACC_NetChar.I_Net_InitACC_Char`
  (params (ACC_Character_Net :type "/Game/IS_CharacterCreator/Core/Data/Struct/Network/FStruct_ACC_CharacterNet Structure"))
  ;[0.2656 1 0] Init Network Data
  (set `self.SavedACC_Char_Net` ACC_Character_Net))

(event `/Game/IS_CharacterCreator/Core/Interface/BPI_ACC_Facial.I_Facial_EyeClip`
  (params (Value :type "Float (double-precision)"))
  ;[0.6172 1 0] Eye Close From EyeShapeId
  (`/Engine/EditorBlueprintResources/StandardMacros.IsValid` (`self.GetHeadMesh`)))

(event `self.BP_ACC_MCC_HmnDefault.OnParamChange`
  (params (ParamName :type Name))
  (switch `name` ParamName
    (:`Gender`
      (set `CharacterMovementComponent.MaxWalkSpeed` (`self.GetWalkSpeedMaturity`) (`self.CharacterMovement`)))))

(fn `GetAnimInst`
  (returns (ReturnValue :type "AnimInstance Object Reference"))
  (return (`SkeletalMeshComponent.GetAnimInstance` (`self.Mesh`))))

(fn `GetBodyMesh`
  (returns (BodyMesh :type "SkeletalMeshComponent Object Reference"))
  (return (`self.Mesh`)))

(fn `GetHeadMesh`
  (returns (HeadMesh :type "SkeletalMeshComponent Object Reference"))
  (bind _mesh (`self.I_GetHeadMesh`))
  (return _mesh))

(fn `GetModularCharComp`
  (returns (ModularCharacter :type "/Game/IS_CharacterCreator/Core/Component/BP_ACC_MCC_Base Object Reference"))
  (return (`self.BP_ACC_MCC_HmnDefault`)))

(fn `GetWalkSpeedMaturity`
  (returns (Value :type "Float (double-precision)") (ReturnValue :type Boolean))
  (bind _modularcharcomp (`self.I_GetModularComp`))
  (bind (_value _returnvalue) (`BlueprintMapLibrary.Map_Find` (`self.WalkSpeed`) (`/Game/IS_CharacterCreator/Core/Component/BP_ACC_MCC_Base.Maturity` _modularcharcomp)))
  (return _value _returnvalue))

(fn `I_GetBodyMesh`
  (returns (Mesh :type "SkeletalMeshComponent Object Reference") (AnimeMesh :type "/Game/IS_CharacterCreator/Core/Data/Struct/FStruct_ACC_AnimeMesh Structure"))
  (bind _bodymesh (`self.GetBodyMesh`))
  (return _bodymesh (make `/Game/IS_CharacterCreator/Core/Data/Struct/FStruct_ACC_AnimeMesh` _bodymesh (`self.BodyOutline`))))

(fn `I_GetHeadMesh`
  (returns (Mesh :type "SkeletalMeshComponent Object Reference") (AnimeMesh :type "/Game/IS_CharacterCreator/Core/Data/Struct/FStruct_ACC_AnimeMesh Structure"))
  (bind _headmesh (`self.GetHeadMesh`))
  (return _headmesh (make `/Game/IS_CharacterCreator/Core/Data/Struct/FStruct_ACC_AnimeMesh` _headmesh)))

(fn `I_GetModularComp`
  (returns (ModularCharComp :type "/Game/IS_CharacterCreator/Core/Component/BP_ACC_MCC_Base Object Reference"))
  (return (`self.GetModularCharComp`)))

(fn `I_GetRefMesh`
  (returns (RefMesh :type "SkeletalMeshComponent Object Reference"))
  (return (`self.Mesh`)))

(fn `OnRep_SavedACC_Char_Net`
  (locals (TempACC_Character :type "/Game/IS_CharacterCreator/Core/Data/Struct/FStruct_ACC_Character Structure") (CurrentEquipKey :type Name) (TmpEquipIdList :type Boolean))
  (bind _tempacc_character (`local.TempACC_Character`))
  ;[0 0.8125 1] Before Init, we need to map and load item
  (bind _acc_character (`/Game/IS_CharacterCreator/Core/Library/BPFL_ACC_Network.MapNetTo_ACCChar` (`self.SavedACC_Char_Net`)))
  (set `local.TempACC_Character` _acc_character)
  ;[0 1 0.3438] Finally store retrieve equip data and init
  (bind _modularcharcomp (`self.I_GetModularComp`))
  (`/Game/IS_CharacterCreator/Core/Component/BP_ACC_MCC_Base.ChangeSpecie` _modularcharcomp (`.Specie_35_2B7BBCA6419FE018D0239486B86E5365` (break `/Game/IS_CharacterCreator/Core/Data/Struct/Customization/FStruct_ACC_CharacterCustom` (`.CharCustom_2_185AFF684768515E4FE853A48612311C` (break `/Game/IS_CharacterCreator/Core/Data/Struct/FStruct_ACC_Character` _tempacc_character)))))
  (`/Game/IS_CharacterCreator/Core/Component/BP_ACC_MCC_Base.InitDefaultSetUp` _modularcharcomp)
  (`/Game/IS_CharacterCreator/Core/Component/BP_ACC_MCC_Base.InitFromACCCharDataAsync` _modularcharcomp _tempacc_character) ; User for network
)

(fn `SetCharacterData`
  (params (ACC_Character :type "/Game/IS_CharacterCreator/Core/Data/Struct/FStruct_ACC_Character Structure"))
  (bind _acc_character_net (`/Game/IS_CharacterCreator/Core/Library/BPFL_ACC_Network.MapACC_Char_ToNet` ACC_Character))
  (set `self.SavedACC_Char_Net` _acc_character_net))

(fn `UpdateLookAt`
  (bind _returnvalue (`SkeletalMeshComponent.GetAnimInstance` (`self.GetHeadMesh`)))
  (if (`KismetSystemLibrary.IsDedicatedServer`)
    _
    (elif (`self.bTestLookAt`)
      (bind _mesh (`self.I_GetHeadMesh`))
      (`/Engine/EditorBlueprintResources/StandardMacros.IsValid` _returnvalue
        (:`Is Valid`
          (message `/Game/IS_CharacterCreator/Core/Interface/BPI_ACC_CharacterHead.I_LookAt` _returnvalue (`KismetMathLibrary.MakeRotator` 0.0 (- (.pitch (`KismetMathLibrary.FindLookAtRotation` (`SceneComponent.K2_GetComponentLocation` _mesh) (`self.K2_GetActorLocation` (select `bool` (`self.bLookAtPlayer`) :`false` (`GameplayStatics.GetPlayerCameraManager` 0) :`true` (`GameplayStatics.GetPlayerCharacter` 0) :!type "Actor Object Reference")))) (.pitch (`self.K2_GetActorRotation`))) (- (.yaw (`KismetMathLibrary.FindLookAtRotation` (`SceneComponent.K2_GetComponentLocation` _mesh) (`self.K2_GetActorLocation` (select `bool` (`self.bLookAtPlayer`) :`false` (`GameplayStatics.GetPlayerCameraManager` 0) :`true` (`GameplayStatics.GetPlayerCharacter` 0) :!type "Actor Object Reference")))) (.yaw (`self.K2_GetActorRotation`)))))
          (return)))
      (else
        (return)))))

(fn `UserConstructionScript`)