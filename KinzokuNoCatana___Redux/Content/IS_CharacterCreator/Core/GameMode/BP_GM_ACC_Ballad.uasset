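; BP_GM_ACC_Ballad is a character creator game mode that spawns and possesses each player's custom character.
; SpawnCharacter resolves the character class from the species config data table, then spawns it at an X offset based on the current player count.
; It records the spawned BP_ACC_Character in a list, passes it the net character data through an interface message and has the given controller possess it.
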(fn `CountNumberPlayer`
  (returns (Count :type Integer))
  (return (`KismetArrayLibrary.Array_Length` (`self.NetCharacterList`))))

(fn `GetSpecieBP`
  (params (Specie :type Name))
  (returns (CharacterBPClass :type "Actor Class Reference") (Found :type Boolean))
  (bind _returnvalue (`|GetDataTableRow` (`self.DT_SpecieGameConfig`) Specie)
    (:`then`
      (return (`.CharacterBPClass_3_3ADDDBF342863D79E6224F8BEADB44D9` (break `/Game/IS_CharacterCreator/Core/Data/Struct/Example/FStruct_ACC_SpecieGameConfig` _returnvalue)) true))
    (:`RowNotFound`
      (return "/Script/Engine.Actor" false))))

(fn `SpawnCharacter`
  (params (ACC_Character_Net :type "/Game/IS_CharacterCreator/Core/Data/Struct/Network/FStruct_ACC_CharacterNet Structure") (Controller :type "PlayerController Object Reference"))
  (locals (CurrentCharacter :type "Character Object Reference"))
  (bind _count (`self.CountNumberPlayer`))
  (bind _characterbpclass (`self.GetSpecieBP` (`.Specie_41_81B913974634AF3B7042B49F8DB1AA42` (break `/Game/IS_CharacterCreator/Core/Data/Struct/Network/FStruct_ACC_CharCustom_Net` (`.CharCustom_18_185AFF684768515E4FE853A48612311C` (break `/Game/IS_CharacterCreator/Core/Data/Struct/Network/FStruct_ACC_CharacterNet` ACC_Character_Net))))))
  (bind _returnvalue (`|SpawnActorFromClass` _characterbpclass (`KismetMathLibrary.MakeTransform` (`KismetMathLibrary.MakeVector` (`KismetMathLibrary.Conv_IntToDouble` (* _count 200)) 0.0 100.0) (struct :`Yaw` 180.0)) "Undefined" "OverrideRootScale" null null))
  (bind _asbp_acc_character (cast `/Game/IS_CharacterCreator/Core/Character/BP_ACC_Character` _returnvalue))
  (bind _output_get (set `local.CurrentCharacter` _asbp_acc_character))
  ;[0.07812 1 0] Add to list
  (`KismetArrayLibrary.Array_Add` (`self.NetCharacterList`) _output_get)
  ;[0 1 0.08594] Init Character Data
  (message `/Game/IS_CharacterCreator/Core/Interface/BPI_ACC_NetChar.I_Net_InitACC_Char` (`local.CurrentCharacter`) ACC_Character_Net)
  ;[0.3594 1 0] Possess the character
  (`Controller.Possess` Controller (`local.CurrentCharacter`)))

(fn `UserConstructionScript`)