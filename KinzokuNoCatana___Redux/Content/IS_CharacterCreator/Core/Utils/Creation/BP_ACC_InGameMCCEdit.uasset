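; In-game trigger point that lets the player edit their current character through the ACC character creator.
; When the player enters its box, it spawns a task that moves the character to the edit point.
; Once the character is ready, it hides the Ballad HUD, spawns a creation manager with the Ballad creation widget and blocks input.
; Destruction of that manager ends editing, restoring the HUD and game input.
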(event `self.Box.OnComponentBeginOverlap`
  (params (OverlappedComponent :type "PrimitiveComponent Object Reference") (OtherActor :type "Actor Object Reference") (OtherComp :type "PrimitiveComponent Object Reference") (OtherBodyIndex :type Integer) (bFromSweep :type Boolean) (SweepResult :type "HitResult Structure (by ref)"))
  (if (== OtherActor (`GameplayStatics.GetPlayerCharacter` 0))
    ;[0 0.8828 1] Spawn task to move character to him
    (bind _returnvalue (`|SpawnActorFromClass` "/Game/IS_CharacterCreator/Core/Utils/Task/BP_ACC_MoveToEdition_Task.BP_ACC_MoveToEdition_Task_C" (`self.GetTransform`) "Undefined" "OverrideRootScale" null self null))
    ;[0.5 1 0] Bind when task finished
    (add `/Game/IS_CharacterCreator/Core/Utils/Task/BP_ACC_Task.OnFinished` _returnvalue (`|CreateDelegate` :!event `OnCharacteReady`))))

(fn `OnCharacteReady`
  (`|ExecutionSequence`
    (:`then_0`
      ;[0.1953 1 0] First hide ballad UI
      (`self.SetBalladUIVisible` false))
    (:`then_1`
      ;[0.7109 0 1] It's editing actual character
      (`/Game/IS_CharacterCreator/Core/Object/Module/BP_ACC_MCCEdition.SetActionMode` (`/Game/IS_CharacterCreator/Core/Object/Module/BP_ACC_Gameplay.GetMCCEdition` (`/Game/IS_CharacterCreator/Core/Library/BPFL_ACC_Common.GetACCGameplay`)) true)
      (bind _returnvalue (`|SpawnActorFromClass` "/Game/IS_CharacterCreator/Core/Manager/BP_ACC_CreationManager.BP_ACC_CreationManager_C" (`self.GetTransform` (`GameplayStatics.GetPlayerCharacter` 0)) "Undefined" "OverrideRootScale" null "/Game/IS_CharacterCreator/Core/Widget/Screens/Creator/WBP_ACC_BalladCharacterCreation.WBP_ACC_BalladCharacterCreation_C" 1.5 null))
      ;[0.5469 0 1] Listen when bp destroyed (end edition)
      (add `self.OnDestroyed` _returnvalue (`|CreateDelegate` :!event `OnEditionEnd`))
      (`/Game/IS_CharacterCreator/Core/Library/BPFL_ACC_Common.BlockInput` (`/Game/IS_CharacterCreator/Core/Manager/BP_ACC_CreationManager.CurrentUI` _returnvalue)))))

(fn `OnEditionEnd`
  (params (DestroyedActor :type "Actor Object Reference"))
  (`self.SetBalladUIVisible` true)
  (`/Game/IS_CharacterCreator/Core/Library/BPFL_ACC_Common.RestoreGameInput`))

(fn `SetBalladUIVisible`
  (params (Visible :type Boolean))
  (bind _asbp_acc_hud_ballad (cast `/Game/IS_CharacterCreator/Core/HUD/BP_ACC_HUD_Ballad` (`PlayerController.GetHUD` (`GameplayStatics.GetPlayerController` 0))))
  (`/Game/IS_CharacterCreator/Core/HUD/BP_ACC_HUD_Ballad.SetBalladUIVisible` _asbp_acc_hud_ballad Visible))

(fn `UserConstructionScript`)