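; A short-lived task actor that auto-walks the player character to the character creator's edition point.
; On BeginPlay it slows walk speed, blocks input and starts SimpleMoveToLocation toward MCCEditionPoint.
; Tick treats the loss of a valid current path as arrival, then matches the point's rotation and restores speed.
; It finally snaps the character to the point's X and Y, keeping its Z, and destroys itself.
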(event `self.ReceiveBeginPlay`
  (bind _charactermovement (`Character.CharacterMovement` (`GameplayStatics.GetPlayerCharacter` 0)))
  (`parent.ReceiveBeginPlay`)
  ;[0.7109 0 1] Store old walk speed
  (set `self.InitialWalkSpeed` (`CharacterMovementComponent.MaxWalkSpeed` _charactermovement))
  (set `CharacterMovementComponent.MaxWalkSpeed` 200.0 _charactermovement)
  (`|ExecutionSequence`
    (:`then_0`
      ;[0 0.7891 1] Force stop input (and locig inside lick disable dash)
      (`/Game/IS_CharacterCreator/Core/Library/BPFL_ACC_Common.BlockInput` null))
    (:`then_1`
      ;[0 1 0.7188] Stop any character movement
      (`MovementComponent.StopMovementImmediately` (`Character.CharacterMovement` (`GameplayStatics.GetPlayerCharacter` 0)))
      ;[0.5469 0 1] Start auto move character to goal location
      (`AIBlueprintHelperLibrary.SimpleMoveToLocation` (`GameplayStatics.GetPlayerController` 0) (`self.GetGoalLocation`))
      (set `self.Moving` true))))

(event `self.ReceiveTick`
  (params (DeltaSeconds :type "Float (single-precision)"))
  (`parent.ReceiveTick` DeltaSeconds)
  ;[0.5703 0 1] While moving goal location
  (if (`self.Moving`)
    (`/Engine/EditorBlueprintResources/StandardMacros.IsValid` (`AIBlueprintHelperLibrary.GetCurrentPath` (`GameplayStatics.GetPlayerController` 0)) ; To check if reached the goal point
      (:`Is Not Valid`
        (`MovementComponent.StopMovementImmediately` (`Character.CharacterMovement` (`GameplayStatics.GetPlayerCharacter` 0)))
        (`self.K2_SetActorRotation` (`GameplayStatics.GetPlayerCharacter` 0) (`self.K2_GetActorRotation` (`self.MCCEditionPoint`)) false)
        (set `self.Moving` false)
        ;[0 0.8125 1] Restore walk speed
        (set `CharacterMovementComponent.MaxWalkSpeed` (`self.InitialWalkSpeed`) (`Character.CharacterMovement` (`GameplayStatics.GetPlayerCharacter` 0)))
        ;[1 0 0.6797] Avoid some bug
        (`self.FixLocation`)
        (`self.K2_DestroyActor`)))))

(fn `FixLocation`
  (bind (_returnvalue_x _returnvalue_y) (`KismetMathLibrary.BreakVector` (`self.GetGoalLocation`)))
  (bind _returnvalue (`GameplayStatics.GetPlayerCharacter` 0))
  (bind (_returnvalue_x_2 _returnvalue_y_2 _returnvalue_z) (`KismetMathLibrary.BreakVector` (`self.K2_GetActorLocation` _returnvalue)))
  (`self.K2_SetActorLocation` _returnvalue (`KismetMathLibrary.MakeVector` _returnvalue_x _returnvalue_y _returnvalue_z) false false))

(fn `GetGoalLocation`
  (returns (ReturnValue :type "Vector Structure"))
  (return (`self.K2_GetActorLocation` (`self.MCCEditionPoint`))))

(fn `UserConstructionScript`
  (`parent.UserConstructionScript`))