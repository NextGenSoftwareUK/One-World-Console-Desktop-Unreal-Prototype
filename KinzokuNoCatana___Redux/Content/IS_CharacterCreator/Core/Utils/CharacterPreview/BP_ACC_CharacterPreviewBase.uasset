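; Base Blueprint for character creator preview actors, providing look-at behavior toward the player character or camera.
; UpdateLookAt skips dedicated servers and, when TestLookAt is on, sends the actor-relative rotation from head to target to the head and body anim instances via an interface message.
; GetHeadMesh and TransferCharCustomParam are empty stubs, and Tick is empty, so nothing here calls UpdateLookAt.
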(event `self.ReceiveTick`
  (params (DeltaSeconds :type "Float (single-precision)")))

(fn `GetHeadMesh`
  (returns (HeadMesh :type "SkeletalMeshComponent Object Reference"))
  (return null))

(fn `TransferCharCustomParam`
  (params (CharParameters :type "/Game/IS_CharacterCreator/Core/Data/Struct/Customization/FStruct_ACC_CharacterCustom Structure")))

(fn `UpdateLookAt`
  (bind _returnvalue (`KismetMathLibrary.NormalizedDeltaRotator` (`KismetMathLibrary.FindLookAtRotation` (`SceneComponent.K2_GetComponentLocation` (`self.GetHeadMesh`)) (`self.K2_GetActorLocation` (select `bool` (`self.LookAtPlayer`) :`false` (`GameplayStatics.GetPlayerCameraManager` 0) :`true` (`GameplayStatics.GetPlayerCharacter` 0) :!type "Actor Object Reference"))) (`self.K2_GetActorRotation`)))
  (if (`KismetSystemLibrary.IsDedicatedServer`)
    _
    (elif (`self.TestLookAt`)
      ;[0.2891 0 1] If head valid
      (`/Engine/EditorBlueprintResources/StandardMacros.IsValid` (`self.GetHeadMesh`)
        (:`Is Valid`
          ;[0 1 0.9766] Head Look At
          (message `/Game/IS_CharacterCreator/Core/Interface/BPI_ACC_CharacterHead.I_LookAt` (`SkeletalMeshComponent.GetAnimInstance` (`self.GetHeadMesh`)) _returnvalue)
          ;[0 0.7187 1] Body Look At
          (bind _mesh (message `/Game/IS_CharacterCreator/Core/Interface/BPI_ACC_CharacterCustomization.I_GetBodyMesh` self))
          (message `/Game/IS_CharacterCreator/Core/Interface/BPI_ACC_CharacterHead.I_LookAt` (`SkeletalMeshComponent.GetAnimInstance` _mesh) _returnvalue)
          (return)))
      (else
        (return)))))

(fn `UserConstructionScript`)