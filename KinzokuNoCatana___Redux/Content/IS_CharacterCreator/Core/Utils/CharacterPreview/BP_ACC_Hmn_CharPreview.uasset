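; Preview actor for a human character in the character creator, exposing its body mesh, outline and modular customization component through interface getters.
; Character parameters initialize the modular component, while change notifications are forwarded to the body mesh's anim instance.
; Tick updates look-at, and once the component signals init, eye-clip calls drive the "Close" morph target on the head mesh.
; The head mesh getter returns nothing in this class.
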(event `self.ReceiveBeginPlay`)

(event `self.ReceiveTick`
  (params (DeltaSeconds :type "Float (single-precision)"))
  (`self.UpdateLookAt`))

(event `/Game/IS_CharacterCreator/Core/Interface/BPI_ACC_Facial.I_Facial_EyeClip`
  (params (Value :type "Float (double-precision)"))
  ;[1 0.9844 0] Eye Close From EyeShapeId
  (if (`self.bACCInit`)
    (`/Engine/EditorBlueprintResources/StandardMacros.IsValid` null
      (:`Is Valid`
        (`self.I_GetModularComp`)
        (bind _mesh (`self.I_GetHeadMesh`))
        (`SkeletalMeshComponent.SetMorphTarget` _mesh (`/Game/IS_CharacterCreator/Core/Library/BPFL_ACC_Common.GetEyeMorphKey` 0 "Close") Value true)))))

(event `self.BP_ACC_MCC_HmnDefault.OnACCInit`
  ;[0.4062 1 0] Notified on ACC is init
  (set `self.bACCInit` true))

(event `self.I_OnCharCtmChange`
  (params (ACC_CharCtm :type "/Game/IS_CharacterCreator/Core/Data/Struct/Customization/FStruct_ACC_CharacterCustom Structure"))
  ;[0 0.2734 1] Notify to any parameters change
  (message `/Game/IS_CharacterCreator/Core/Interface/BPI_ACC_CharParamListener.I_OnCharParamChange` (`SkeletalMeshComponent.GetAnimInstance` (`self.BodyMesh`)) ACC_CharCtm))

(fn `GetHeadMesh`
  (returns (HeadMesh :type "SkeletalMeshComponent Object Reference"))
  (bind _mesh (`self.I_GetHeadMesh`))
  (return _mesh))

(fn `I_GetBodyMesh`
  (returns (Mesh :type "SkeletalMeshComponent Object Reference") (AnimeMesh :type "/Game/IS_CharacterCreator/Core/Data/Struct/FStruct_ACC_AnimeMesh Structure"))
  (bind _bodymesh (`self.BodyMesh`))
  (return _bodymesh (make `/Game/IS_CharacterCreator/Core/Data/Struct/FStruct_ACC_AnimeMesh` _bodymesh (`self.BodyOutline`))))

(fn `I_GetHeadMesh`
  (returns (Mesh :type "SkeletalMeshComponent Object Reference") (AnimeMesh :type "/Game/IS_CharacterCreator/Core/Data/Struct/FStruct_ACC_AnimeMesh Structure"))
  (return null))

(fn `I_GetModularComp`
  (returns (ModularCharComp :type "/Game/IS_CharacterCreator/Core/Component/BP_ACC_MCC_Base Object Reference"))
  (return (`self.BP_ACC_MCC_HmnDefault`)))

(fn `I_GetRefMesh`
  (returns (RefMesh :type "SkeletalMeshComponent Object Reference"))
  (return (`self.BodyMesh`)))

(fn `TransferCharCustomParam`
  (params (CharParameters :type "/Game/IS_CharacterCreator/Core/Data/Struct/Customization/FStruct_ACC_CharacterCustom Structure"))
  (bind _modularcharcomp (`self.I_GetModularComp`))
  (`/Game/IS_CharacterCreator/Core/Component/BP_ACC_MCC_Base.InitFromParameters` _modularcharcomp CharParameters))

(fn `UserConstructionScript`)